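; BP_RiverSpline is a spline-driven actor that lays out river or small waterfall surfaces along an editable path.
; The construction script adds one spline mesh component per segment, matching the start and end positions and tangents to the spline points.
; An IsThicc flag selects a thick or regular plane mesh, and ShowDebugMaterial swaps the waterfall material for a debug one.
; It has no runtime logic.
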(fn `UserConstructionScript`
  (for _index (range (+ (- (`SplineComponent.GetNumberOfSplinePoints` (`self.Spline`)) 2) 1))
    (bind _returnvalue (`AddComponent|NODE_AddSplineMeshComponent-0`))
    (bind _output_get (set `self.SplineMeshComponentRef` _returnvalue))
    (bind (_location _tangent) (`SplineComponent.GetLocationAndTangentAtSplinePoint` (`self.Spline`) _index "Local"))
    (bind (_location_2 _tangent_2) (`SplineComponent.GetLocationAndTangentAtSplinePoint` (`self.Spline`) (+ _index 1) "Local"))
    (`SplineMeshComponent.SetStartAndEnd` _output_get _location _tangent _location_2 _tangent_2 true)
    (`StaticMeshComponent.SetStaticMesh` (`self.SplineMeshComponentRef`) (select `bool` (`self.IsThicc?`) :`false` "/Game/FXs/Waterfall/petitescascades/Meshes/SM_RiverPlane.SM_RiverPlane" :`true` "/Game/FXs/Waterfall/petitescascades/Meshes/SM_RiverPlaneThicc.SM_RiverPlaneThicc" :!type "StaticMesh Object Reference"))
    (`PrimitiveComponent.SetMaterial` (`self.SplineMeshComponentRef`) 0 (select `bool` (`self.ShowDebugMaterial?`) :`false` "/Game/FXs/Waterfall/petitescascades/Materials/Instances/MI_WaterfallDWF.MI_WaterfallDWF" :`true` "/Game/FXs/Waterfall/petitescascades/Materials/Instances/MI_WF_Debug.MI_WF_Debug" :!type "MaterialInterface Object Reference"))))