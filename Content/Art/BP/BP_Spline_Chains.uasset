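; Chain builder actor that lays out a straight row of mesh links along X when constructed, with physics constraint components between them.
; The construction script clears previous components, then spaces links by the mesh bounds, alternating their rotation by 90 degrees through a FlipFlop.
; Constraints are added from the second link onward, with no components passed to them.
; An unused spline-mesh path remains disconnected, so the spline does not shape the chain.
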(fn `UserConstructionScript`
  (bind _chain_siz_x (`KismetMathLibrary.BreakVector` (`self.Chain_Siz`)))
  (bind _listofmesh (`self.ListOfMesh`))
  (bind _listofconstraints (`self.ListOfConstraints`))
  (bind (_returnvalue_min _returnvalue_max) (break `Box` (`StaticMesh.GetBoundingBox` (`self.Render Mesh`))))
  (for _array_element _listofconstraints
    (`ActorComponent.K2_DestroyComponent` _array_element))
  (`KismetArrayLibrary.Array_Clear` _listofconstraints)
  (for _array_element_2 (`self.ListOfMesh`)
    (`ActorComponent.K2_DestroyComponent` _array_element_2))
  (`KismetArrayLibrary.Array_Clear` (`self.ListOfMesh`))
  (set `self.Chain_Siz` (- _returnvalue_max _returnvalue_min))
  (for _index (range (+ (`self.ChainLength`) 1))
    (`/Engine/EditorBlueprintResources/StandardMacros.FlipFlop`
      (:`A`
        (bind _returnvalue (* _index (- _chain_siz_x 75.0)))
        (bind _returnvalue_2 (`AddComponent|NODE_AddStaticMeshComponent-0` :`RelativeTransform` (`KismetMathLibrary.MakeTransform` (`KismetMathLibrary.MakeVector` _returnvalue))))
        (`KismetArrayLibrary.Array_Add` _listofmesh _returnvalue_2))
      (:`B`
        (bind _returnvalue_3 (`AddComponent|NODE_AddStaticMeshComponent-1` :`RelativeTransform` (`KismetMathLibrary.MakeTransform` (`KismetMathLibrary.MakeVector` _returnvalue) (struct :`Roll` 90.0))))
        (`KismetArrayLibrary.Array_Add` _listofmesh _returnvalue_3)
        (set `self.Constraints?` true)))
    (if (`self.Constraints?`)
      (bind _returnvalue_4 (`AddComponent|NODE_AddPhysicsConstraintComponent-0` :`RelativeTransform` (`KismetMathLibrary.MakeTransform` (`KismetMathLibrary.MakeVector` (* _index (- _chain_siz_x 150.0))))))
      (`KismetArrayLibrary.Array_Add` (`self.ListOfConstraints`) _returnvalue_4)
      (`PhysicsConstraintComponent.SetConstrainedComponents` _returnvalue_4 null "None" null "None"))))