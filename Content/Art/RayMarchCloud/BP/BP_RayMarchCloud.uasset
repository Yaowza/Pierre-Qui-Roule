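; BP_RayMarchCloud is an actor that displays a ray-marched volumetric cloud inside a scaled cube.
; Its construction script creates a dynamic material instance, applies it to the cube and uniformly sets the cube's world scale from BoxScale.
; MaterialSettings then pushes the actor's variables into that material: volume texture, march and shadow quality, density, colors, jitter, UV scale and lighting.
; The event graph has no active logic.
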(fn `materialSettings`
  (bind _dynamicmat (`self.DynamicMat`))
  (`MaterialInstanceDynamic.SetTextureParameterValue` _dynamicmat "VolumeTexture" (`self.VolumeTexture`))
  (`MaterialInstanceDynamic.SetScalarParameterValue` _dynamicmat "Steps" (`self.Max Steps`))
  (`MaterialInstanceDynamic.SetScalarParameterValue` _dynamicmat "Density" (`self.Cloud Density`))
  (`MaterialInstanceDynamic.SetScalarParameterValue` _dynamicmat "ShadowSteps" (`self.Shadow Steps`))
  (`MaterialInstanceDynamic.SetScalarParameterValue` _dynamicmat "ShadowDensity" (`self.Shadow Density`))
  (`MaterialInstanceDynamic.SetScalarParameterValue` _dynamicmat "ShadowThreshold" (`self.Shadow Threshold`))
  (`MaterialInstanceDynamic.SetVectorParameterValue` _dynamicmat "Sun Color" (`self.Cloud Color`))
  (`MaterialInstanceDynamic.SetVectorParameterValue` _dynamicmat "Sky Color" (`self.Sky Color`))
  (`MaterialInstanceDynamic.SetScalarParameterValue` _dynamicmat "Ambient Density" (`self.Ambient Density`))
  (`MaterialInstanceDynamic.SetScalarParameterValue` _dynamicmat "Jitter" (`self.Jitter`))
  (`MaterialInstanceDynamic.SetScalarParameterValue` _dynamicmat "AlignPlanes" (`self.AlignPlanes`))
  (`MaterialInstanceDynamic.SetVectorParameterValue` _dynamicmat "UvScale" (`KismetMathLibrary.Conv_VectorToLinearColor` (`self.UVScale`)))
  (`MaterialInstanceDynamic.SetScalarParameterValue` _dynamicmat "DistanceFieldShadowSteps" (`self.DistanceFieldShadowSteps`))
  (`MaterialInstanceDynamic.SetScalarParameterValue` _dynamicmat "LightTangent" (`self.LightTangent`)))

(fn `UserConstructionScript`
  (bind _box_scale (`self.Box Scale`))
  (bind _cube (`self.Cube`))
  (bind _returnvalue (`KismetMaterialLibrary.CreateDynamicMaterialInstance` (`self.Mat`)))
  (bind _output_get (set `self.DynamicMat` _returnvalue))
  (`PrimitiveComponent.SetMaterial` _cube 0 _output_get)
  (`SceneComponent.SetWorldScale3D` _cube (`KismetMathLibrary.MakeVector` _box_scale _box_scale _box_scale))
  (`self.materialSettings`))