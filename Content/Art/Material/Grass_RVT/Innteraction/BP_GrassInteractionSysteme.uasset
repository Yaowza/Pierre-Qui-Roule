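; Grass interaction actor that writes a trail of its owner pawn into the MC_GrassInteraction parameter collection, presumably for grass materials.
; A looping timer cycles six trail slots, writing stored location with a game-time stamp, plus velocity.
; Tick computes velocity but overwrites it with the foot-level location, and PawnLocation is only set at BeginPlay.
; BeginPlay writes radius, falloff and timescale values all to TrailTimescale, and starts a DrawDebugTrail timer.
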(event `self.ReceiveBeginPlay`
  (bind _returnvalue (`ActorComponent.GetOwner` (`self.Target`)))
  (`/Engine/EditorBlueprintResources/StandardMacros.IsValid` _returnvalue
    (:`Is Valid`
      (set `self.PawnLocation` (`self.K2_GetActorLocation` _returnvalue))
      (set `self.PawnVelocity` (0.0 0.0 0.0))
      (`KismetMaterialLibrary.SetScalarParameterValue` "/Game/Art/Material/Grass_RVT/Innteraction/MC_GrassInteraction.MC_GrassInteraction" "TrailTimescale" (`self.ParticuleRaduis`))
      (`KismetMaterialLibrary.SetScalarParameterValue` "/Game/Art/Material/Grass_RVT/Innteraction/MC_GrassInteraction.MC_GrassInteraction" "TrailTimescale" (`self.ParticuleRaduisFalloff`))
      (`KismetMaterialLibrary.SetScalarParameterValue` "/Game/Art/Material/Grass_RVT/Innteraction/MC_GrassInteraction.MC_GrassInteraction" "TrailTimescale" (/ (* (`self.ParticuleSpawnRate`) 0.0) 1.0))
      (`KismetSystemLibrary.K2_SetTimer` null "IncrementTrailParticules" (`self.ParticuleSpawnRate`) true)
      (if true
        (`KismetSystemLibrary.K2_SetTimer` null "DrawDebugTrail" (`self.ParticuleSpawnRate`) true)))))

(event `self.ReceiveTick`
  (params (DeltaSeconds :type "Float (single-precision)"))
  (`self.UpdateTrailParticules` DeltaSeconds))

(fn `IncrementTrailParticules`
  (bind _this_string (`self.This String`))
  (set `self.Particule index` (mod (+ (`self.Particule index`) 1) 6))
  (set `self.This String` (`KismetStringLibrary.Concat_StrStr` "Trail" (`KismetStringLibrary.Conv_IntToString` (+ (`self.Particule index`) 1))))
  (`KismetMaterialLibrary.SetVectorParameterValue` "/Game/Art/Material/Grass_RVT/Innteraction/MC_GrassInteraction.MC_GrassInteraction" (`KismetStringLibrary.Conv_StringToName` (`KismetStringLibrary.Concat_StrStr` _this_string "Location")) (make `LinearColor` (.x (`self.PawnLocation`)) (.y (`self.PawnLocation`)) (.z (`self.PawnLocation`)) (`KismetSystemLibrary.GetGameTimeInSeconds`)))
  (`KismetMaterialLibrary.SetVectorParameterValue` "/Game/Art/Material/Grass_RVT/Innteraction/MC_GrassInteraction.MC_GrassInteraction" (`KismetStringLibrary.Conv_StringToName` (`KismetStringLibrary.Concat_StrStr` _this_string "Velocity")) (make `LinearColor` (.x (`self.PawnVelocity`)) (.y (`self.PawnVelocity`)) (.z (`self.PawnVelocity`))))
  (return))

(fn `UpdateTrailParticules`
  (params (Deltatime :type "Float (double-precision)"))
  (bind _output_get (set `self.This owner` (`ActorComponent.GetOwner` (`self.Target`))))
  (set `self.This Location` (- (`self.K2_GetActorLocation` _output_get) (`KismetMathLibrary.MakeVector` 0.0 0.0 (`self.PawnHalfheight`))))
  (set `self.PawnVelocity` (/ (- (`self.PawnLocation`) (`self.This Location`)) Deltatime))
  (set `self.PawnVelocity` (`self.This Location`))
  (return))

(fn `UserConstructionScript`)