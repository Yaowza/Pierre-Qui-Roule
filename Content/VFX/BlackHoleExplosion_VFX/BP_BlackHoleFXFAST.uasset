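; BP_BlackHoleFXFAST is a self-destroying effect actor that plays the fast black hole explosion.
; BeginPlay randomises the "RingAxe" vector on the Goute effect, then waits briefly before detonating.
; Detonation spawns the slash-explosion Niagara system and BP_BlackHoleTiny with sound, camera shake, a brief post-process impact frame, timeline-driven chromatic aberration and an achievement push.
; The trace and falling-sweep intro is disconnected and never runs.
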(event `self.ReceiveBeginPlay`
  (bind _returnvalue (`self.K2_GetActorLocation`))
  ;[0.195 1 0] Ring Axis Randomise
  (if (`KismetMathLibrary.RandomBool`)
    (`|ExecutionSequence`
      (:`then_0`
        (set `self.X` (`KismetMathLibrary.RandomFloatInRange` 0.0 1.0)))
      (:`then_1`
        (if (`KismetMathLibrary.RandomBool`) :!label _label
          (`|ExecutionSequence`
            (:`then_0`
              (set `self.Y` (`KismetMathLibrary.RandomFloatInRange` 0.0 1.0)))
            (:`then_1`
              (if (`KismetMathLibrary.RandomBool`) :!label _label_2
                (`|ExecutionSequence`
                  (:`then_0`
                    (set `self.Z` (`KismetMathLibrary.RandomFloatInRange` 0.0 1.0)))
                  (:`then_1`
                    (`NiagaraComponent.SetVariableVec3` (`self.Goute`) "RingAxe" (`KismetMathLibrary.MakeVector` (`self.X`) (`self.Y`) (`self.Z`)) :!label _label_3)
                    (`KismetSystemLibrary.Delay` 2.1)
                    (`|ExecutionSequence`
                      (:`then_0`
                        ;[0 1 0.9767] Final Explsion
                        (`NiagaraFunctionLibrary.SpawnSystemAtLocation` "/Game/VFX/BlackHoleExplosion_VFX/NiagaraSystems/NS_SlashExplosionFAST.NS_SlashExplosionFAST" _returnvalue)
                        (`|SpawnActorFromClass` "/Game/VFX/TrouNoir/BP_BlackHoleTiny.BP_BlackHoleTiny_C" (`KismetMathLibrary.MakeTransform` _returnvalue (struct) (0.21 0.21 0.21)) "Undefined" "MultiplyWithRoot" null null)
                        (`GameplayStatics.PlaySound2D` "/Game/Audio/Sounds/SFX/Impact/SFXBLKHOLE.SFXBLKHOLE" 1.3 1.0 0.0 null null)
                        (`|ExecutionSequence`
                          (:`then_0`
                            ;[0 0 0] Impact Frame effect
                            (set `PostProcessComponent.bEnabled` true (`self.PostProcess`))
                            (`KismetSystemLibrary.Delay` 0.38)
                            (set `PostProcessComponent.bEnabled` false (`self.PostProcess`))
                            (`KismetSystemLibrary.Delay` 15.0)
                            (`self.K2_DestroyActor`))
                          (:`then_1`
                            (`TimelineComponent.SetPlayRate` (`self.Chromatic aberation`) (/ 1.0 2.0))
                            ;[0 1 0.1697] Chromatic aberration
                            (bind (_direction _newtrack_0) (`Timeline|Chromatic aberation` :!via `PlayFromStart`)
                              (:`Update`
                                (set `PostProcessComponent.Settings` (make `PostProcessSettings` :`SceneFringeIntensity` (* _newtrack_0 10.0)) (`self.PostProcess1`)))))
                          (:`then_2`
                            (`/Game/Blueprint/BFL_Rock.PushAchievement` 2))))
                      (:`then_1`
                        ;[0 0.3733 1] Shake Screen
                        (`GameplayStatics.PlayWorldCameraShake` "/Game/VFX/CameraShakes/Explosion.Explosion_C" _returnvalue 1000.0 50000.0)))))
                (else
                  (goto _label_3)))))
          (else
            (goto _label_2)))))
    (else
      (goto _label))))

(fn `UserConstructionScript`)