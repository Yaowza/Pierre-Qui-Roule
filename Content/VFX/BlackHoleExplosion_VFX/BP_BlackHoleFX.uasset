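; BP_BlackHoleFX is a self-destroying actor that sequences a falling black hole explosion effect.
; On BeginPlay it randomizes the Goute effect's ring axis, waits, then uses a downward trace and timeline to drop to a point above the hit.
; There it spawns sparkles, removes Goute, then spawns the slash explosion and BP_BlackHoleBig.
; A briefly enabled post-process creates an impact frame while a second timeline drives chromatic aberration.
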(event `self.ReceiveBeginPlay`
  (bind _returnvalue (`self.K2_GetActorLocation`))
  ;[0.195 1 0] Ring Axis Randomise
  (if (`KismetMathLibrary.RandomBool`)
    (`|ExecutionSequence`
      (:`then_0`
        (set `self.X` (`KismetMathLibrary.RandomFloatInRange` 0.0 1.0)))
      (:`then_1`
        (if (`KismetMathLibrary.RandomBool`) :!label _label
          (`|ExecutionSequence`
            (:`then_0`
              (set `self.Y` (`KismetMathLibrary.RandomFloatInRange` 0.0 1.0)))
            (:`then_1`
              (if (`KismetMathLibrary.RandomBool`) :!label _label_2
                (`|ExecutionSequence`
                  (:`then_0`
                    (set `self.Z` (`KismetMathLibrary.RandomFloatInRange` 0.0 1.0)))
                  (:`then_1`
                    (`NiagaraComponent.SetVariableVec3` (`self.Goute`) "RingAxe" (`KismetMathLibrary.MakeVector` (`self.X`) (`self.Y`) (`self.Z`)) :!label _label_3)
                    (`KismetSystemLibrary.Delay` 5.7)
                    ;[0.7798 1 0] Determine VFX fall distance and duration
                    (bind _outhit (`KismetSystemLibrary.LineTraceSingle` _returnvalue (- _returnvalue (0.0 0.0 10000000.0)) "TraceTypeQuery1"))
                    (set `self.LocStart` (`self.K2_GetActorLocation`))
                    (bind (_direction _sweep) (`Timeline|Sweep` :!via `PlayFromStart`)
                      (:`Update`
                        (bind _returnvalue_2 (+ (`.Location` (`GameplayStatics.BreakHitResult` _outhit)) (0.0 0.0 1200.0)))
                        (`self.K2_SetActorLocation` (`KismetMathLibrary.VLerp` (`self.LocStart`) _returnvalue_2 _sweep)))
                      (:`Finished`
                        ;[0 1 0.9606] 1st sparkle spawn
                        (`NiagaraFunctionLibrary.SpawnSystemAtLocation` "/Game/VFX/BlackHoleExplosion_VFX/NiagaraSystems/Sparkles.Sparkles" _returnvalue_2)
                        (`ActorComponent.K2_DestroyComponent` (`self.Goute`))
                        (`KismetSystemLibrary.Delay` 1.5)
                        (`|ExecutionSequence`
                          (:`then_0`
                            ;[0 1 0.9767] Final Explsion
                            (`NiagaraFunctionLibrary.SpawnSystemAtLocation` "/Game/VFX/BlackHoleExplosion_VFX/NiagaraSystems/NS_SlashExplosion.NS_SlashExplosion" _returnvalue_2)
                            (`|SpawnActorFromClass` "/Game/VFX/TrouNoir/BP_BlackHoleBig.BP_BlackHoleBig_C" (`KismetMathLibrary.MakeTransform` _returnvalue_2) "Undefined" "MultiplyWithRoot" null null)
                            (`|ExecutionSequence`
                              (:`then_0`
                                ;[0 0 0] Impact Frame effect
                                (set `PostProcessComponent.bEnabled` true (`self.PostProcess`))
                                (`KismetSystemLibrary.Delay` 0.38)
                                (set `PostProcessComponent.bEnabled` false (`self.PostProcess`))
                                (`KismetSystemLibrary.Delay` 15.0)
                                (`self.K2_DestroyActor`))
                              (:`then_1`
                                ;[0 1 0.1697] Chromatic aberration
                                (bind (_direction_2 _newtrack_0) (`Timeline|Chromatic aberation` :!via `PlayFromStart`)
                                  (:`Update`
                                    (set `PostProcessComponent.Settings` (make `PostProcessSettings` :`SceneFringeIntensity` _newtrack_0) (`self.PostProcess1`))))))))))))
                (else
                  (goto _label_3)))))
          (else
            (goto _label_2)))))
    (else
      (goto _label))))

(fn `UserConstructionScript`)