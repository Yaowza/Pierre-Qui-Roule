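; Short-lived moss particle actor that flies from a Start component to a Target component, with lost and gain sounds, then destroys itself.
; On BeginPlay it takes a random rotation, moves to Start and drifts toward a random nearby point at a randomized interp speed.
; After a second it homes on Target while shrinking toward zero scale.
; Looping timers drive the VInterpTo movement and scaling instead of Tick.
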(event `self.ReceiveBeginPlay`
  (`KismetSystemLibrary.DelayUntilNextTick`)
  (`self.K2_SetActorRotation` (`KismetMathLibrary.RandomRotator` true))
  (`self.K2_SetActorLocation` (`SceneComponent.K2_GetComponentLocation` (`self.Start`)))
  (set `self.Interp Speed` (`KismetMathLibrary.RandomFloatInRange` 2.5 5.0))
  (set `self.TargetLoc` (+ (* (`KismetMathLibrary.RandomUnitVector`) 1000.0) (`SceneComponent.K2_GetComponentLocation` (`self.Start`))))
  (bind _returnvalue (`KismetSystemLibrary.K2_SetTimer` null "MovingParticle" 0.01 true true))
  (`GameplayStatics.PlaySoundAtLocation` "/Game/Audio/Sounds/SFX/Moss/SC_MossLost.SC_MossLost" (`self.K2_GetActorLocation`) (struct) 1.0 1.0 0.0 null null null null)
  (`KismetSystemLibrary.Delay` 1.0)
  (`KismetSystemLibrary.K2_ClearAndInvalidateTimerHandle` _returnvalue)
  (set `self.Lerp?` true)
  (bind _returnvalue_2 (`KismetSystemLibrary.K2_SetTimer` null "MovingParticle" 0.01 true true))
  (bind _returnvalue_3 (`KismetSystemLibrary.K2_SetTimer` null "UpdateScale" 0.01 true true))
  (`KismetSystemLibrary.Delay` 0.5)
  (`GameplayStatics.PlaySoundAtLocation` "/Game/Audio/Sounds/SFX/Moss/SC_MossGain.SC_MossGain" (`self.K2_GetActorLocation`) (struct) 1.0 1.0 0.0 null null null null)
  (`KismetSystemLibrary.Delay` 0.5)
  (`KismetSystemLibrary.K2_ClearAndInvalidateTimerHandle` _returnvalue_2)
  (`KismetSystemLibrary.K2_ClearAndInvalidateTimerHandle` _returnvalue_3)
  (`self.K2_DestroyActor`))

(fn `MovingParticle`
  (if (`self.Lerp?`)
    (set `self.TargetLoc` (`SceneComponent.K2_GetComponentLocation` (`self.Target`))))
  (`self.K2_SetActorLocation` (`KismetMathLibrary.VInterpTo` (`self.K2_GetActorLocation`) (`self.TargetLoc`) (`GameplayStatics.GetWorldDeltaSeconds`) (`self.Interp Speed`))))

(fn `UpdateScale`
  (`self.SetActorScale3D` (`KismetMathLibrary.VInterpTo` (`self.GetActorScale3D`) (0.0 0.0 0.0) (`GameplayStatics.GetWorldDeltaSeconds`) (`self.Interp Speed`))))

(fn `UserConstructionScript`)