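; Construction-script scatter tool that places random rock meshes along a spline.
; On each construction it clears the old components and creates one Hierarchical Instanced Static Mesh component per mesh in the Rocks array.
; It then adds up to RocksNumber instances to randomly picked components, at random spline positions with ranged rotation and uniform scale.
; All randomness draws from a single random stream.
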(fn `UserConstructionScript`
  (bind _stream (`self.Stream`))
  (bind (_outitem _outindex) (`KismetArrayLibrary.Array_RandomFromStream` (`self.HISM_List`) (`self.Stream`)))
  (for _array_element (`self.HISM_List`)
    (`ActorComponent.K2_DestroyComponent` _array_element))
  (`KismetArrayLibrary.Array_Clear` (`self.HISM_List`))
  (for _array_element_2 (`self.Rocks`)
    (bind _returnvalue (`AddComponent|NODE_AddHierarchicalInstancedStaticMeshComponent-0`))
    (`/Engine/EditorBlueprintResources/StandardMacros.IsValid` _returnvalue
      (:`Is Valid`
        (`KismetArrayLibrary.Array_Add` (`self.HISM_List`) _returnvalue)
        (`StaticMeshComponent.SetStaticMesh` _returnvalue _array_element_2))))
  (for _ (range (`self.Rocks_Number`))
    (`/Engine/EditorBlueprintResources/StandardMacros.IsValid` _outitem
      (:`Is Valid`
        (`InstancedStaticMeshComponent.AddInstance` _outitem (`KismetMathLibrary.MakeTransform` (`SplineComponent.GetLocationAtTime` (`self.Spline`) (`KismetMathLibrary.RandomFloatInRangeFromStream` (`self.Stream`) 0.0 1.0) "Local" false) (`KismetMathLibrary.MakeRotator` (`KismetMathLibrary.RandomFloatInRangeFromStream` _stream (`self.X MinRotation`) (`self.X_MaxRotation`)) (`KismetMathLibrary.RandomFloatInRangeFromStream` _stream (`self.Y MinRotation`) (`self.YMaxRotation`)) (`KismetMathLibrary.RandomFloatInRangeFromStream` _stream (`self.Z MinRotation`) (`self.Z MaxRotation`))) (`KismetMathLibrary.Conv_DoubleToVector` (`KismetMathLibrary.RandomFloatInRangeFromStream` _stream (`self.2_Scale Min`) (`self.2_Scale Max`)))) false)))))