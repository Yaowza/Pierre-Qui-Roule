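; BP_Foliage is a procedural foliage clump actor that builds a cluster of skeletal mesh plants, such as ferns.
; Its Construction Script adds a configurable number of SkeletalMeshComponents, all using the Foliage mesh.
; Each component gets a random rotation within per-axis limits and a random uniform scale, with no position offset, so the plants fan out from the actor origin.
; Unseeded randomness reshuffles the layout whenever construction reruns; the event graph is unused.
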(fn `UserConstructionScript`
  (locals (NewLocalVar :type "Actor Object Reference"))
  (for _ (range (`self.Fern_Number`))
    (bind _returnvalue (`AddComponent|NODE_AddSkeletalMeshComponent-1` :`RelativeTransform` (`KismetMathLibrary.MakeTransform` (0.0 0.0 0.0) (`KismetMathLibrary.MakeRotator` (`KismetMathLibrary.RandomFloatInRange` (`self.X MinRotation`) (`self.X_MaxRotation`)) (`KismetMathLibrary.RandomFloatInRange` (`self.Y MinRotation`) (`self.YMaxRotation`)) (`KismetMathLibrary.RandomFloatInRange` (`self.Z MinRotation`) (`self.Z MaxRotation`))) (`KismetMathLibrary.Conv_DoubleToVector` (`KismetMathLibrary.RandomFloatInRange` (`self.Scale Min`) (`self.Scale Max`))))))
    (`SkeletalMeshComponent.SetSkeletalMeshAsset` _returnvalue (`self.Foliage`))))