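; Moss character test actor that builds a moss-covered body with a face in the Construction Script, with no active event logic.
; A dynamic face material sets eye and mouth textures on the scaled static mesh.
; The moss HISM is rebuilt by scattering instances on random unit vectors, at a radius from a reference mesh's bounds, with rotations derived from random directions.
; Scale-based culling and alternative distributions, including a golden-angle sphere, remain unconnected.
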(fn `UserConstructionScript`
  (locals (i :type Integer) (x :type "Float (double-precision)") (r :type "Float (double-precision)") (A :type "Float (double-precision)") (z :type "Float (double-precision)") (y :type "Float (double-precision)") (Loc :type "Vector Structure") (u :type "Float (double-precision)") (T :type "Float (double-precision)"))
  (bind _staticmesh (`self.StaticMesh`))
  (bind _returnvalue (* (`KismetMathLibrary.RandomUnitVector`) (`local.r`)))
  (bind (_returnvalue_min _returnvalue_max) (break `Box` (`StaticMesh.GetBoundingBox` (`StaticMeshComponent.StaticMesh` (`self.SM_PersoMOSSonly`)))))
  (bind (_returnvalue_roll _returnvalue_pitch _returnvalue_yaw) (`KismetMathLibrary.BreakRotator` (`KismetMathLibrary.MakeRotFromZ` (- _returnvalue (0.0 0.0 0.0)))))
  (bind _returnvalue_x (`KismetMathLibrary.BreakVector` (* (- _returnvalue_max _returnvalue_min) (`self.radmult`))))
  (bind _returnvalue_2 (`KismetMaterialLibrary.CreateDynamicMaterialInstance` "/Game/Art/Material/Face/M_Face.M_Face"))
  (set `self.FaceMaterial` _returnvalue_2)
  (`MaterialInstanceDynamic.SetTextureParameterValue` (`self.FaceMaterial`) "eyes_texture" "/Game/Art/Material/Face/e_none.e_none")
  (`MaterialInstanceDynamic.SetTextureParameterValue` (`self.FaceMaterial`) "mouth_texture" "/Game/Art/Material/Face/m_happy.m_happy")
  (`PrimitiveComponent.SetMaterial` (`self.StaticMesh`) 0 (`self.FaceMaterial`))
  (`StaticMeshComponent.SetStaticMesh` (`self.HISM_Moss`) (`self.MossMesh`))
  (`SceneComponent.SetRelativeScale3D` _staticmesh (* (`SceneComponent.RelativeScale3D` _staticmesh) (`self.FaceScale`)))
  (`InstancedStaticMeshComponent.ClearInstances` (`self.HISM_Moss`))
  (for _index (range (`self.Mousse`))
    (set `local.i` _index)
    (set `local.r` _returnvalue_x)
    (`InstancedStaticMeshComponent.AddInstance` (`self.HISM_Moss`) (`KismetMathLibrary.MakeTransform` _returnvalue (`KismetMathLibrary.MakeRotator` _returnvalue_roll _returnvalue_pitch _returnvalue_yaw) (* (1.0 1.0 1.0) (`self.hismscale`))) false)))