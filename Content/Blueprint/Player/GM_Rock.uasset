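; Game mode that tracks achievements, per-level moss scores and best times, and pushes them to PQR_HUD.
; Achievement states are sized from DT_Achievements rows; each unlocks once by index, showing its name and icon.
; A looping timer drives a minutes/seconds chrono, saved on stop.
; Score and timer updates write into the current level's entry in the Levels array, replacing its time only when the saved one is faster.
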(event `self.ReceiveBeginPlay`
  (`self.Init Achievements`))

(event `Init Achievements`
  (bind _outrownames (`DataTableFunctionLibrary.GetDataTableRowNames` "/Game/Blueprint/Achievements/DT_Achievements.DT_Achievements"))
  (for _ _outrownames
    (`KismetArrayLibrary.Array_Add` (`self.AchievementStates`))))

(event `Push Achievement`
  (params (Index :type Integer))
  (if (and (>= Index 0) (<= Index (`KismetArrayLibrary.Array_LastIndex` (`self.AchievementStates`))))
    (if (not (`|GetArrayItem` (`self.AchievementStates`) Index))
      (`KismetArrayLibrary.Array_Set` (`self.AchievementStates`) Index true)
      (bind _outrownames (`DataTableFunctionLibrary.GetDataTableRowNames` "/Game/Blueprint/Achievements/DT_Achievements.DT_Achievements"))
      (bind _output (`|GetArrayItem` _outrownames Index))
      (bind _returnvalue (`|GetDataTableRow` "/Game/Blueprint/Achievements/DT_Achievements.DT_Achievements" _output)
        (:`then`
          (bind _aspqr_hud (cast `/Game/Blueprint/HUD/PQR_HUD` (`PlayerController.GetHUD` (`GameplayStatics.GetPlayerController` 0))))
          (`/Game/Blueprint/HUD/PQR_HUD.Achievement` _aspqr_hud (`KismetStringLibrary.Replace` (`KismetStringLibrary.Conv_NameToString` _output) "_" " ") (break `/Game/Blueprint/Achievements/F_Achievements` _returnvalue)))))))

(event `Change Level`
  (params (`Current Level` :type Integer))
  (set `self.Current Level` `Current Level`))

(event `Update Current Score`
  (params (`Player Moss Score` :type Integer))
  (bind _current_level (`self.Current Level`))
  (bind (_output_levelname _output_levelunlocked _output_levelmaxmoss _output_levelmosstounlock _output_playermossscore _output_playertimesec _output_playertimemin _output_playercurrentmoss) (break `/Game/Blueprint/Player/F_LevelData` (`|GetArrayItem` (`self.Levels`) _current_level)))
  (`KismetArrayLibrary.Array_Set` (`self.Levels`) _current_level (make `/Game/Blueprint/Player/F_LevelData` _output_levelname _output_levelunlocked _output_levelmaxmoss _output_levelmosstounlock `Player Moss Score` _output_playertimesec _output_playertimemin _output_playercurrentmoss))
  (bind _aspqr_hud (cast `/Game/Blueprint/HUD/PQR_HUD` (`PlayerController.GetHUD` (`GameplayStatics.GetPlayerController` 0))))
  (`/Game/Blueprint/HUD/PQR_HUD.Update Moss` _aspqr_hud `Player Moss Score`))

(event `UpdateTimer`
  (bind _savedtimerseconds (`self.SavedTimerSeconds`))
  (bind _savedtimerminutes (`self.SavedTimerMinutes`))
  (bind _current_level (`self.Current Level`))
  (bind (_output_levelname _output_levelunlocked _output_levelmaxmoss _output_levelmosstounlock _output_playermossscore _output_playertimesec _output_playertimemin _output_playercurrentmoss) (break `/Game/Blueprint/Player/F_LevelData` (`|GetArrayItem` (`self.Levels`) _current_level)))
  (if (> (+ (* _output_playertimemin 100) _output_playertimesec) (+ (* _savedtimerminutes 100) _savedtimerseconds))
    (`KismetArrayLibrary.Array_Set` (`self.Levels`) _current_level (make `/Game/Blueprint/Player/F_LevelData` _output_levelname _output_levelunlocked _output_levelmaxmoss _output_levelmosstounlock _output_playermossscore _savedtimerseconds _savedtimerminutes _output_playercurrentmoss)))
  (set `self.LastTimerSeconds` (`self.SavedTimerSeconds`))
  (set `self.LastTimerMinutes` (`self.SavedTimerMinutes`)))

(event `StartTimer`
  (params (DisplayTimer :type Boolean))
  (`/Game/Blueprint/HUD/PQR_HUD.DisplayTimer` (cast `/Game/Blueprint/HUD/PQR_HUD` (`PlayerController.GetHUD` (`GameplayStatics.GetPlayerController` 0)) :!pure true) DisplayTimer)
  (bind _returnvalue (`KismetSystemLibrary.K2_SetTimerDelegate` (delegate `Chrono`) 0.01 true true)))

(event `StopTimer`
  (`KismetSystemLibrary.K2_ClearAndInvalidateTimerHandle` (stale `StartTimer` _returnvalue))
  (`/Game/Blueprint/HUD/PQR_HUD.DisplayTimer` (cast `/Game/Blueprint/HUD/PQR_HUD` (`PlayerController.GetHUD` (`GameplayStatics.GetPlayerController` 0)) :!pure true) false)
  (set `self.SavedTimerSeconds` (`self.TimerSeconds`))
  (set `self.SavedTimerMinutes` (`self.TimerMinutes`))
  (set `self.TimerSeconds` 0)
  (set `self.TimerMinutes` 0)
  (set `self.Timer` 0.0))

(event `Chrono`
  (bind _timerseconds (`self.TimerSeconds`))
  (bind _timerminutes (`self.TimerMinutes`))
  (bind _timerminutes_2 (`self.TimerMinutes`))
  (bind _returnvalue (>= (`self.TimerSeconds`) 60))
  (set `self.Timer` (`KismetMathLibrary.SelectFloat` 0.0 (+ (`KismetSystemLibrary.K2_GetTimerElapsedTimeHandle` (stale `StartTimer` _returnvalue)) (`self.Timer`)) _returnvalue))
  (set `self.TimerSeconds` (`KismetMathLibrary.SelectInt` 0 (`KismetMathLibrary.FFloor` (`self.Timer`)) _returnvalue))
  (set `self.TimerMinutes` (`KismetMathLibrary.SelectInt` (+ _timerminutes_2 1) _timerminutes_2 _returnvalue))
  (`/Game/Blueprint/HUD/PQR_HUD.UpdateTextTimer` (cast `/Game/Blueprint/HUD/PQR_HUD` (`PlayerController.GetHUD` (`GameplayStatics.GetPlayerController` 0)) :!pure true) (`KismetStringLibrary.Conv_IntToString` _timerminutes) (`KismetStringLibrary.Conv_IntToString` _timerseconds))
  (`KismetSystemLibrary.PrintString` (`KismetStringLibrary.Concat_StrStr` (`KismetStringLibrary.Conv_IntToString` _timerminutes) " : " (`KismetStringLibrary.Conv_IntToString` _timerseconds) "               " (`KismetStringLibrary.Conv_DoubleToString` (`self.Timer`))) true false (struct :`G` 0.66 :`B` 1.0 :`A` 1.0) 0.0))

(fn `UserConstructionScript`)