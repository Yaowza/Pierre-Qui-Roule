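; Moss pickup that launches in an arc to a landing point, then bobs until the rock player collects it.
; Timelines drive the quadratic Bezier flight and hover, while AutoRecup instead cuts the flight short to pull it toward the player.
; Sphere overlap grants Moss once, spawning ground-shock Niagara and moss particles aimed at the rock before self-destructing.
; The construction script scatters outward-facing HISM moss instances in a spherical shell sized from the Sac mesh.
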(event `self.ReceiveBeginPlay`
  (bind (_landlocation_x _landlocation_y _landlocation_z) (`KismetMathLibrary.BreakVector` (`self.LandLocation`)))
  (bind _startlocation (`self.StartLocation`))
  (bind _landlocation (`self.LandLocation`))
  (bind (_returnvalue_x _returnvalue_y _returnvalue_z) (`KismetMathLibrary.BreakVector` (`KismetMathLibrary.VLerp` _startlocation _landlocation 0.5)))
  (`KismetSystemLibrary.Delay` (`KismetMathLibrary.RandomFloatInRange` 0.0 0.25))
  (bind (_direction _xy_alpha) (`Timeline|Timeline` :!via `PlayFromStart` :!label _label)
    (:`Update`
      (`self.K2_SetActorLocation` (`self.CurveLerp` _startlocation (`KismetMathLibrary.MakeVector` _returnvalue_x _returnvalue_y (+ _returnvalue_z 1400.0)) _landlocation _xy_alpha))
      (if (`self.AutoRecup`)
        (`|ExecutionSequence`
          (:`then_0`
            (set `self.CanBeTriggered?` true)
            (set `self.StartLocation` (`self.K2_GetActorLocation`))
            (`TimelineComponent.SetPlayRate` (`self.absorb`) (/ 1.0 2.0))
            (bind (_direction_2 _alpha) (`Timeline|absorb` :!via `PlayFromStart`)
              (:`Update`
                (`self.K2_SetActorLocation` (`KismetMathLibrary.VLerp` (`self.StartLocation`) (`SceneComponent.K2_GetComponentLocation` (`/Game/Blueprint/Player/BP_PlayerRock.GetMovingComponent` (`/Game/Blueprint/BFL_Rock.GetPlayerActorRef`))) _alpha)))))
          (:`then_1`
            (goto _label :!via `Stop`)))))
    (:`Finished`
      (set `self.CanBeTriggered?` true)
      (bind (_direction_3 _newtrack_0) (`Timeline|Timeline_0` :!via `PlayFromStart` :!label _label_2)
        (:`Update`
          (`self.K2_SetActorLocation` (`KismetMathLibrary.MakeVector` _landlocation_x _landlocation_y (`|EaseFunction` "EaseInOut" _newtrack_0 _landlocation_z (+ _landlocation_z 100.0)))))
        (:`Finished`
          (`self.DownAnim`))))))

(event `DownAnim`
  (`/Engine/EditorBlueprintResources/StandardMacros.FlipFlop`
    (:`A`
      (goto _label_2 :!via `ReverseFromEnd`))
    (:`B`
      (goto _label_2 :!via `PlayFromStart`))))

(event `self.ReceiveTick`
  (params (DeltaSeconds :type "Float (single-precision)"))
  (bind _moss (`self.moss`))
  (if (`PrimitiveComponent.IsOverlappingActor` (`self.Sphere`) (`/Game/Blueprint/BFL_Rock.GetPlayerActorRef`))
    (`/Engine/EditorBlueprintResources/StandardMacros.DoOnce` false :!label _label_3
      (:`Completed`
        (`NiagaraFunctionLibrary.SpawnSystemAtLocation` "/Game/VFX/Choc/NS_ChocGround.NS_ChocGround" (`SceneComponent.K2_GetComponentLocation` (`self.Sac`)) (struct) (/ (`self.GetActorScale3D`) 10.0))
        (`KismetSystemLibrary.PrintString` (`KismetStringLibrary.Conv_IntToString` _moss) true false (struct :`R` 0.38125 :`B` 1.0 :`A` 1.0) 10.0)
        (`/Game/Blueprint/Player/BP_PlayerRock.GainMoss` (stale `OnStay` _asbp_player_rock) _moss)
        (for _ (range (+ _moss 1))
          (`|SpawnActorFromClass` "/Game/Blueprint/BP_MossParticle.BP_MossParticle_C" (`KismetMathLibrary.MakeTransform` (0.0 0.0 0.0)) "AlwaysSpawn" "MultiplyWithRoot" null (`/Game/Blueprint/Player/BP_PlayerRock.SM_Rock` (`/Game/Blueprint/BFL_Rock.GetPlayerActorRef`)) (`self.Sac`) null))
        (`KismetSystemLibrary.DelayUntilNextTick`)
        (`KismetSystemLibrary.DelayUntilNextTick`)
        (`self.K2_DestroyActor`)))))

(event `OnStay`
  (if (`self.CanStay?`)
    (if (`self.CanBeTriggered?`) :!label _label_4
      (bind _asbp_player_rock (cast `/Game/Blueprint/Player/BP_PlayerRock` (stale `self.Sphere.OnComponentBeginOverlap` OtherActor))
        (:`then`
          (goto _label_3))
        (:`CastFailed`
          (`KismetSystemLibrary.DelayUntilNextTick`)
          (`self.OnStay`)))
      (else
        (`KismetSystemLibrary.DelayUntilNextTick`)
        (`self.OnStay`)))))

(event `self.Sphere.OnComponentBeginOverlap`
  (params (OverlappedComponent :type "PrimitiveComponent Object Reference") (OtherActor :type "Actor Object Reference") (OtherComp :type "PrimitiveComponent Object Reference") (OtherBodyIndex :type Integer) (bFromSweep :type Boolean) (SweepResult :type "HitResult Structure (by ref)"))
  (set `self.CanStay?` true)
  (goto _label_4))

(event `self.Sphere.OnComponentEndOverlap`
  (params (OverlappedComponent :type "PrimitiveComponent Object Reference") (OtherActor :type "Actor Object Reference") (OtherComp :type "PrimitiveComponent Object Reference") (OtherBodyIndex :type Integer))
  (cast `/Game/Blueprint/Player/BP_PlayerRock` OtherActor)
  (set `self.CanStay?` false))

(fn `CurveLerp`
  (params (A :type "Vector Structure") (B :type "Vector Structure") (C :type "Vector Structure") (Alpha :type "Float (single-precision)"))
  (returns (ReturnValue :type "Vector Structure"))
  (return (`|EaseFunction` "Linear" Alpha (`KismetMathLibrary.VLerp` A B Alpha) (`KismetMathLibrary.VLerp` B C Alpha))))

(fn `UserConstructionScript`
  (bind _returnvalue (* (`KismetMathLibrary.RandomUnitVector`) (`self.r`)))
  (bind (_returnvalue_min _returnvalue_max) (break `Box` (`StaticMesh.GetBoundingBox` (`StaticMeshComponent.StaticMesh` (`self.Sac`)))))
  (bind (_returnvalue_roll _returnvalue_pitch _returnvalue_yaw) (`KismetMathLibrary.BreakRotator` (`KismetMathLibrary.MakeRotFromZ` (- _returnvalue (0.0 0.0 0.0)))))
  (bind _returnvalue_x (`KismetMathLibrary.BreakVector` (* (- _returnvalue_max _returnvalue_min) (`self.radmult`))))
  (`InstancedStaticMeshComponent.ClearInstances` (`self.HISM_Moss`))
  (for _ (range (`self.Mousse`))
    (set `self.r` _returnvalue_x)
    (`InstancedStaticMeshComponent.AddInstance` (`self.HISM_Moss`) (`KismetMathLibrary.MakeTransform` _returnvalue (`KismetMathLibrary.MakeRotator` _returnvalue_roll _returnvalue_pitch _returnvalue_yaw) (* (1.0 1.0 1.0) (`self.hismscale`))) false)))