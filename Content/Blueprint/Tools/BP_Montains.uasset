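; BP_Montains is a construction-script tool actor that scatters a seeded random set of mountain meshes within a box sized by Radius and Height.
; On construction, with valid inputs, it destroys its previous HISM components and creates one per entry in StaticMeshes.
; A random stream picks the mountain count, then each instance's component, position from a box centered on the actor location, and uniform scale, leaving rotation at default.
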(fn `UserConstructionScript`
  (bind _radius (`self.Radius`))
  (if (and (`KismetArrayLibrary.Array_IsNotEmpty` (`self.StaticMeshes`)) (> (`self.MontainNumberMax`) 0) (> (`self.Radius`) 0.0))
    (for _array_element (`self.HISM_List`)
      (`ActorComponent.K2_DestroyComponent` _array_element))
    (`KismetArrayLibrary.Array_Clear` (`self.HISM_List`))
    (for _array_element_2 (`self.StaticMeshes`)
      (bind _returnvalue (`AddComponent|NODE_AddHierarchicalInstancedStaticMeshComponent-2`))
      (`KismetArrayLibrary.Array_Add` (`self.HISM_List`) _returnvalue)
      (`StaticMeshComponent.SetStaticMesh` _returnvalue _array_element_2))
    (for _ (range (+ (`KismetMathLibrary.RandomIntegerInRangeFromStream` (`self.Seed`) (`self.MontainNumberMin`) (`self.MontainNumberMax`)) 1))
      (`InstancedStaticMeshComponent.AddInstance` (`KismetArrayLibrary.Array_RandomFromStream` (`self.HISM_List`) (`self.Seed`)) (`KismetMathLibrary.MakeTransform` (`KismetMathLibrary.RandomPointInBoundingBoxFromStream` (`self.Seed`) (`self.K2_GetActorLocation`) (`KismetMathLibrary.MakeVector` _radius _radius (`self.Height`))) (struct) (`KismetMathLibrary.Conv_DoubleToVector` (`KismetMathLibrary.RandomFloatInRangeFromStream` (`self.Seed`) (`self.MinSize`) (`self.MaxSize`)))) false))))