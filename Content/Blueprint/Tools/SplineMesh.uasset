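; Spline-built mesh actor that tiles a chosen mesh along an optionally looped spline, with an optional camera that rides the spline.
; Construction adds colliding, shadowless spline mesh segments spaced by mesh Z size and places sphere triggers at the ends.
; When Cam is set, Tick eases the camera toward the spline point nearest the player's camera, facing the physics player.
; Trigger overlap events are empty; the view-toggle logic is disconnected.
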(event `self.StartTrigerBox.OnComponentBeginOverlap`
  (params (OverlappedComponent :type "PrimitiveComponent Object Reference") (OtherActor :type "Actor Object Reference") (OtherComp :type "PrimitiveComponent Object Reference") (OtherBodyIndex :type Integer) (bFromSweep :type Boolean) (SweepResult :type "HitResult Structure (by ref)")))

(event `self.EndTrigerBox.OnComponentBeginOverlap`
  (params (OverlappedComponent :type "PrimitiveComponent Object Reference") (OtherActor :type "Actor Object Reference") (OtherComp :type "PrimitiveComponent Object Reference") (OtherBodyIndex :type Integer) (bFromSweep :type Boolean) (SweepResult :type "HitResult Structure (by ref)")))

(event `self.ReceiveTick`
  (params (DeltaSeconds :type "Float (single-precision)"))
  (if (`self.cam`)
    (`|ExecutionSequence`
      (:`then_0`
        (`SceneComponent.K2_SetWorldLocationAndRotation` (`self.Camera`) (`KismetMathLibrary.VInterpTo` (`SceneComponent.K2_GetComponentLocation` (`self.Camera`)) (`SplineComponent.FindLocationClosestToWorldLocation` (`self.Spline`) (`SceneComponent.K2_GetComponentLocation` (`/Game/Blueprint/Player/BP_PlayerRock.ThirdPersonCamera` (`/Game/Blueprint/BFL_Rock.GetPlayerActorRef`))) "World") (`GameplayStatics.GetWorldDeltaSeconds`) 5.0) (`KismetMathLibrary.FindLookAtRotation` (`SceneComponent.K2_GetComponentLocation` (`self.Camera`)) (`SceneComponent.K2_GetComponentLocation` (`/Game/Blueprint/BFL_Rock.GetPhysicPlayerRef`))) false false)
        (`/Game/Blueprint/Player/BP_PlayerRock.ResetCameraRotation_Canon` (`/Game/Blueprint/BFL_Rock.GetPlayerActorRef`))))))

(fn `GetClosestPointPositionAlongSpline`
  (params (`In Location` :type "Vector Structure"))
  (returns (LengthAtClothestDistance :type "Float (double-precision)"))
  (bind _spline (`self.Spline`))
  (bind _checklength (`self.CheckLength`))
  (bind _checklength_2 (`self.CheckLength`))
  (bind _returnvalue (`KismetMathLibrary.Vector_Distance` (`SplineComponent.GetLocationAtDistanceAlongSpline` _spline _checklength "World") `In Location`))
  (if (< _checklength (`SplineComponent.GetSplineLength` _spline)) :!label _label
    (if (> (`self.ClothestDistance`) _returnvalue)
      (set `self.ClothestDistance` _returnvalue)
      (set `self.CheckLength` _checklength_2))
    (set `self.CheckLength` (+ _checklength_2 10.0))
    (goto _label)
    (else
      (return (`self.LengthAtClothestDistance`)))))

(fn `UserConstructionScript`
  (bind _spline (`self.Spline`))
  (bind _spline_2 (`self.Spline`))
  (bind _spline_3 (`self.Spline`))
  (bind _spline_4 (`self.Spline`))
  (bind (_returnvalue_min _returnvalue_max) (break `Box` (`StaticMesh.GetBoundingBox` (`self.Mesh`))))
  (bind (_returnvalue_x _returnvalue_y _returnvalue_z) (`KismetMathLibrary.BreakVector` (+ (`KismetMathLibrary.Vector_GetAbs` _returnvalue_min) (`KismetMathLibrary.Vector_GetAbs` _returnvalue_max))))
  (`SphereComponent.SetSphereRadius` (`self.StartTrigerBox`) (`self.TrigerRadius`) true)
  (`SphereComponent.SetSphereRadius` (`self.EndTrigerBox`) (`self.TrigerRadius`) true)
  (if (`self.Loop?`)
    (`SplineComponent.SetClosedLoop` _spline true true)
    (else
      (`SplineComponent.SetClosedLoop` _spline false true)))
  (bind _output_get (set `self.Xlength` _returnvalue_z))
  (for _index (range (+ (`KismetMathLibrary.FTrunc` (/ (`SplineComponent.GetSplineLength` (`self.Spline`)) _output_get)) 1))
    (bind _returnvalue (`AddComponent|NODE_AddSplineMeshComponent-0`))
    (`PrimitiveComponent.SetCollisionEnabled` _returnvalue "QueryAndPhysics")
    (`SplineMeshComponent.SetForwardAxis` _returnvalue "Z" true)
    (`StaticMeshComponent.SetStaticMesh` _returnvalue (`self.Mesh`))
    (bind _returnvalue_2 (* _index (`self.Xlength`)))
    (bind _returnvalue_3 (* (+ _index 1) (`self.Xlength`)))
    (`SplineMeshComponent.SetStartAndEnd` _returnvalue (`SplineComponent.GetLocationAtDistanceAlongSpline` _spline_4 _returnvalue_2 "Local") (`KismetMathLibrary.ClampVectorSize` (`SplineComponent.GetTangentAtDistanceAlongSpline` _spline_4 _returnvalue_2 "Local") 0.0 (`self.Xlength`)) (`SplineComponent.GetLocationAtDistanceAlongSpline` _spline_3 _returnvalue_3 "Local") (`KismetMathLibrary.ClampVectorSize` (`SplineComponent.GetTangentAtDistanceAlongSpline` _spline_3 _returnvalue_3 "Local") 0.0 (`self.Xlength`)) true)
    (`PrimitiveComponent.SetCollisionResponseToChannel` _returnvalue "ECC_Camera" "ECR_Block")
    (`PrimitiveComponent.SetCollisionResponseToChannel` _returnvalue "ECC_Visibility" "ECR_Block")
    (`PrimitiveComponent.SetCollisionResponseToChannel` _returnvalue "ECC_GameTraceChannel1" "ECR_Block")
    (`PrimitiveComponent.SetCastShadow` _returnvalue false))
  (`SceneComponent.K2_SetWorldLocation` (`self.StartTrigerBox`) (`SplineComponent.GetLocationAtSplinePoint` _spline_2 0 "World") false false)
  (`SceneComponent.K2_SetWorldLocation` (`self.EndTrigerBox`) (`SplineComponent.GetLocationAtSplinePoint` (`self.Spline`) (`SplineComponent.GetNumberOfSplinePoints` _spline_2) "World") false false))