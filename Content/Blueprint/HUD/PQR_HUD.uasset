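; PQR_HUD is the game's HUD Blueprint, a single entry point for on-screen UI and cinematic dialogue.
; On BeginPlay it creates WBP_HUD, initially hidden, and WBP_CineDialogue, then adds both to the viewport.
; Its custom events are thin forwarders: visibility, timer, tutorial text, moss count and maximum, and achievement pop-ups go to WBP_HUD, while dialogue open and close go to WBP_CineDialogue.
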(event `self.ReceiveBeginPlay`
  (bind _returnvalue (`|CreateWidget` "/Game/UI/WBP/WBP_HUD.WBP_HUD_C"))
  (bind _output_get (set `self.HUD Widget` _returnvalue))
  (`Widget.SetVisibility` _output_get "Hidden")
  (`UserWidget.AddToViewport` _output_get 0)
  (bind _returnvalue_2 (`|CreateWidget` "/Game/UI/WBP/WBP_CineDialogue.WBP_CineDialogue_C"))
  (bind _output_get_2 (set `self.CineDialogueRef` _returnvalue_2))
  (`UserWidget.AddToViewport` _output_get_2 0))

(event `OpenCineDialogue`
  (params (SetTextSpeed :type "Float (single-precision)") (InputText :type String))
  (`/Game/UI/WBP/WBP_CineDialogue.Open` (`self.CineDialogueRef`) SetTextSpeed InputText))

(event `Set Visibility`
  (params (visibility :type Boolean))
  (`Widget.SetVisibility` (`self.HUD Widget`) (select `bool` visibility :`false` "Hidden" :`true` "Visible" :!type "ESlateVisibility Enum")))

(event `DisplayTimer`
  (params (`Visible?` :type Boolean))
  (`/Game/UI/WBP/WBP_HUD.DisplayTimer` (`self.HUD Widget`) `Visible?`))

(event `UpdateTextTimer`
  (params (Mintues :type String) (Seconds :type String))
  (`/Game/UI/WBP/WBP_HUD.UpdateTextTimer` (`self.HUD Widget`) Mintues Seconds))

(event `CloseCineDialogue`
  (`/Game/UI/WBP/WBP_CineDialogue.Close` (`self.CineDialogueRef`)))

(event `Update Moss`
  (params (Quantity :type Integer))
  (`/Game/UI/WBP/WBP_HUD.Pop up Moss Update` (`self.HUD Widget`) Quantity))

(event `DisplayTuto`
  (params (`Visible?` :type Boolean))
  (`/Game/UI/WBP/WBP_HUD.DisplayTuto` (`self.HUD Widget`) `Visible?`))

(event `Set Max Moss`
  (params (Max :type Integer))
  (`/Game/UI/WBP/WBP_HUD.Pop up Moss Max` (`self.HUD Widget`) Max))

(event `SetTutoText`
  (params (InputText :type String :default "Appuie sur <img id=\"AButton\"/> pour sauter"))
  (`/Game/UI/WBP/WBP_HUD.SetTutoText` (`self.HUD Widget`) InputText))

(event `Achievement`
  (params (Name :type String) (Icon :type "Texture2D Object Reference"))
  (`/Game/UI/WBP/WBP_HUD.Pop up Achievement` (`self.HUD Widget`) Name Icon))

(fn `UserConstructionScript`)