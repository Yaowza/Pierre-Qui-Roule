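; BP_EndLevelManager runs the end-of-level sequence: blend to its camera, lock and reset the player to PlayerStart, then show WBP_EndLevel results.
; Time, best time and moss score come from GM_Rock and level data at hardcoded index 4.
; A looping timer fills the gauge with ExpoOut easing while removing player moss toward MossTarget.
; It then plays the MS_plottwistnew cinematic with the player hidden, unlocking and revealing them afterward.
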(event `self.ReceiveBeginPlay`
  (bind _returnvalue (`GameplayStatics.GetActorOfClass` "/Script/Engine.PlayerStart"))
  (set `self.PlayerStartRef` _returnvalue)
  (bind _returnvalue_2 (`|CreateWidget` "/Game/UI/WBP/WBP_EndLevel.WBP_EndLevel_C"))
  (set `self.WidgetRef` _returnvalue_2)
  (`UserWidget.AddToViewport` (`self.WidgetRef`) 0))

(event `ClearAnim`
  (bind _asbp_player_rock (`/Game/Blueprint/BFL_Rock.GetPlayerActorRef`))
  (`KismetSystemLibrary.K2_ClearAndInvalidateTimerHandle` (stale `EndLevel` _returnvalue_2))
  (set `self.Alpha` 0.0)
  (`KismetSystemLibrary.Delay` 1.0)
  (`/Game/UI/WBP/WBP_EndLevel.DisplayWidget` (`self.WidgetRef`) "" "" "" 0 0 false)
  (`KismetSystemLibrary.Delay` 0.5)
  (bind (_outactor _returnvalue) (`LevelSequencePlayer.CreateLevelSequencePlayer` "/Game/Cinematic/SEQ_2_PlotTwist/MS_plottwistnew.MS_plottwistnew"))
  (`MovieSceneSequencePlayer.Play` (`LevelSequenceActor.SequencePlayer` _outactor))
  (`self.SetActorHiddenInGame` (`/Game/Blueprint/BFL_Rock.GetPlayerActorRef`) true)
  (add `MovieSceneSequencePlayer.OnStop` _returnvalue (delegate `CineStopped`))
  (`PlayerController.SetViewTargetWithBlend` (`GameplayStatics.GetPlayerController` 0) _asbp_player_rock 0.0 "VTBlend_Linear" 0.0 false)
  (`/Game/Blueprint/Player/BP_PlayerRock.SetCurrentCameraUsed` _asbp_player_rock (`/Game/Blueprint/Player/BP_PlayerRock.ThirdPersonCamera` _asbp_player_rock)))

(event `EndLevel`
  (bind _asbp_player_rock (`/Game/Blueprint/BFL_Rock.GetPlayerActorRef`))
  (bind _playerstartref (`self.PlayerStartRef`))
  (bind (_levelname _levelunlocked _levelmaxmoss _levelmosstounlock _playermossscore _playertimesec _playertimemin) (break `/Game/Blueprint/Player/F_LevelData` (`/Game/Blueprint/BFL_Rock.Get Level Data` 4)))
  (bind _asgm_rock (cast `/Game/Blueprint/Player/GM_Rock` (`GameplayStatics.GetGameMode`) :!pure true))
  (bind _returnvalue (`KismetStringLibrary.Concat_StrStr` (`KismetStringLibrary.Conv_IntToString` (`/Game/Blueprint/Player/GM_Rock.LastTimerMinutes` _asgm_rock)) ":" (`KismetStringLibrary.Conv_IntToString` (`/Game/Blueprint/Player/GM_Rock.LastTimerSeconds` _asgm_rock))))
  (`PlayerController.SetViewTargetWithBlend` (`GameplayStatics.GetPlayerController` 0) self 1.0 "VTBlend_Linear" 0.0 false)
  (`KismetSystemLibrary.Delay` 1.25)
  (`/Game/Blueprint/Player/BP_PlayerRock.SetCurrentCameraUsed` _asbp_player_rock (`self.Camera`))
  (`/Game/Blueprint/Player/BP_PlayerRock.LockPlayer` _asbp_player_rock)
  (`SceneComponent.K2_SetWorldLocationAndRotation` (`/Game/Blueprint/BFL_Rock.GetPhysicPlayerRef`) (`self.K2_GetActorLocation` _playerstartref) (`self.K2_GetActorRotation` _playerstartref) false false)
  (`/Game/UI/WBP/WBP_EndLevel.DisplayWidget` (`self.WidgetRef`) _levelname _returnvalue (`KismetMathLibrary.SelectString` _returnvalue (`KismetStringLibrary.Concat_StrStr` (`KismetStringLibrary.Conv_IntToString` _playertimemin) ":" (`KismetStringLibrary.Conv_IntToString` _playertimesec)) (and (<= _playertimesec 0) (<= _playertimemin 0))) _playermossscore _levelmaxmoss true)
  (set `self.MossQuantity` _playermossscore)
  (`KismetSystemLibrary.Delay` 2.0)
  (bind _returnvalue_2 (`KismetSystemLibrary.K2_SetTimerDelegate` (delegate `Anim`) 0.25 true)))

(event `CineStopped`
  (bind _asbp_player_rock (`/Game/Blueprint/BFL_Rock.GetPlayerActorRef`))
  (`KismetSystemLibrary.Delay` 1.0)
  (`/Game/Blueprint/Player/BP_PlayerRock.UnlockPlayer` _asbp_player_rock)
  (`self.SetActorHiddenInGame` _asbp_player_rock false))

(event `Anim`
  (bind _mossquantity (`self.MossQuantity`))
  (set `self.Alpha` (+ (`self.Alpha`) (/ (/ _mossquantity (* (`self.AnimDuration`) (`self.StepsPerSecond`))) _mossquantity)))
  (if (>= (`self.Alpha`) 1.0)
    (`self.ClearAnim`)
    (else
      (`/Game/UI/WBP/WBP_EndLevel.SetJauge` (`self.WidgetRef`) (`|EaseFunction` "ExpoOut" (`self.Alpha`) 0.0 (`KismetMathLibrary.Conv_IntToDouble` (`self.MossQuantity`))))
      (`/Game/Blueprint/Player/BP_PlayerRock.CustomRemoveMoss` (`/Game/Blueprint/BFL_Rock.GetPlayerActorRef`) (/ (`self.MossQuantity`) (* (`self.AnimDuration`) (`self.StepsPerSecond`))) (`self.MossTarget`)))))

(fn `UserConstructionScript`)