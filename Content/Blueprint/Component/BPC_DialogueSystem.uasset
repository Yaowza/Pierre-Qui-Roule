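; Dialogue component for rock characters that can physically roam between random points around their start location.
; Interacting in range locks the player, halts roaming, turns both toward each other and shows WBP_Dialogue lines.
; A shared BP_CameraDialogue frames the pair, with randomized rotation and spring-interpolated zoom driven by looping timers.
; Ending or leaving range restores player and camera; ending can also add a follow-up component and destroy this one.
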(event `self.ReceiveBeginPlay`
  (bind (_returnvalue_min _returnvalue_max) (break `Box` (`StaticMesh.GetBoundingBox` (`StaticMeshComponent.StaticMesh` (`/Game/Blueprint/IA/BP_IARock.SM_Rock` (`self.GetParentRef`))))))
  ;[0 1 0.5794] Begin Play
  (`parent.ReceiveBeginPlay`)
  (bind _returnvalue (`GameplayStatics.GetActorOfClass` "/Game/Blueprint/BP_CameraDialogue.BP_CameraDialogue_C"))
  (set `self.ParentSize` (- _returnvalue_max _returnvalue_min))
  (set `self.StartLoc` (`Actor.K2_GetActorLocation` (`self.GetParentRef`)))
  (`/Engine/EditorBlueprintResources/StandardMacros.IsValid` _returnvalue
    (:`Is Valid`
      (set `self.CameraRef` _returnvalue))
    (:`Is Not Valid`
      (bind _returnvalue_2 (`|SpawnActorFromClass` "/Game/Blueprint/BP_CameraDialogue.BP_CameraDialogue_C" (`KismetMathLibrary.MakeTransform` (0.0 0.0 0.0)) "AlwaysSpawn" "MultiplyWithRoot" null null))
      (set `self.CameraRef` _returnvalue_2))))

(event `self.StartSystem`
  ;[1 0.2165 0.7284] Start & Stop System
  (`parent.StartSystem`)
  (set `/Game/Blueprint/IA/BP_IARock.DialogueSystemActive?` true (`self.GetParentRef`))
  (if (`self.Roaming?`)
    (`self.SetupRoaming`)))

(event `self.StopSystem`
  ;[1 0.2165 0.7284] Start & Stop System
  (`parent.StopSystem`)
  (`self.StopDialogue`)
  (set `/Game/Blueprint/IA/BP_IARock.DialogueSystemActive?` false (`self.GetParentRef`)))

(event `PlayCurrentDialogue`
  ;[1 0.2165 0.7284] Dialogue System
  ;;[1 1 1] Play Dialogue
  (`/Game/UI/WBP/WBP_Dialogue.PlayDialogue` (`self.WBP_Ref`))
  (set `self.DialogueTextIndex` (`KismetMathLibrary.SelectInt` 0 (+ (`self.DialogueTextIndex`) 1) (> (`self.DialogueTextIndex`) (- (`KismetArrayLibrary.Array_Length` (`self.Dialogue Text`)) 1))))
  (if (<= (`self.DialogueTextIndex`) 0)
    (`KismetSystemLibrary.DelayUntilNextTick`)
    (`KismetSystemLibrary.DelayUntilNextTick`)
    (`self.StopDialogue`)
    (`self.StopLookAt`)
    (`KismetSystemLibrary.PrintString` "OUT" true false (struct :`R` 1.0 :`G` 0.000994 :`A` 1.0) 10.0)
    (else
      (`KismetSystemLibrary.DelayUntilNextTick`)
      (`KismetSystemLibrary.DelayUntilNextTick`)
      (`self.ResetNextDialogue`)
      (`KismetSystemLibrary.PrintString` "NEXT" true false (struct :`R` 0.369427 :`G` 1.0 :`B` 0.164032 :`A` 1.0) 10.0))))

(event `ForceDialogue`
  ;[1 0.2165 0.7284] Dialogue System
  ;;[1 1 1] Dialogue Conditions
  (`/Engine/EditorBlueprintResources/StandardMacros.DoOnce` false :!label _label
    (:`Completed`
      (`/Game/Blueprint/Player/BP_PlayerRock.LockPlayer` (`/Game/Blueprint/BFL_Rock.GetPlayerActorRef`))
      (`self.ClearRoaming`)
      (bind _returnvalue (`KismetSystemLibrary.K2_SetTimerDelegate` (delegate `LookAt`) 0.01 true true))
      (`/Engine/EditorBlueprintResources/StandardMacros.IsValid` (`self.WBP_Ref`)
        (:`Is Valid`
          ;;[1 1 1] Update WIdget
          (set `/Game/UI/WBP/WBP_Dialogue.DialogueWrintingSpeed` (`|GetArrayItem` (`self.Dialogue Wrinting Speed`) (`self.DialogueTextIndex`)) (`self.WBP_Ref`))
          (set `/Game/UI/WBP/WBP_Dialogue.DialogueText` (`|GetArrayItem` (`self.Dialogue Text`) (`self.DialogueTextIndex`)) (`self.WBP_Ref`))
          (`self.PlayCurrentDialogue`)
          (`self.STartUpdateCamera`))
        (:`Is Not Valid`
          ;;[1 1 1] Create Widget
          (bind _returnvalue_2 (`|CreateWidget` "/Game/UI/WBP/WBP_Dialogue.WBP_Dialogue_C" (`GameplayStatics.GetPlayerController` 0) (`|GetArrayItem` (`self.Dialogue Wrinting Speed`) (`self.DialogueTextIndex`)) (`|GetArrayItem` (`self.Dialogue Text`) (`self.DialogueTextIndex`)) (`self.SpeakerName`)))
          (set `self.WBP_Ref` _returnvalue_2)
          (`UserWidget.AddToViewport` (`self.WBP_Ref`) 0)
          (`self.PlayCurrentDialogue`)
          (`self.PlayCamera`))))))

(event `self.PlayerInRange`
  ;[1 0.2165 0.7284] Dialogue System
  ;;[1 1 1] Dialogue Conditions
  (`parent.PlayerInRange`)
  (if (`/Game/Blueprint/Player/BP_PlayerRock.GetInteracted?` (`/Game/Blueprint/BFL_Rock.GetPlayerActorRef`))
    (goto _label)
    (else
      ;;[1 1 1] Remove Widget
      (`/Engine/EditorBlueprintResources/StandardMacros.DoOnce` false :!label _label_2
        (:`Completed`
          (`/Game/Blueprint/Player/BP_PlayerRock.UnlockPlayer` (`/Game/Blueprint/BFL_Rock.GetPlayerActorRef`) :!label _label_3)
          (set `self.ShouldRoam?` true)
          (`self.Roaming`)
          (`/Engine/EditorBlueprintResources/StandardMacros.IsValid` (`self.WBP_Ref`)
            (:`Is Valid`
              (`Widget.RemoveFromParent` (`self.WBP_Ref`))
              (set `self.WBP_Ref` (`self.WBP_Invalid`))
              (`self.StopCamera`)
              (`KismetSystemLibrary.Delay` 1.5)
              (`self.ResetNextDialogue`))
            (:`Is Not Valid`
              (`KismetSystemLibrary.Delay` 1.5)
              (`self.ResetNextDialogue`))))))))

(event `ResetNextDialogue`
  ;[1 0.2165 0.7284] Dialogue System
  ;;[1 1 1] Dialogue Conditions
  (goto _label :!via `Reset`))

(event `StopLookAt`
  ;[1 0.2165 0.7284] Dialogue System
  (`KismetSystemLibrary.K2_ClearAndInvalidateTimerHandle` (stale `ForceDialogue` _returnvalue)))

(event `StopDialogue`
  ;[1 0.2165 0.7284] Dialogue System
  ;;[1 1 1] Remove Widget
  (`self.ResetRemoveDialogue`)
  (`self.EndDialogueEvent`)
  (goto _label_2))

(event `self.PlayerOutRange`
  ;[1 0.2165 0.7284] Dialogue System
  ;;[1 1 1] Remove Widget
  (`parent.PlayerOutRange`)
  (`/Engine/EditorBlueprintResources/StandardMacros.IsValid` (`self.WBP_Ref`)
    (:`Is Valid`
      (`self.ResetRemoveDialogue`)
      (set `self.DialogueTextIndex` (- (`self.DialogueTextIndex`) 1))
      (goto _label_2))))

(event `STartUpdateCamera`
  ;[1 0.2165 0.7284] Dialogue System
  ;;[1 1 1] Camera
  (`self.ClearUpdateCamera`)
  (set `self.CameraTargetRotation` (`KismetMathLibrary.MakeRotator` 0.0 0.0 (`KismetMathLibrary.RandomFloatInRange` 0.0 359.0)) :!label _label_4)
  (set `self.CameraUpdateRotationSpeed` (`KismetMathLibrary.RandomFloatInRange` 0.1 2.0))
  (set `self.CameraZoom` (`KismetMathLibrary.RandomFloatInRange` 30.0 60.0))
  (bind _returnvalue (`KismetSystemLibrary.K2_SetTimerDelegate` (delegate `UpdateCamera`) 0.01 true)))

(event `ResetRemoveDialogue`
  ;[1 0.2165 0.7284] Dialogue System
  ;;[1 1 1] Remove Widget
  (goto _label_2 :!via `Reset`))

(event `PlayCamera`
  (bind _returnvalue (`SceneComponent.K2_GetComponentLocation` (`/Game/Blueprint/BFL_Rock.GetPhysicPlayerRef`)))
  (bind _returnvalue_2 (`SceneComponent.K2_GetComponentLocation` (`.CollisionShape` (`self.GetParentRef`))))
  ;[1 0.2165 0.7284] Dialogue System
  ;;[1 1 1] Camera
  (set `self.DialogueOriginLoc` (+ (/ (+ _returnvalue_2 _returnvalue) 2.0) (0.0 0.0 1000.0)))
  (`Actor.K2_SetActorLocation` (`self.CameraRef`) (`self.DialogueOriginLoc`) false false)
  (set `SpringArmComponent.TargetArmLength` (+ (* (`KismetMathLibrary.Vector_Distance` _returnvalue_2 _returnvalue) 4.0) (`KismetMathLibrary.VSize` (`self.ParentSize`))) (`/Game/Blueprint/BP_CameraDialogue.SpringArm` (`self.CameraRef`)))
  (`PlayerController.SetViewTargetWithBlend` (`GameplayStatics.GetPlayerController` 0) (`self.CameraRef`) 0.5 "VTBlend_Linear" 0.0 false)
  (`/Game/Blueprint/Player/BP_PlayerRock.SetCurrentCameraUsed` (`/Game/Blueprint/BFL_Rock.GetPlayerActorRef`) (`/Game/Blueprint/BP_CameraDialogue.CineCamera` (`self.CameraRef`)))
  (goto _label_4))

(event `ClearUpdateCamera`
  ;[1 0.2165 0.7284] Dialogue System
  ;;[1 1 1] Camera
  (`KismetSystemLibrary.K2_ClearAndInvalidateTimerHandle` (stale `STartUpdateCamera` _returnvalue)))

(event `UpdateCamera`
  (bind _cameraref (`self.CameraRef`))
  (bind _cinecamera (`/Game/Blueprint/BP_CameraDialogue.CineCamera` (`self.CameraRef`)))
  (bind _cinecamera_2 (`/Game/Blueprint/BP_CameraDialogue.CineCamera` _cameraref))
  ;[1 0.2165 0.7284] Dialogue System
  ;;[1 1 1] Camera
  ;;;[1 1 1] Camera Animation
  (`Actor.K2_SetActorRotation` (`self.CameraRef`) (`KismetMathLibrary.RInterpTo` (`Actor.K2_GetActorRotation` (`self.CameraRef`)) (`self.CameraTargetRotation`) (`GameplayStatics.GetWorldDeltaSeconds`) (`self.CameraUpdateRotationSpeed`)) false)
  (set `CineCameraComponent.FocusSettings` (make `CameraFocusSettings` "Manual" (`KismetMathLibrary.Vector_Distance` (`self.DialogueOriginLoc`) (`SceneComponent.K2_GetComponentLocation` (`/Game/Blueprint/BP_CameraDialogue.CineCamera` (`self.CameraRef`)))) (struct :`RelativeOffset` (0.0 0.0 0.0)) true) _cinecamera)
  (bind _returnvalue (`KismetMathLibrary.FloatSpringInterp` (`CineCameraComponent.CurrentFocalLength` _cinecamera) (`self.CameraZoom`) (make `FloatSpringState`) 30.0 0.1 (`GameplayStatics.GetWorldDeltaSeconds`) 2.5))
  (set `CineCameraComponent.CurrentFocalLength` _returnvalue (`/Game/Blueprint/BP_CameraDialogue.CineCamera` (`self.CameraRef`)))
  (`SceneComponent.K2_SetWorldRotation` _cinecamera_2 (`KismetMathLibrary.FindLookAtRotation` (`SceneComponent.K2_GetComponentLocation` _cinecamera_2) (`SceneComponent.K2_GetComponentLocation` (`/Game/Blueprint/BP_CameraDialogue.SpringArm` _cameraref))) false false))

(event `EndDialogueEvent`
  ;[1 0.2165 0.7284] Dialogue System
  ;;[1 1 1] End Dialogue Event
  (if (`KismetSystemLibrary.IsValidClass` (`self.ComponentToAdd`))
    (`|AddComponentByClass` (`self.GetParentRef`) (`self.ComponentToAdd`))
    (`|ExecutionSequence`
      (:`then_0`
        (goto _label_3))
      (:`then_1`
        (`KismetSystemLibrary.Delay` 1.0)
        (`self.K2_DestroyComponent`)))))

(event `StopCamera`
  (bind _asbp_player_rock (`/Game/Blueprint/BFL_Rock.GetPlayerActorRef`))
  (bind _cameraref (`self.CameraRef`))
  ;[1 0.2165 0.7284] Dialogue System
  ;;[1 1 1] Camera
  ;;;[1 1 1] ClearCamera
  (`self.ClearUpdateCamera`)
  (`PlayerController.SetViewTargetWithBlend` (`GameplayStatics.GetPlayerController` 0) (`/Game/Blueprint/BFL_Rock.GetPlayerActorRef`) 0.5 "VTBlend_Linear" 0.0 false)
  (`KismetSystemLibrary.Delay` 0.6)
  (`/Game/Blueprint/Player/BP_PlayerRock.SetCurrentCameraUsed` _asbp_player_rock (`/Game/Blueprint/Player/BP_PlayerRock.ThirdPersonCamera` _asbp_player_rock))
  (`Actor.K2_SetActorLocationAndRotation` :`self` _cameraref)
  (`SceneComponent.K2_SetRelativeLocationAndRotation` :`self` (`/Game/Blueprint/BP_CameraDialogue.CineCamera` _cameraref)))

(event `LookAt`
  (bind (_parentref _collisionshape) (`self.GetParentRef`))
  (bind _movingcomponent (`/Game/Blueprint/BFL_Rock.GetPhysicPlayerRef`))
  (bind _lookatspeed (`self.LookAtSpeed`))
  ;[1 0.2165 0.7284] Dialogue System
  ;;[1 1 1] LookAt
  (`SceneComponent.K2_SetWorldRotation` (`/Game/Blueprint/BFL_Rock.GetPhysicPlayerRef`) (`KismetMathLibrary.RInterpTo` (`SceneComponent.K2_GetComponentRotation` _movingcomponent) (`KismetMathLibrary.FindLookAtRotation` (`SceneComponent.K2_GetComponentLocation` _movingcomponent) (`SceneComponent.K2_GetComponentLocation` (`.CollisionShape` (`self.GetParentRef`)))) (`GameplayStatics.GetWorldDeltaSeconds`) _lookatspeed) false false)
  (`SceneComponent.K2_SetWorldRotation` (`.CollisionShape` (`self.GetParentRef`)) (`KismetMathLibrary.RInterpTo` (`SceneComponent.K2_GetComponentRotation` _collisionshape) (`KismetMathLibrary.FindLookAtRotation` (`SceneComponent.K2_GetComponentLocation` _collisionshape) (`SceneComponent.K2_GetComponentLocation` (`/Game/Blueprint/BFL_Rock.GetPhysicPlayerRef`))) (`GameplayStatics.GetWorldDeltaSeconds`) _lookatspeed) false false)
  (`KismetSystemLibrary.Delay` 1.5)
  (`self.StopLookAt`))

(event `SetupRoaming`
  (bind (_parentref _collisionshape) (`self.GetParentRef`))
  ;[1 0.2177 0.738] Roaming
  (`PrimitiveComponent.SetLinearDamping` _collisionshape 1.0)
  (`PrimitiveComponent.SetSimulatePhysics` _collisionshape true)
  (`PrimitiveComponent.SetPhysicsLinearVelocity` _collisionshape (0.0 0.0 0.0) false "None")
  (set `self.ShouldRoam?` true)
  (`self.Roaming`))

(event `ResetRoaming`
  ;[1 0.2177 0.738] Roaming
  (if (`self.Roaming?`)
    (`KismetSystemLibrary.K2_ClearAndInvalidateTimerHandle` (stale `Roaming` _returnvalue) :!label _label_5)))

(event `ClearRoaming`
  (bind (_parentref _collisionshape) (`self.GetParentRef`))
  ;[1 0.2177 0.738] Roaming
  (if (`self.Roaming?`)
    (`PrimitiveComponent.SetPhysicsLinearVelocity` _collisionshape (0.0 0.0 0.0) false "None")
    (`PrimitiveComponent.SetPhysicsAngularVelocityInRadians` _collisionshape (0.0 0.0 0.0) false "None")
    (set `self.ShouldRoam?` false)
    (goto _label_5)))

(event `Roaming`
  (bind _roamingradius (`self.RoamingRadius`))
  ;[1 0.2177 0.738] Roaming
  (if (and (`self.ShouldRoam?`) (`self.Roaming?`))
    (set `self.RoamingTarget` (`KismetMathLibrary.RandomPointInBoundingBox` (`self.StartLoc`) (`KismetMathLibrary.MakeVector` _roamingradius _roamingradius 100.0)))
    (bind _returnvalue (`KismetSystemLibrary.K2_SetTimerDelegate` (delegate `Moving`) 0.01 true true))))

(event `Moving`
  (bind (_parentref _collisionshape) (`self.GetParentRef`))
  (bind _roamingtarget (`self.RoamingTarget`))
  (bind _roamingspeed (`self.RoamingSpeed`))
  (bind _returnvalue (`SceneComponent.K2_GetComponentLocation` _collisionshape))
  (bind (_returnvalue_x _returnvalue_y) (`KismetMathLibrary.BreakVector` (`KismetMathLibrary.GetDirectionUnitVector` _returnvalue _roamingtarget)))
  ;[1 0.2177 0.738] Roaming
  (`PrimitiveComponent.AddForce` _collisionshape (`KismetMathLibrary.MakeVector` (* _returnvalue_x _roamingspeed) (* _returnvalue_y _roamingspeed)) "None" false)
  (if (not (and (== _returnvalue _roamingtarget :`ErrorTolerance` 250.0) (`self.Roaming?`)))
    (`KismetSystemLibrary.Delay` 3.0))
  (`self.ResetRoaming`)
  (`KismetSystemLibrary.DelayUntilNextTick`)
  (`self.Roaming`))