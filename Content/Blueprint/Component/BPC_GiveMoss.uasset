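; Actor component for BP_IARock that hands the rock's moss to the player and then swaps in its next-dialogue rock.
; On BeginPlay it passes the moss quantity through the player's Damage call from the rock's collision location, then removes it from the rock.
; After a one-second delay, any valid NextDialogueRef rock teleports to this rock's collision transform, and this rock moves to that rock's former location.
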(event `self.ReceiveBeginPlay`
  (bind _new_rock (`self.New_Rock`))
  (bind _collision_shape (`self.Collision Shape`))
  (bind _asbp_iarock (cast `/Game/Blueprint/IA/BP_IARock` (`self.GetOwner`)))
  (set `self.Collision Shape` (`/Game/Blueprint/IA/BP_IARock.CollisionShape` _asbp_iarock))
  (bind _nextdialogueref (`/Game/Blueprint/IA/BP_IARock.NextDialogueRef` _asbp_iarock))
  (`/Engine/EditorBlueprintResources/StandardMacros.IsValid` _nextdialogueref
    (:`Is Valid`
      (set `self.New_Rock` _nextdialogueref)
      (set `self.InRot` (`SceneComponent.K2_GetComponentRotation` _collision_shape))
      (set `self.InLoc` (`SceneComponent.K2_GetComponentLocation` _collision_shape))
      (set `self.OutLoc` (`Actor.K2_GetActorLocation` (`self.New_Rock`))))
    (:`Is Not Valid`
      _))
  (set `self.Moss Quantity` (`/Game/Blueprint/IA/BP_IARock.MossQuantity` _asbp_iarock))
  (`/Game/Blueprint/Player/BP_PlayerRock.Damage` (`/Game/Blueprint/BFL_Rock.GetPlayerActorRef`) (`self.Moss Quantity`) (`SceneComponent.K2_GetComponentLocation` (`self.Collision Shape`)) false)
  (`/Game/Blueprint/IA/BP_IARock.RemoveMoss` _asbp_iarock (`self.Moss Quantity`))
  (`KismetSystemLibrary.Delay` 1.0)
  (`/Engine/EditorBlueprintResources/StandardMacros.IsValid` _new_rock
    (:`Is Valid`
      (`Actor.K2_SetActorLocation` _new_rock (`self.InLoc`) false false)
      (`Actor.K2_SetActorRotation` _new_rock (`self.InRot`) false)
      (`Actor.K2_SetActorLocation` _asbp_iarock (`self.OutLoc`) false false))))