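; BPC_Bubble is a component that gives its parent actor speech-bubble dialogue, with optional roaming.
; Range events show intro/outro text and interact prompts, and register interactions with the player by distance.
; Dialogue feeds each line's text, speed and face to WBP_Bubble, optionally looping, and can add components as one-time events.
; Looping timers drive physics-force roaming toward random points, turning to face the player, and easing back to the start rotation.
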(event `self.ReceiveBeginPlay`
  (bind _parentref (`self.GetParentRef`))
  ;[0 1 0.5794] Begin Play
  (`parent.ReceiveBeginPlay`)
  (`SceneComponent.SetHiddenInGame` (`.WBP_Bubble` (`self.GetBubble`)) true false)
  (set `self.StartLoc` (`Actor.K2_GetActorLocation` _parentref))
  (set `self.StartRot` (`Actor.K2_GetActorRotation` _parentref)))

(event `self.StartSystem`
  ;[1 0.2165 0.7284] Start & Stop System
  (`parent.StartSystem`)
  (set `/Game/Blueprint/IA/BP_IARock.DialogueSystemActive?` true (`self.GetParentRef`))
  (if (`self.Roaming?`)
    (`self.SetupRoaming`)))

(event `self.StopSystem`
  ;[1 0.2165 0.7284] Start & Stop System
  (`parent.StopSystem`)
  (`self.StopDialogue`)
  (set `/Game/Blueprint/IA/BP_IARock.DialogueSystemActive?` false (`self.GetParentRef`)))

(event `SkipDialgue`
  (bind _dialoguetextindex (`self.DialogueTextIndex`))
  ;[1 0.2165 0.7284] Dialogue System
  ;;[1 1 1] Play Dialogue
  (if (== _dialoguetextindex 0) :!label _label
    (switch `int` (`self.FlipFlop`)
      (:`0`
        (set `self.FlipFlop` 1)
        (set `self.DialogueTextIndex` (`KismetMathLibrary.SelectInt` 0 (+ _dialoguetextindex 1) (> (`self.DialogueTextIndex`) (- (`KismetArrayLibrary.Array_Length` (`self.Dialogue Text`)) 2))) :!label _label_2)
        (`self.ResetNextDialogue`))
      (:`1`
        (set `self.FlipFlop` 0)
        (if (`self.LoopText`)
          (`self.TrueEndDialogue`)
          (goto _label_2)
          (else
            (`self.IntroOutro` (- (`KismetArrayLibrary.Array_Length` (`self.Intro_Outro_Text`)) 1))
            (set `self.DialogueEnded` true)
            (`KismetSystemLibrary.Delay` 2.0)
            (`self.StopLookAt`)
            (`self.ResetRotaTimer`)
            (`SceneComponent.SetHiddenInGame` (`.WBP_Bubble` (`self.GetBubble`)) true false)
            (`KismetSystemLibrary.Delay` 2.0)
            (set `self.DialogueEnded` false)
            (`self.ResetSetup once`)))))
    (else
      (goto _label_2))))

(event `PlayCurrentDialogue`
  ;[1 0.2165 0.7284] Dialogue System
  ;;[1 1 1] Play Dialogue
  (`/Game/UI/WBP/WBP_Bubble.PlayDialogue` (`self.GetBubble`))
  (goto _label))

(event `self.PlayerInRange`
  (bind _parentref (`self.GetParentRef`))
  ;[1 0.2165 0.7284] Dialogue System
  ;;[1 1 1] Dialogue Conditions
  (`parent.PlayerInRange`)
  (if (not (`self.DialogueEnded`))
    (`|ExecutionSequence`
      (:`then_0`
        ;;; Distance
        (if (<= (`/Game/Blueprint/IA/BP_IARock.GetDistanceToPlayer` (`self.GetParentRef`)) (`self.InteractionRadius`))
          (`/Game/UI/WBP/WBP_Bubble.DisplayInteract` (`self.GetBubble`) true)
          (if (`/Game/Blueprint/Player/BP_PlayerRock.GetInteracted?` (`/Game/Blueprint/BFL_Rock.GetPlayerActorRef`))
            (`BlueprintMapLibrary.Map_Add` (`/Game/Blueprint/Player/BP_PlayerRock.NewDialogueDistance` (`/Game/Blueprint/BFL_Rock.GetPlayerActorRef`)) _parentref (`/Game/Blueprint/IA/BP_IARock.GetDistanceToPlayer` _parentref))
            (`/Engine/EditorBlueprintResources/StandardMacros.DoOnce` false :!label _label_3
              (:`Completed`
                (`|ExecutionSequence`
                  (:`then_1`
                    (`self.ResetOutRangeOnce`))))))
          (else
            (`/Engine/EditorBlueprintResources/StandardMacros.DoOnce` true :!label _label_4
              (:`Completed`
                (`|ExecutionSequence`
                  (:`then_0`
                    (goto _label_3 :!via `Reset`))
                  (:`then_1`
                    (if (`self.LoopText`)
                      (`self.IntroOutro` (- (`KismetArrayLibrary.Array_Length` (`self.Intro_Outro_Text`)) 1))
                      (set `self.DialogueTextIndex` 0)))))))))
      (:`then_1`
        (`/Engine/EditorBlueprintResources/StandardMacros.DoOnce` false :!label _label_5
          (:`Completed`
            (set `self.DialogueTextIndex` 0)
            (`self.IntroOutro` 0)
            (set `self.Lerp` 0.0)
            (`self.ResetNextDialogue`)
            (set `self.FlipFlop` 0)
            (`SceneComponent.SetHiddenInGame` (`.WBP_Bubble` (`self.GetBubble`)) false false)
            (goto _label_8 :!via `Reset`)))))))

(event `ResetRotaTimer`
  ;[1 0.2165 0.7284] Dialogue System
  ;;[1 1 1] Play Dialogue
  (bind _returnvalue (`KismetSystemLibrary.K2_SetTimerDelegate` (delegate `RersetRota`) 0.02 true true)))

(event `ResetOutRangeOnce`
  ;[1 0.2165 0.7284] Dialogue System
  ;;[1 1 1] Dialogue Conditions
  (goto _label_4 :!via `Reset`))

(event `ResetSetup once`
  ;[1 0.2165 0.7284] Dialogue System
  ;;[1 1 1] Dialogue Conditions
  (goto _label_5 :!via `Reset`))

(event `Dialogue`
  (bind _aswbp_bubble (`self.GetBubble`))
  (bind (_aswbp_bubble_2 _wbp_bubble) (`self.GetBubble`))
  (bind _dialoguetextindex (`self.DialogueTextIndex`))
  (bind _output (`|GetArrayItem` (`self.Dialogue Text`) (`self.DialogueTextIndex`)))
  ;[1 0.2165 0.7284] Dialogue System
  (if (not (`self.DialogueEnded`)) :!label _label_6
    (`/Engine/EditorBlueprintResources/StandardMacros.DoOnce` false :!label _label_7
      (:`Completed`
        (set `self.Intro_Outro_Index` 1)
        (`self.ResetOutRangeOnce`)
        (`self.ClearRoaming`)
        (`self.EndDialogueEvent`)
        (if (`self.ShouldLookAt?`)
          (bind _returnvalue (`KismetSystemLibrary.K2_SetTimerDelegate` (delegate `LookAt`) 0.01 true true)))
        (set `/Game/UI/WBP/WBP_Bubble.DialogueWrintingSpeed` (`|GetArrayItem` (`self.Dialogue Wrinting Speed`) (`self.DialogueTextIndex`)) _aswbp_bubble)
        (set `/Game/UI/WBP/WBP_Bubble.DialogueText` _output _aswbp_bubble)
        (`/Game/Blueprint/IA/BP_IARock.SetFace` (`self.GetParentRef`) (`|GetArrayItem` (`self.Eye_Dialogue`) _dialoguetextindex) (`|GetArrayItem` (`self.Mouth_Dialogue`) _dialoguetextindex) true)
        (if (`KismetStringLibrary.IsEmpty` _output)
          (`SceneComponent.SetHiddenInGame` _wbp_bubble true false)
          (`self.SkipDialgue`)
          (else
            (`SceneComponent.SetHiddenInGame` _wbp_bubble false false)
            (`self.PlayCurrentDialogue`)))))))

(event `ForceDialogue`
  ;[1 0.2165 0.7284] Dialogue System
  (goto _label_6))

(event `RersetRota`
  (bind (_parentref _collisionshape) (`self.GetParentRef`))
  (bind _startrot (`self.StartRot`))
  ;[1 0.2165 0.7284] Dialogue System
  ;;[1 1 1] Play Dialogue
  (set `self.Lerp` (+ (`self.Lerp`) 0.05))
  (if (== (`SceneComponent.K2_GetComponentRotation` _collisionshape) _startrot :`ErrorTolerance` 10.0)
    (`KismetSystemLibrary.K2_ClearAndInvalidateTimerHandle` (stale `ResetRotaTimer` _returnvalue))
    (else
      (`SceneComponent.K2_SetWorldRotation` _collisionshape (`KismetMathLibrary.RLerp` (`self.ActualRot`) _startrot (`self.Lerp`) true) false false))))

(event `ResetNextDialogue`
  ;[1 0.2165 0.7284] Dialogue System
  (goto _label_7 :!via `Reset`))

(event `StopLookAt`
  ;[1 0.2165 0.7284] Dialogue System
  (`KismetSystemLibrary.K2_ClearAndInvalidateTimerHandle` (stale `Dialogue` _returnvalue)))

(event `self.PlayerOutRange`
  ;[1 0.2165 0.7284] Dialogue System
  ;;[1 1 1] Remove Widget
  (`parent.PlayerOutRange`)
  (`/Engine/EditorBlueprintResources/StandardMacros.DoOnce` false :!label _label_8
    (:`Completed`
      (`SceneComponent.SetHiddenInGame` (`.WBP_Bubble` (`self.GetBubble`)) true false)
      (`self.StopLookAt`)
      (`self.ResetRotaTimer`)
      (set `self.ShouldRoam?` true)
      (`self.Roaming`)
      (`self.ResetOutRangeOnce`)
      (goto _label_5 :!via `Reset`))))

(event `EndDialogueEvent`
  ;[1 0.2165 0.7284] Dialogue System
  ;;[1 1 1] End Dialogue Event
  (`/Engine/EditorBlueprintResources/StandardMacros.DoOnce` false
    (:`Completed`
      (if (`KismetSystemLibrary.IsValidClass` (`self.ComponentToAdd`))
        (`|AddComponentByClass` (`self.GetParentRef`) (`self.ComponentToAdd`))))))

(event `TrueEndDialogue`
  ;[1 0.2165 0.7284] Dialogue System
  (`/Engine/EditorBlueprintResources/StandardMacros.DoOnce` false
    (:`Completed`
      (if (`KismetSystemLibrary.IsValidClass` (`self.EndComponentToAdd`))
        (`|AddComponentByClass` (`self.GetParentRef`) (`self.EndComponentToAdd`))))))

(event `StopDialogue`
  ;[1 0.2165 0.7284] Dialogue System
  ;;[1 1 1] Remove Widget
  (goto _label_8))

(event `LookAt`
  (bind (_parentref _collisionshape) (`self.GetParentRef`))
  (bind _returnvalue (`KismetMathLibrary.RInterpTo` (`SceneComponent.K2_GetComponentRotation` _collisionshape) (`KismetMathLibrary.FindLookAtRotation` (`SceneComponent.K2_GetComponentLocation` _collisionshape) (`SceneComponent.K2_GetComponentLocation` (`/Game/Blueprint/BFL_Rock.GetPhysicPlayerRef`))) (`GameplayStatics.GetWorldDeltaSeconds`) (`self.LookAtSpeed`)))
  ;[1 0.2165 0.7284] Dialogue System
  ;;[1 1 1] LookAt
  (`SceneComponent.K2_SetWorldRotation` (`.CollisionShape` (`self.GetParentRef`)) _returnvalue false false)
  (set `self.ActualRot` _returnvalue))

(event `SetupRoaming`
  (bind (_parentref _collisionshape) (`self.GetParentRef`))
  ;[1 0.2177 0.738] Roaming
  (`PrimitiveComponent.SetLinearDamping` _collisionshape 1.0)
  (`PrimitiveComponent.SetSimulatePhysics` _collisionshape true)
  (`PrimitiveComponent.SetPhysicsLinearVelocity` _collisionshape (0.0 0.0 0.0) false "None")
  (set `self.ShouldRoam?` true)
  (`self.Roaming`))

(event `ResetRoaming`
  ;[1 0.2177 0.738] Roaming
  (if (`self.Roaming?`)
    (`KismetSystemLibrary.K2_ClearAndInvalidateTimerHandle` (stale `Roaming` _returnvalue) :!label _label_9)))

(event `ClearRoaming`
  (bind (_parentref _collisionshape) (`self.GetParentRef`))
  ;[1 0.2177 0.738] Roaming
  (if (`self.Roaming?`)
    (`PrimitiveComponent.SetPhysicsLinearVelocity` _collisionshape (0.0 0.0 0.0) false "None")
    (`PrimitiveComponent.SetPhysicsAngularVelocityInRadians` _collisionshape (0.0 0.0 0.0) false "None")
    (set `self.ShouldRoam?` false)
    (goto _label_9)))

(event `Roaming`
  (bind _roamingradius (`self.RoamingRadius`))
  ;[1 0.2177 0.738] Roaming
  (if (and (`self.ShouldRoam?`) (`self.Roaming?`))
    (set `self.RoamingTarget` (`KismetMathLibrary.RandomPointInBoundingBox` (`self.StartLoc`) (`KismetMathLibrary.MakeVector` _roamingradius _roamingradius 100.0)))
    (bind _returnvalue (`KismetSystemLibrary.K2_SetTimerDelegate` (delegate `Moving`) 0.01 true true))))

(event `Moving`
  (bind (_parentref _collisionshape) (`self.GetParentRef`))
  (bind _roamingtarget (`self.RoamingTarget`))
  (bind _roamingspeed (`self.RoamingSpeed`))
  (bind _returnvalue (`SceneComponent.K2_GetComponentLocation` _collisionshape))
  (bind (_returnvalue_x _returnvalue_y) (`KismetMathLibrary.BreakVector` (`KismetMathLibrary.GetDirectionUnitVector` _returnvalue _roamingtarget)))
  ;[1 0.2177 0.738] Roaming
  (`PrimitiveComponent.AddForce` _collisionshape (`KismetMathLibrary.MakeVector` (* _returnvalue_x _roamingspeed) (* _returnvalue_y _roamingspeed)) "None" false)
  (if (not (and (== _returnvalue _roamingtarget :`ErrorTolerance` 250.0) (`self.Roaming?`)))
    (`KismetSystemLibrary.Delay` 3.0))
  (`self.ResetRoaming`)
  (`KismetSystemLibrary.DelayUntilNextTick`)
  (`self.Roaming`))

(fn `GetBubble`
  (returns (`AsWBP Bubble` :type "/Game/UI/WBP/WBP_Bubble Object Reference") (WBP_Bubble :type "WidgetComponent Object Reference"))
  (bind _wbp_bubble (`/Game/Blueprint/IA/BP_IARock.WBP_Bubble` (`self.GetParentRef`)))
  (return (cast `/Game/UI/WBP/WBP_Bubble` (`WidgetComponent.GetWidget` _wbp_bubble) :!pure true) _wbp_bubble))

(fn `IntroOutro`
  (params (Intro_Outro_Index :type Integer))
  (bind (_aswbp_bubble _wbp_bubble) (`self.GetBubble`))
  (bind _output (`|GetArrayItem` (`self.Intro_Outro_Text`) (`self.Intro_Outro_Index`)))
  (bind _returnvalue (`KismetStringLibrary.IsEmpty` _output))
  (set `self.Intro_Outro_Index` Intro_Outro_Index)
  (`/Game/UI/WBP/WBP_Bubble.DisplayInteract` (`self.GetBubble`) false)
  (set `/Game/UI/WBP/WBP_Bubble.DialogueWrintingSpeed` (`|GetArrayItem` (`self.Intro_Outro_Speed`) (`self.Intro_Outro_Index`)) _aswbp_bubble)
  (set `/Game/UI/WBP/WBP_Bubble.DialogueText` _output _aswbp_bubble)
  (if _returnvalue
    (`SceneComponent.SetHiddenInGame` _wbp_bubble true false)
    (else
      (`SceneComponent.SetHiddenInGame` _wbp_bubble _returnvalue false)
      (`/Game/UI/WBP/WBP_Bubble.PlayDialogue` _aswbp_bubble)))
  (return))