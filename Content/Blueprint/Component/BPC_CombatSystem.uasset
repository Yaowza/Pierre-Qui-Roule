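; Combat behavior component for an enemy that chases the player when in range, toggled by starting and stopping the system.
; In range, it pushes the owner's physics collision shape toward the player, with force scaled between min and max combat speed by its moss quantity.
; DoOnce gates register it in the player's combat pool and fire exclamation VFX and aggro sound.
; Leaving range, stopping or the ignore flag removes it; leaving or ignoring also raises damping.
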(event `self.ReceiveBeginPlay`
  ;[0 1 0.5794] Begin Play
  (`parent.ReceiveBeginPlay`))

(event `self.StartSystem`
  ;[1 0.2165 0.7284] Start & Stop Component
  (`parent.StartSystem`)
  (set `/Game/Blueprint/IA/BP_IARock.CombatSystemActive?` true (`self.GetParentRef`)))

(event `self.StopSystem`
  ;[1 0.2165 0.7284] Start & Stop Component
  (`parent.StopSystem`)
  (set `/Game/Blueprint/IA/BP_IARock.CombatSystemActive?` false (`self.GetParentRef`))
  (`self.StopCombatPool`))

(event `self.PlayerInRange`
  (bind _parentref (`self.GetParentRef`))
  (bind _collisionshape (`/Game/Blueprint/IA/BP_IARock.CollisionShape` (`self.GetParentRef`)))
  (bind _returnvalue (`SceneComponent.K2_GetComponentLocation` _collisionshape))
  (bind (_returnvalue_x _returnvalue_y) (`KismetMathLibrary.BreakVector` (* (`KismetMathLibrary.Normal` (`KismetMathLibrary.GetDirectionUnitVector` _returnvalue (`SceneComponent.K2_GetComponentLocation` (`/Game/Blueprint/BFL_Rock.GetPhysicPlayerRef`)))) (`KismetMathLibrary.MapRangeClamped` (`KismetMathLibrary.Conv_IntToDouble` (`/Game/Blueprint/IA/BP_IARock.MossQuantity` _parentref)) 0.0 (`KismetMathLibrary.Conv_IntToDouble` (`/Game/Blueprint/IA/BP_IARock.MaxMossQuantity` _parentref)) (`self.CombatSpeedMin`) (`self.CombatSpeedMax`)))))
  ;[1 0.2165 0.7284] CombatSystem
  ;;[1 1 1] Player In
  (`parent.PlayerInRange`)
  (if (`self.Ignore?`)
    (`/Game/Blueprint/Player/BP_PlayerRock.UpdateCombatPool` (`/Game/Blueprint/BFL_Rock.GetPlayerActorRef`) false (`/Game/Blueprint/IA/BP_IARock.CollisionShape` (`self.GetParentRef`)))
    (`PrimitiveComponent.SetLinearDamping` (`/Game/Blueprint/IA/BP_IARock.CollisionShape` (`self.GetParentRef`)) 2.5)
    (`self.ResetPlayerInRange`)
    (else
      (`|ExecutionSequence`
        (:`then_0`
          (`/Engine/EditorBlueprintResources/StandardMacros.DoOnce` false :!label _label
            (:`Completed`
              (if (not (`SceneComponent.IsSimulatingPhysics` (`/Game/Blueprint/IA/BP_IARock.CollisionShape` (`self.GetParentRef`)) "None"))
                (`PrimitiveComponent.SetSimulatePhysics` (`/Game/Blueprint/IA/BP_IARock.CollisionShape` (`self.GetParentRef`)) true))
              (`/Game/Blueprint/Player/BP_PlayerRock.UpdateCombatPool` (`/Game/Blueprint/BFL_Rock.GetPlayerActorRef`) true (`/Game/Blueprint/IA/BP_IARock.CollisionShape` (`self.GetParentRef`)))
              (`self.ResetPlayerOutRange`)
              (`PrimitiveComponent.SetLinearDamping` (`/Game/Blueprint/IA/BP_IARock.CollisionShape` (`self.GetParentRef`)) 0.1)
              (`self.Activate` (`/Game/Blueprint/IA/BP_IARock.NS_Exclamation` (`self.GetParentRef`)) true))))
        (:`then_1`
          (`PrimitiveComponent.AddForce` _collisionshape (`KismetMathLibrary.MakeVector` _returnvalue_x _returnvalue_y) "None" false))
        (:`then_2`
          (`/Engine/EditorBlueprintResources/StandardMacros.DoOnce` false :!label _label_2
            (:`Completed`
              (`GameplayStatics.PlaySoundAtLocation` "/Game/Audio/Sounds/SFX/SC_EnnemyAggro.SC_EnnemyAggro" _returnvalue (struct) 1.0 1.0 0.0 null null null null))))))))

(event `ResetPlayerInRange`
  ;[1 0.2165 0.7284] CombatSystem
  ;;[1 1 1] Player In
  (goto _label :!via `Reset`))

(event `StopCombatPool`
  ;[1 0.2165 0.7284] CombatSystem
  ;;[1 1 1] PlayerOut
  (`/Game/Blueprint/Player/BP_PlayerRock.UpdateCombatPool` (`/Game/Blueprint/BFL_Rock.GetPlayerActorRef`) false (`/Game/Blueprint/IA/BP_IARock.CollisionShape` (`self.GetParentRef`)) :!label _label_3)
  (`self.ResetPlayerInRange`))

(event `self.PlayerOutRange`
  ;[1 0.2165 0.7284] CombatSystem
  ;;[1 1 1] PlayerOut
  (`parent.PlayerOutRange`)
  (`|ExecutionSequence`
    (:`then_0`
      (`/Engine/EditorBlueprintResources/StandardMacros.DoOnce` false :!label _label_4
        (:`Completed`
          (goto _label_3))))
    (:`then_1`
      (`PrimitiveComponent.SetLinearDamping` (`/Game/Blueprint/IA/BP_IARock.CollisionShape` (`self.GetParentRef`)) 2.5))
    (:`then_2`
      (goto _label_2 :!via `Reset`))))

(event `ResetPlayerOutRange`
  ;[1 0.2165 0.7284] CombatSystem
  ;;[1 1 1] PlayerOut
  (goto _label_4 :!via `Reset`))