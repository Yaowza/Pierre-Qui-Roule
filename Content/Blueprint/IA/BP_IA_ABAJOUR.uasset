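; Lampshade actor, going by its name, that jitters by randomly twisting its CollisionShape component.
; Tick runs the parent logic, then a random Delay of up to a tenth of a second spaces the twists irregularly.
; Each twist sets an absolute world rotation with a small random yaw around zero and no pitch or roll, overriding any placed orientation of that component.
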(event `self.ReceiveTick`
  (params (DeltaSeconds :type "Float (single-precision)"))
  (`parent.ReceiveTick` DeltaSeconds)
  (`KismetSystemLibrary.Delay` (`KismetMathLibrary.RandomFloatInRange` 0.0 0.1))
  (`SceneComponent.K2_SetWorldRotation` (`self.CollisionShape`) (`KismetMathLibrary.MakeRotator` 0.0 0.0 (`KismetMathLibrary.RandomFloatInRange` -5.0 5.0)) false false))

(fn `UserConstructionScript`
  (`parent.UserConstructionScript`))