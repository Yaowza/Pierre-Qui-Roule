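; AI rock character with an animated face that physically rolls to an objective, notifies its house of entering or leaving, then destroys itself.
; A looping timer drives velocity; the Jesus variant instead ascends with halo FX after a delay, while Canon skips movement.
; Construction scales body, moss, face and ground trace from MossQuantity, with separate Boss ranges.
; A tick sphere trace feeds rolling smoke and audio.
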(event `self.ReceiveBeginPlay`
  ;[0 1 0.5776] Begin Play
  (`/Game/Blueprint/IMPORTED/Component/BPC_AudioRock.Initialize` (`self.BPC_AudioRock`) (`self.SM_Rock`) (`self.MaxSpeedRemap`))
  (bind _returnvalue (`KismetMaterialLibrary.CreateDynamicMaterialInstance` "/Game/Art/Material/Face/M_Face.M_Face"))
  (set `self.FaceMaterial` _returnvalue)
  (`self.SetFace` (`self.Eyes`) (`self.Mouth`))
  (`self.IdleFaceAnim`)
  (set `self.StartRotFaceAnim` (`SceneComponent.RelativeRotation` (`self.SM_Face`)))
  (`self.RotationFaceAnim`))

(event `self.ReceiveTick`
  (params (DeltaSeconds :type "Float (single-precision)"))
  ;[0 1 0.5794] Tick
  (bind (_outhit _returnvalue) (`self.GroundCheck` (`self.GroundCheckRadius`) (`self.Ground Check Distance`)))
  (set `self.Grounded?` _returnvalue)
  (`self.MovingFX` (`self.Grounded?`))
  (set `/Game/Blueprint/IMPORTED/Component/BPC_AudioRock.Grounded?` (`self.Grounded?`) (`self.BPC_AudioRock`)))

(event `InitialliseAll`
  (params (Speed :type "Float (double-precision)") (LeaveObjectiveLoc :type "Vector Structure") (HouseREF :type "/Game/Blueprint/IA/HouseManager Object Reference") (Leaving :type Boolean) (Mooving :type Boolean) (`Canon?` :type Boolean) (Jesus :type Boolean))
  (set `self.HouseREF` HouseREF)
  (set `self.Speed` Speed)
  (set `self.ObjectiveLoc` LeaveObjectiveLoc)
  (set `self.Leaving` Leaving)
  (set `self.Mooving` Mooving)
  (set `self.Alive` true)
  (set `self.Jesus` Jesus)
  (if `Canon?`
    (`KismetSystemLibrary.Delay` 2.5)
    (`/Game/Blueprint/IA/HouseManager.LeftHouse` (`self.HouseREF`))
    (set `self.Alive` false)
    (`self.K2_DestroyActor`)
    (else
      (`self.StartMooving`))))

(event `MovingFX`
  (params (`Grounded?` :type Boolean))
  (bind _ns_rollingsmoke (`self.NS_RollingSmoke`))
  (bind _maxspeedremap (`self.MaxSpeedRemap`))
  (bind _returnvalue (`KismetMathLibrary.VSize` (`SceneComponent.GetComponentVelocity` (`self.CollisionShape`))))
  ;[1 1 1] Moving Smoke Fx
  (if (and `Grounded?` (> (`KismetMathLibrary.VSize` (`SceneComponent.GetComponentVelocity` (`self.CollisionShape`))) 0.0))
    (`FXSystemComponent.SetFloatParameter` _ns_rollingsmoke "SmokeSizeMin" (`KismetMathLibrary.MapRangeClamped` _returnvalue 0.0 _maxspeedremap 0.0 0.5))
    (`FXSystemComponent.SetFloatParameter` _ns_rollingsmoke "SmokeSizeMax" (`KismetMathLibrary.MapRangeClamped` _returnvalue 0.0 _maxspeedremap 0.0 1.0))
    (`/Engine/EditorBlueprintResources/StandardMacros.DoOnce` false :!label _label
      (:`Completed`
        (`ActorComponent.Activate` (`self.NS_RollingSmoke`) false)
        (goto _label_2 :!via `Reset`)))
    (else
      (`/Engine/EditorBlueprintResources/StandardMacros.DoOnce` false :!label _label_2
        (:`Completed`
          (`ActorComponent.Deactivate` (`self.NS_RollingSmoke`))
          (goto _label :!via `Reset`))))))

(event `IdleFaceAnim`
  (`self.SetFace` "NewEnumerator3" (`self.Current Mouth`))
  (`KismetSystemLibrary.Delay` 0.5)
  (`self.SetFace` (`self.CurrentEyes`) (`self.Current Mouth`))
  (`KismetSystemLibrary.Delay` (`KismetMathLibrary.RandomFloatInRange` 0.5 10.0))
  (`self.IdleFaceAnim`))

(event `StartMooving`
  ;[0 0.9896 0.6619 0.5] Movement
  (bind _returnvalue (`KismetSystemLibrary.K2_SetTimerDelegate` (delegate `Moove`) 0.02 true true))
  (set `self.Timer` _returnvalue))

(event `Moove`
  (bind _houseref (`self.HouseREF`))
  (bind (_objectiveloc_x _objectiveloc_y) (`KismetMathLibrary.BreakVector` (`self.ObjectiveLoc`)))
  (bind (_returnvalue_x _returnvalue_y) (`KismetMathLibrary.BreakVector` (`SceneComponent.K2_GetComponentLocation` (`self.CollisionShape`))))
  (bind (_returnvalue_x_2 _returnvalue_y_2) (`KismetMathLibrary.BreakVector` (* (`KismetMathLibrary.Normal` (`KismetMathLibrary.GetDirectionUnitVector` (`SceneComponent.K2_GetComponentLocation` (`self.CollisionShape`)) (`self.ObjectiveLoc`))) (`self.Speed`))))
  ;[0 0.9896 0.6619 0.5] Movement
  (if (`self.Mooving`)
    (`PrimitiveComponent.SetPhysicsLinearVelocity` (`self.CollisionShape`) (`KismetMathLibrary.MakeVector` _returnvalue_x_2 _returnvalue_y_2) false "None")
    (if (`self.Jesus`)
      (`KismetSystemLibrary.Delay` (`KismetMathLibrary.MapRangeUnclamped` (`self.Speed`) 700.0 1800.0 1.5 0.5))
      (`self.ActivateJesus`)
      (else
        (if (and (`KismetMathLibrary.NearlyEqual_FloatFloat` _returnvalue_x _objectiveloc_x 70.0) (`KismetMathLibrary.NearlyEqual_FloatFloat` _returnvalue_y _objectiveloc_y 70.0)) :!label _label_3
          (`/Engine/EditorBlueprintResources/StandardMacros.DoOnce` false
            (:`Completed`
              (if (`self.Leaving`)
                (`/Game/Blueprint/IA/HouseManager.LeftHouse` _houseref)
                (else
                  (`/Game/Blueprint/IA/HouseManager.AddInHouse` _houseref)))
              (set `self.Alive` false)
              (`self.K2_DestroyActor`))))))
    (else
      (goto _label_3))))

(event `RotationFaceAnim`
  (`/Engine/EditorBlueprintResources/StandardMacros.FlipFlop`
    (:`A`
      (set `self.TargetRotFaceAnim` (`KismetMathLibrary.ComposeRotators` (`self.StartRotFaceAnim`) (`KismetMathLibrary.MakeRotator` 0.0 (`KismetMathLibrary.RandomFloatInRange` -15.0 15.0) (`KismetMathLibrary.RandomFloatInRange` -15.0 15.0))))
      (set `self.RotFaceAnimDelay` (`KismetMathLibrary.RandomFloatInRange` 0.0 2.0))
      (bind (_direction _alpha) (`Timeline|RotFaceAnim` :!via `PlayFromStart` :!label _label_4)
        (:`Update`
          (`SceneComponent.K2_SetRelativeRotation` (`self.SM_Face`) (`|EaseFunction` "ExpoInOut" _alpha (`self.StartRotFaceAnim`) (`self.TargetRotFaceAnim`)) false false))
        (:`Finished`
          (`KismetSystemLibrary.Delay` (`self.RotFaceAnimDelay`))
          (`self.RotationFaceAnim`))))
    (:`B`
      (set `self.RotFaceAnimDelay` (`KismetMathLibrary.RandomFloatInRange` 0.0 10.0))
      (goto _label_4 :!via `ReverseFromEnd`))))

(event `ActivateJesus`
  (bind _collisionshape (`self.CollisionShape`))
  (bind _startjesusloc (`self.StartJesusLoc`))
  (`KismetSystemLibrary.K2_ClearAndInvalidateTimerHandle` (`self.Timer`))
  (`ActorComponent.Activate` (`self.NS_Auréole`) true)
  (`NiagaraFunctionLibrary.SpawnSystemAtLocation` "/Game/VFX/Minigame/NS_JesusTime.NS_JesusTime" (`SceneComponent.K2_GetComponentLocation` (`self.CollisionShape`)))
  (`PrimitiveComponent.SetPhysicsLinearVelocity` _collisionshape (0.0 0.0 0.0) false "None")
  (`PrimitiveComponent.SetSimulatePhysics` _collisionshape false)
  (`TimelineComponent.SetPlayRate` (`self.LerpPos`) (/ 1.0 5.0))
  (set `self.StartJesusLoc` (`SceneComponent.K2_GetComponentLocation` (`self.CollisionShape`)))
  (bind (_direction _newtrack_0) (`Timeline|LerpPos` :!via `PlayFromStart`)
    (:`Update`
      (`SceneComponent.K2_SetWorldLocation` (`self.CollisionShape`) (`KismetMathLibrary.VLerp` _startjesusloc (+ _startjesusloc (0.0 0.0 2000.0)) _newtrack_0) false false))
    (:`Finished`
      (set `self.Alive` false)
      (`self.K2_DestroyActor`))))

(event `EVENTT`
  (`KismetSystemLibrary.K2_ClearAndInvalidateTimerHandle` (stale `StartMooving` _returnvalue))
  (`ActorComponent.Activate` (`self.NS_Jesus`) false)
  (`ActorComponent.Activate` (`self.NS_Auréole`) false)
  (`PrimitiveComponent.SetSimulatePhysics` (`self.CollisionShape`) false))

(fn `GetDistanceToPlayer`
  (returns (DistanceToPlayer :type "Float (double-precision)"))
  (return (`self.DistanceToPlayer`)))

(fn `GroundCheck`
  (params (Radius :type "Float (double-precision)") (GroundCheckDistance :type "Float (double-precision)"))
  (returns (OutHit :type "HitResult Structure") (ReturnValue :type Boolean))
  (bind _returnvalue (`SceneComponent.K2_GetComponentLocation` (`self.CollisionShape`)))
  (bind (_outhit _returnvalue_2) (`KismetSystemLibrary.SphereTraceSingle` :`Start` _returnvalue :`End` (+ _returnvalue (* (0.0 0.0 -1.0) GroundCheckDistance)) :`Radius` Radius :`TraceChannel` "TraceTypeQuery1" :`bTraceComplex` true :`DrawTime` 1.0))
  (return _outhit _returnvalue_2))

(fn `RemapVelocity`
  (params (MinValue :type "Float (double-precision)") (MaxValue :type "Float (double-precision)"))
  (returns (ReturnValue :type "Float (double-precision)"))
  (return 0.0))

(fn `SetFace`
  (params (eyes :type "/Game/Art/Material/Face/E_eyes Enum" :default "NewEnumerator0") (mouth :type "/Game/Art/Material/Face/E_mouth Enum" :default "NewEnumerator0") (`ShouldSaveFace?` :type Boolean :default true))
  (locals (NewLocalVar :type "Texture Object Reference") (eyes_happy_texture :type "Texture Object Reference" :default "/Script/Engine.Texture2D'/Game/Art/Material/Face/e_happy.e_happy'") (eyes_sad_texture :type "Texture Object Reference" :default "/Script/Engine.Texture2D'/Game/Art/Material/Face/e_sad.e_sad'") (eyes_tired_texture :type "Texture Object Reference" :default "/Script/Engine.Texture2D'/Game/Art/Material/Face/e_tired.e_tired'") (eyes_suspicious_texture :type "Texture Object Reference" :default "/Script/Engine.Texture2D'/Game/Art/Material/Face/e_suspicious.e_suspicious'") (eyes_normal_texture :type "Texture Object Reference" :default "/Script/Engine.Texture2D'/Game/Art/Material/Face/e_none.e_none'") (eyes_angry_texture :type "Texture Object Reference" :default "/Script/Engine.Texture2D'/Game/Art/Material/Face/e_angry.e_angry'") (mouth_happy_texture :type "Texture Object Reference" :default "/Script/Engine.Texture2D'/Game/Art/Material/Face/m_happy.m_happy'") (mouth_sad_texture :type "Texture Object Reference" :default "/Script/Engine.Texture2D'/Game/Art/Material/Face/m_sad.m_sad'") (mouth_surpised_texture :type "Texture Object Reference" :default "/Script/Engine.Texture2D'/Game/Art/Material/Face/m_surprised.m_surprised'"))
  (`MaterialInstanceDynamic.SetTextureParameterValue` (`self.FaceMaterial`) "eyes_texture" (select `/Game/Art/Material/Face/E_eyes` eyes :`NewEnumerator0` (`local.eyes_happy_texture`) :`NewEnumerator1` (`local.eyes_sad_texture`) :`NewEnumerator2` (`local.eyes_tired_texture`) :`NewEnumerator3` (`local.eyes_suspicious_texture`) :`NewEnumerator4` (`local.eyes_normal_texture`) :`NewEnumerator5` (`local.eyes_angry_texture`)))
  (`MaterialInstanceDynamic.SetTextureParameterValue` (`self.FaceMaterial`) "mouth_texture" (select `/Game/Art/Material/Face/E_mouth` mouth :`NewEnumerator0` (`local.mouth_happy_texture`) :`NewEnumerator1` (`local.mouth_sad_texture`) :`NewEnumerator2` (`local.mouth_surpised_texture`)))
  (`PrimitiveComponent.SetMaterial` (`self.SM_Face`) 0 (`self.FaceMaterial`))
  (if (`local.ShouldSaveFace?`)
    (set `self.Current Mouth` (`self.Mouth`))
    (set `self.CurrentEyes` (`self.Eyes`))))

(fn `UpdateScale`
  (bind _returnvalue (`KismetMathLibrary.MapRangeClamped` (`KismetMathLibrary.Conv_IntToDouble` (`self.MossQuantity`)) 150.0 4250.0 1.0 43.0))
  (bind _returnvalue_2 (`KismetMathLibrary.MapRangeClamped` (`KismetMathLibrary.Conv_IntToDouble` (`self.MossQuantity`)) 0.0 1000.0 100.0 50.0))
  (bind _returnvalue_3 (`KismetMathLibrary.MapRangeClamped` (`KismetMathLibrary.Conv_IntToDouble` (`self.MossQuantity`)) 0.0 10000.0 100.0 200.0))
  (`MeshComponent.SetScalarParameterValueOnMaterials` (`self.SM_Rock`) "BlendBias_Normal" (`KismetMathLibrary.MapRangeClamped` (`KismetMathLibrary.Conv_IntToDouble` (`self.MossQuantity`)) 0.0 150.0 -2.0 3.0))
  (if (`self.Boss?`)
    (`MeshComponent.SetScalarParameterValueOnMaterials` (`self.SM_Rock`) "MOSSROCK_SizeTexture" _returnvalue_3)
    (`MeshComponent.SetScalarParameterValueOnMaterials` (`self.SM_Moss`) "MOSS_TextureSize" _returnvalue_3)
    (`SceneComponent.SetWorldScale3D` (`self.CollisionShape`) (* (`KismetMathLibrary.Conv_DoubleToVector` _returnvalue) (`self.Scale`)))
    (`SceneComponent.SetWorldScale3D` (`self.SM_Moss`) (* (`KismetMathLibrary.Conv_DoubleToVector` _returnvalue) (`self.Scale`)))
    (`SceneComponent.SetRelativeScale3D` (`self.SM_Face`) (`KismetMathLibrary.Conv_DoubleToVector` (`KismetMathLibrary.Lerp` 0.99 44.8 (`CurveFloat.GetFloatValue` (`self.VisageScalingCurve`) (`KismetMathLibrary.MapRangeClamped` (`KismetMathLibrary.Conv_IntToDouble` (`self.MossQuantity`)) 0.0 4250.0 0.0 1.0)))))
    (`MeshComponent.SetScalarParameterValueOnMaterials` (`self.SM_Face`) "Size" (`KismetMathLibrary.MapRangeClamped` (`KismetMathLibrary.Conv_IntToDouble` (`self.MossQuantity`)) 150.0 4250.0 0.5 0.3))
    (else
      (`MeshComponent.SetScalarParameterValueOnMaterials` (`self.SM_Rock`) "MOSSROCK_SizeTexture" _returnvalue_2)
      (`MeshComponent.SetScalarParameterValueOnMaterials` (`self.SM_Moss`) "MOSS_TextureSize" _returnvalue_2)
      (`SceneComponent.SetWorldScale3D` (`self.CollisionShape`) (* (`KismetMathLibrary.Conv_DoubleToVector` (`KismetMathLibrary.MapRangeClamped` (`KismetMathLibrary.Conv_IntToDouble` (`self.MossQuantity`)) 150.0 1000.0 1.0 10.0)) (`self.Scale`)))
      (`SceneComponent.SetWorldScale3D` (`self.SM_Moss`) (* (`KismetMathLibrary.Conv_DoubleToVector` (`KismetMathLibrary.MapRangeClamped` (`KismetMathLibrary.Conv_IntToDouble` (`self.MossQuantity`)) 150.0 1000.0 0.59 10.0)) (`self.Scale`)))
      (`SceneComponent.SetRelativeScale3D` (`self.SM_Face`) (`KismetMathLibrary.Conv_DoubleToVector` (`KismetMathLibrary.Lerp` 0.99 3.08 (`CurveFloat.GetFloatValue` (`self.VisageScalingCurve`) (`KismetMathLibrary.MapRangeClamped` (`KismetMathLibrary.Conv_IntToDouble` (`self.MossQuantity`)) 0.0 1000.0 0.0 1.0)))))
      (`MeshComponent.SetScalarParameterValueOnMaterials` (`self.SM_Face`) "Size" (`KismetMathLibrary.MapRangeClamped` (`KismetMathLibrary.Conv_IntToDouble` (`self.MossQuantity`)) 150.0 1000.0 0.5 0.01))))
  (`SceneComponent.SetWorldScale3D` (`self.SM_Rock`) (`KismetMathLibrary.Conv_DoubleToVector` (`self.Scale`)))
  (set `self.GroundCheckRadius` (`KismetMathLibrary.MapRangeClamped` (`KismetMathLibrary.Conv_IntToDouble` (`self.MossQuantity`)) 150.0 1000.0 45.0 300.0))
  (set `self.Ground Check Distance` (`KismetMathLibrary.MapRangeClamped` (`KismetMathLibrary.Conv_IntToDouble` (`self.MossQuantity`)) 150.0 1000.0 45.0 300.0))
  (return))

(fn `UserConstructionScript`
  (`self.UpdateScale`))