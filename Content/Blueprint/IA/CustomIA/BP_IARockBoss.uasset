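; Two-phase rock boss fight, started when the player rock enters its trigger.
; Phase 1 loops a timeline-driven comet charge into an explosion until hits cancel it, strip moss and trigger a cinematic drop through broken ground.
; Phase 2 is whack-a-mole: it dives between random, non-repeating holes with telegraphs, adding feints and panic hops as hits land.
; TakeDmg's hit counter drives every transition, ending in a death cinematic at five hits.
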(event `self.ReceiveBeginPlay`
  (`parent.ReceiveBeginPlay`)
  (bind _outactors (`GameplayStatics.GetAllActorsOfClass` "/Game/Blueprint/Boss/BP_BossArenaManager.BP_BossArenaManager_C"))
  (for _array_element _outactors
    (set `self.ArenaREF` _array_element))
  (bind _returnvalue (`GameplayStatics.SpawnSound2D` "/Game/Audio/Sounds/SFX/Boss/SC_Boss_P2_OutIdle.SC_Boss_P2_OutIdle" 1.0 1.0 0.0 null))
  (bind _output_get (set `self.OutIdleSoundRef` _returnvalue))
  (`AudioComponent.Play` _output_get 0.0)
  (`AudioComponent.SetVolumeMultiplier` _output_get 0.0))

(event `self.Triggerboss.OnComponentBeginOverlap`
  (params (OverlappedComponent :type "PrimitiveComponent Object Reference") (OtherActor :type "Actor Object Reference") (OtherComp :type "PrimitiveComponent Object Reference") (OtherBodyIndex :type Integer) (bFromSweep :type Boolean) (SweepResult :type "HitResult Structure (by ref)"))
  ;[0 1 0.5039 0.5 50] Sart
  (cast `/Game/Blueprint/Player/BP_PlayerRock` OtherActor)
  (`self.StartPhase1`)
  (set `self.HitCount` 0)
  (set `/Game/Blueprint/Player/BP_PlayerRock.MossQuantity` 0 (`/Game/Blueprint/BFL_Rock.GetPlayerActorRef`))
  (`ActorComponent.K2_DestroyComponent` (`self.Triggerboss`)))

(event `Explosion`
  (bind _returnvalue (`self.K2_GetActorLocation`))
  ;[0.03151 0.3918 1 0.5 50] Phase 1
  (`NiagaraFunctionLibrary.SpawnSystemAtLocation` "/Game/VFX/Jump/NS_JumpBIG.NS_JumpBIG" (`self.K2_GetActorLocation`) (struct) (20.0 20.0 20.0))
  (`NiagaraFunctionLibrary.SpawnSystemAtLocation` "/Game/VFX/Jump/NS_JumpBigNored.NS_JumpBigNored" (+ (`self.K2_GetActorLocation`) (0.0 0.0 -3000.0)) (struct) (20.0 20.0 20.0))
  (`NiagaraFunctionLibrary.SpawnSystemAtLocation` "/Game/VFX/Jump/NS_JumpBigNored.NS_JumpBigNored" (+ _returnvalue (0.0 0.0 3000.0)) (struct) (20.0 20.0 20.0))
  (`GameplayStatics.PlayWorldCameraShake` "/Game/Blueprint/Player/CameraShakePlayer/CS_ImpactBoss.CS_ImpactBoss_C" _returnvalue 50000.0 10000.0)
  (`/Game/Blueprint/Boss/BP_BossArenaManager.CallFX` (`self.ArenaREF`)))

(event `StartPhase1`
  ;[0.03151 0.3918 1 0.5 50] Phase 1
  (set `self.Phase1` false)
  (bind _returnvalue (`KismetSystemLibrary.K2_SetTimerDelegate` (delegate `Attacks`) 0.1 true true))
  (set `self.TimelineEnCours` _returnvalue))

(event `Attacks`
  ;[0.03151 0.3918 1 0.5 50] Phase 1
  (`/Engine/EditorBlueprintResources/StandardMacros.Gate` false :!label _label
    (:`Exit`
      (`|ExecutionSequence`
        (:`then_0`
          (`|ExecutionSequence`
            (:`then_1`
              (bind _returnvalue (`GameplayStatics.SpawnSoundAtLocation` "/Game/Audio/Sounds/SFX/Boss/SC_Boss_P1.SC_Boss_P1" (`self.K2_GetActorLocation`) (struct) 1.0 1.0 0.0 null null))
              (set `self.attackSound` _returnvalue)
              (bind (_direction _location _rotation _fire) (`Timeline|ChargeAttack` :!via `PlayFromStart` :!label _label_2)
                (:`Update`
                  (`SceneComponent.K2_SetRelativeLocationAndRotation` (`self.CollisionShape`) (`KismetMathLibrary.MakeVector` 0.0 0.0 _location) (`KismetMathLibrary.MakeRotator` 0.0 (* _rotation -1.0)) false false)
                  (`NiagaraComponent.SetVariableFloat` (`self.Cometfkpz`) "FireOpacity" _fire))))
            (:`then_2`
              (`KismetSystemLibrary.RetriggerableDelay` 5.15)
              (if (`self.cancelled`)
                _
                (elif (not (`self.Phase2`))
                  (`self.Explosion`)
                  (`KismetSystemLibrary.Delay` (`self.AttacksDelay`))
                  (`self.ReopenGate`))))))
        (:`then_1`
          (goto _label :!via `Close`))
        (:`then_2`
          (set `self.cancelled` false))))))

(event `ReopenGate`
  ;[0.03151 0.3918 1 0.5 50] Phase 1
  (goto _label :!via `Open`))

(event `self.ReceiveTick`
  (params (DeltaSeconds :type "Float (single-precision)")))

(event `Stop CastAttack`
  ;[0.03151 0.3918 1 0.5 50] Phase 1
  (`|ExecutionSequence`
    (:`then_0`
      (set `self.cancelled` true)
      (goto _label_2 :!via `Stop`))
    (:`then_1`
      (`SceneComponent.K2_SetRelativeLocationAndRotation` (`self.CollisionShape`) (0.0 0.0 0.0) (`KismetMathLibrary.MakeRotator` 0.0) false false)
      (`NiagaraComponent.SetVariableFloat` (`self.Cometfkpz`) "FireOpacity" 0.0))
    (:`then_2`
      (`KismetSystemLibrary.Delay` 3.0)
      (`self.ReopenGate`))))

(event `StartPhase 2`
  ;[1 0.3021 0.5254 0.5 50] Phase 2
  (`/Engine/EditorBlueprintResources/StandardMacros.DoOnce` false
    (:`Completed`
      (set `self.PrefallLoc` (`self.K2_GetActorLocation`))
      (`/Game/Blueprint/Boss/BP_BossArenaManager.BreakGround` (`self.ArenaREF`))
      (`PrimitiveComponent.SetCollisionResponseToAllChannels` (`self.CollisionShape`) "ECR_Ignore")
      (`GameplayStatics.LoadStreamLevel` "SL_cinematic" true)
      ;;[1 1 1 0.5] Ciné transition
      (bind (_outactor _returnvalue) (`LevelSequencePlayer.CreateLevelSequencePlayer` "/Game/Cinematic/SEQ_4_Boss2_/MS_Boss2.MS_Boss2"))
      (`/Engine/EditorBlueprintResources/StandardMacros.IsValid` _returnvalue
        (:`Is Valid`
          (bind _sequenceplayer (`LevelSequenceActor.SequencePlayer` _outactor))
          (`MovieSceneSequencePlayer.Play` _sequenceplayer)
          (set `/Game/Blueprint/Player/BP_PlayerRock.ActualCinePlaying` _sequenceplayer (`/Game/Blueprint/BFL_Rock.GetPlayerActorRef`)))
        (:`Is Not Valid`
          _))
      (`KismetMaterialLibrary.SetScalarParameterValue` "/Game/Blueprint/Player/MPC_SEeThgh.MPC_SEeThgh" "Active")
      (add `MovieSceneSequencePlayer.OnStop` _returnvalue (delegate `CustomEvent`))
      (`/Game/Blueprint/Player/BP_PlayerRock.LockPlayer` (`/Game/Blueprint/BFL_Rock.GetPlayerActorRef`)))))

(event `Rotate`
  ;[1 0.3021 0.5254 0.5 50] Phase 2
  (`SceneComponent.K2_SetWorldRotation` (`self.SM_Rock`) (`KismetMathLibrary.FindLookAtRotation` (`self.K2_GetActorLocation`) (`SceneComponent.K2_GetComponentLocation` (`/Game/Blueprint/Player/BP_PlayerRock.GetMovingComponent` (`/Game/Blueprint/BFL_Rock.GetPlayerActorRef`)))) false false))

(event `CustomEvent`
  (bind _prefallloc (`self.PrefallLoc`))
  ;[1 0.3021 0.5254 0.5 50] Phase 2
  ;;[1 1 1 0.5] Ciné transition
  (`KismetSystemLibrary.Delay` 1.0)
  (`KismetMaterialLibrary.SetScalarParameterValue` "/Game/Blueprint/Player/MPC_SEeThgh.MPC_SEeThgh" "Active" 1.0)
  (`/Game/Blueprint/Player/BP_PlayerRock.UnlockPlayer` (`/Game/Blueprint/BFL_Rock.GetPlayerActorRef`))
  (`self.SetActorHiddenInGame` (`/Game/Blueprint/BFL_Rock.GetPlayerActorRef`) false)
  (`GameplayStatics.UnloadStreamLevel` "SL_cinematic")
  (set `self.Phase2` true)
  (bind _outhit (`KismetSystemLibrary.LineTraceSingle` :`Start` _prefallloc :`End` (- _prefallloc (0.0 0.0 100000.0)) :`TraceChannel` "TraceTypeQuery1" :`DrawDebugType` "Persistent"))
  (`TimelineComponent.SetPlayRate` (`self.Fall`) (/ 1.0 5.0))
  (bind (_direction _newtrack_0) (`Timeline|Fall` :!via `PlayFromStart`)
    (:`Update`
      (`self.K2_SetActorLocation` (`KismetMathLibrary.VLerp` (`self.PrefallLoc`) (+ (`.ImpactPoint` (`GameplayStatics.BreakHitResult` _outhit)) (0.0 0.0 150.0)) _newtrack_0)))
    (:`Finished`
      (`KismetSystemLibrary.K2_SetTimerDelegate` (delegate `Rotate`) 0.01 true true)
      (`KismetSystemLibrary.Delay` 2.0)
      (`self.Tauping`))))

(event `IntroStopped`
  ;[0.6451 0.5104 1 0.5 50] Receive Damage
  (`KismetSystemLibrary.Delay` 1.0)
  (`GameplayStatics.UnloadStreamLevel` "SL_cinematic")
  (`/Game/Blueprint/Player/BP_PlayerRock.UnlockPlayer` (`/Game/Blueprint/BFL_Rock.GetPlayerActorRef`))
  (`self.SetActorHiddenInGame` (`/Game/Blueprint/BFL_Rock.GetPlayerActorRef`) false)
  (`KismetMaterialLibrary.SetScalarParameterValue` "/Game/Blueprint/Player/MPC_SEeThgh.MPC_SEeThgh" "Active" 1.0))

(event `self.TakeDmg`
  (params (AttackImpact :type "Vector Structure"))
  (bind _asbp_player_rock (`/Game/Blueprint/BFL_Rock.GetPlayerActorRef`))
  (bind _returnvalue (`self.K2_GetActorLocation`))
  (bind _attacksound (`self.attackSound`))
  (bind _attacksound_2 (`self.attackSound`))
  ;[0.6451 0.5104 1 0.5 50] Receive Damage
  (`/Engine/EditorBlueprintResources/StandardMacros.DoOnce` false :!label _label_3
    (:`Completed`
      (`GameplayStatics.PlaySoundAtLocation` "/Game/Audio/Sounds/SFX/Boss/SC_Boss_Damage.SC_Boss_Damage" (`self.K2_GetActorLocation`) (struct) 1.0 1.0 0.0 null null null null)
      (set `self.HitCount` (+ (`self.HitCount`) 1))
      (if (`self.Phase2`)
        (if (>= (`self.HitCount`) 5)
          (`|ExecutionSequence`
            (:`then_0`
              (`KismetSystemLibrary.PrintString` "MORT")
              (`AudioComponent.SetVolumeMultiplier` (`self.OutIdleSoundRef`) 0.0)
              (`GameplayStatics.LoadStreamLevel` "SL_cinematic" true)
              (`/Game/Blueprint/Player/BP_PlayerRock.LockPlayer` _asbp_player_rock)
              (`self.SetActorHiddenInGame` true)
              ;;[1 1 1 0.5] CinéFin
              (`self.SetActorHiddenInGame` (`/Game/Blueprint/BFL_Rock.GetPlayerActorRef`) true)
              (bind (_outactor _returnvalue_2) (`LevelSequencePlayer.CreateLevelSequencePlayer` "/Game/Cinematic/SEQ_5_Boss3_Outro/MS_Boss3New.MS_Boss3New"))
              (`/Engine/EditorBlueprintResources/StandardMacros.IsValid` _returnvalue_2
                (:`Is Valid`
                  (bind _sequenceplayer (`LevelSequenceActor.SequencePlayer` _outactor))
                  (`MovieSceneSequencePlayer.Play` _sequenceplayer)
                  (set `/Game/Blueprint/Player/BP_PlayerRock.ActualCinePlaying` _sequenceplayer (`/Game/Blueprint/BFL_Rock.GetPlayerActorRef`))
                  (`KismetMaterialLibrary.SetScalarParameterValue` "/Game/Blueprint/Player/MPC_SEeThgh.MPC_SEeThgh" "Active")
                  (add `MovieSceneSequencePlayer.OnStop` _returnvalue_2 (delegate `IntroStopped`))
                  (`/Game/Blueprint/Player/BP_PlayerRock.LockPlayer` (`/Game/Blueprint/BFL_Rock.GetPlayerActorRef`)))
                (:`Is Not Valid`
                  (`/Game/Blueprint/Player/BP_PlayerRock.UnlockPlayer` _asbp_player_rock))))
            (:`then_1`
              (`NiagaraFunctionLibrary.SpawnSystemAtLocation` "/Game/VFX/Choc/SparksHisNoMoss.SparksHisNoMoss" AttackImpact (struct) (2.0 2.0 2.0) true true "None" false :!label _label_4))
            (:`then_2`
              (`self.Panick` :!label _label_5)
              (set `self.hit` true)
              (`|ExecutionSequence`
                (:`then_0`
                  (goto _label_3 :!via `Reset`))
                (:`then_1`
                  (switch `int` (`self.HitCount`) :!label _label_6
                    (:`0`
                      (`self.RemoveMoss` 5000 :!label _label_7)
                      (`SceneComponent.SetWorldScale3D` (`self.CollisionShape`) (4.0 4.0 4.0))
                      (`SceneComponent.SetVisibility` (`self.SM_Moss`) false false)
                      (`SceneComponent.SetVisibility` (`self.HISM_Moss`) false false)
                      (`/Game/Blueprint/Player/BP_PlayerRock.Damage` (`/Game/Blueprint/BFL_Rock.GetPlayerActorRef`) 1000 (`self.K2_GetActorLocation`) true)
                      (`/Engine/EditorBlueprintResources/StandardMacros.IsValid` _attacksound
                        (:`Is Valid`
                          (`AudioComponent.Stop` _attacksound))
                        (:`Is Not Valid`
                          _))
                      (`KismetSystemLibrary.K2_ClearAndInvalidateTimerHandle` (`self.TimelineEnCours`))
                      (`self.StartPhase 2`)
                      (`ActorComponent.K2_DestroyComponent` (`self.Cone1`))
                      (`ActorComponent.K2_DestroyComponent` (`self.Cone`))
                      (set `self.HitCount` 2)
                      (goto _label_3 :!via `Reset`))
                    (:`1`
                      (`self.Stop CastAttack`)
                      (`/Game/Blueprint/Boss/BP_BossArenaManager.Close Entrance` (`self.ArenaREF`))
                      (`self.RemoveMoss` 1250)
                      (`self.K2_SetActorLocation` (- _returnvalue (0.0 0.0 1000.0)))
                      (`/Game/Blueprint/Player/BP_PlayerRock.Damage` (`/Game/Blueprint/BFL_Rock.GetPlayerActorRef`) 400 _returnvalue true)
                      (`|ExecutionSequence`
                        (:`then_0`
                          (`KismetSystemLibrary.Delay` 10.0)
                          (`PrimitiveComponent.SetCollisionResponseToChannel` (`self.Cone1`) "ECC_Pawn" "ECR_Ignore")
                          (goto _label_3 :!via `Reset`))
                        (:`then_1`
                          (set `self.Locbase` (`SceneComponent.RelativeLocation` (`self.Cone`)))
                          (`PrimitiveComponent.SetCollisionResponseToChannel` (`self.Cone`) "ECC_Pawn" "ECR_Block")
                          (`TimelineComponent.SetPlayRate` (`self.MoveCone`) (/ 1.0 2.0))
                          (bind (_direction _newtrack_0) (`Timeline|MoveCone` :!via `PlayFromStart`)
                            (:`Update`
                              (`SceneComponent.K2_SetRelativeLocation` (`self.Cone`) (`KismetMathLibrary.VLerp` (`self.Locbase`) (0.0 0.0 0.0) _newtrack_0) false false))
                            (:`Finished`
                              (`PrimitiveComponent.SetCollisionResponseToChannel` (`self.Cone`) "ECC_Pawn" "ECR_Ignore")
                              (`SceneComponent.K2_SetRelativeLocation` (`self.Cone`) (`self.Locbase`) false false))))
                        (:`then_2`
                          (`/Engine/EditorBlueprintResources/StandardMacros.IsValid` _attacksound_2
                            (:`Is Valid`
                              (`AudioComponent.Stop` _attacksound_2))))))
                    (:`2`
                      (`self.Stop CastAttack`)
                      (goto _label_7))
                    (:`3`
                      (set `self.Finting` true)
                      (goto _label_4))
                    (:`4`
                      (set `self.FINTEWHEIGHT` 0.6)
                      (goto _label_4))
                    (:`5`
                      (goto _label_4)))))))
          (else
            (goto _label_5)))
        (else
          (goto _label_6))))))

(event `Tauping`
  (bind _ns_exclamation2 (`self.NS_Exclamation2`))
  (bind _ns_exclamation (`self.NS_Exclamation`))
  (bind _returnvalue (+ (`self.K2_GetActorLocation` (`self.HolePicked`)) (0.0 0.0 150.0)))
  (bind _returnvalue_2 (+ (`self.K2_GetActorLocation` (`self.HolePicked`)) (0.0 0.0 150.0)))
  ;[1 0.3021 0.5254 0.5 50] Phase 2
  ;;[0.9896 0.06075 0.8511 0.5 249] Pars la
  (`self.SetFace` "NewEnumerator5" "NewEnumerator1")
  (`ActorSequenceComponent.PlaySequence` (`self.Dive in`))
  (`PrimitiveComponent.SetCollisionResponseToAllChannels` (`self.CollisionShape`) "ECR_Ignore")
  (`KismetSystemLibrary.Delay` 0.2)
  (`GameplayStatics.PlayWorldCameraShake` "/Game/Blueprint/Player/CameraShakePlayer/CS_BossUnderground.CS_BossUnderground_C" (`SceneComponent.K2_GetComponentLocation` (`self.CollisionShape`)) 10000.0 15000.0)
  (`NiagaraFunctionLibrary.SpawnSystemAtLocation` "/Game/VFX/Choc/NS_ChocGround.NS_ChocGround" (+ (`SceneComponent.K2_GetComponentLocation` (`self.CollisionShape`)) (0.0 0.0 200.0)) (struct) (5.0 5.0 5.0))
  (`GameplayStatics.PlaySoundAtLocation` "/Game/Audio/Sounds/SFX/Boss/SC_Boss_P2_MoveOut.SC_Boss_P2_MoveOut" (`self.K2_GetActorLocation`) (struct) 1.0 1.0 0.0 null null null null)
  (`AudioComponent.SetVolumeMultiplier` (`self.OutIdleSoundRef`) 1.0)
  (`KismetSystemLibrary.Delay` 0.2)
  (`self.ChooseHole`)
  (`KismetSystemLibrary.Delay` 3.0)
  (if (`self.Finting`)
    (`|ExecutionSequence`
      (:`then_0`
        (`/Engine/EditorBlueprintResources/StandardMacros.DoOnce` false
          (:`Completed`
            (`|ExecutionSequence`
              (:`then_0`
                (`KismetSystemLibrary.PrintString` "FINTE !!!" true false (struct :`R` 1.0 :`B` 0.001876 :`A` 1.0) :!label _label_8)
                (`SceneComponent.K2_SetWorldLocation` _ns_exclamation2 _returnvalue_2 false false)
                (`GameplayStatics.PlaySoundAtLocation` "/Game/Audio/Sounds/SFX/Boss/SC_Boss_P2_Interrogation.SC_Boss_P2_Interrogation" _returnvalue_2 (struct) 1.0 1.0 0.0 null null null null)
                (`ActorComponent.Activate` _ns_exclamation2 true)
                (`KismetSystemLibrary.Delay` 1.2)
                (`ActorComponent.Deactivate` _ns_exclamation2)
                (`self.SetFace` "NewEnumerator0" "NewEnumerator2")
                (`ActorSequenceComponent.PlaySequence` (`self.Dive outanin`))
                (`GameplayStatics.PlaySoundAtLocation` "/Game/Audio/Sounds/SFX/Boss/SC_Boss_P2_MoveOut.SC_Boss_P2_MoveOut" (`self.K2_GetActorLocation`) (struct) 1.0 1.0 0.0 null null null null)
                (`AudioComponent.SetVolumeMultiplier` (`self.OutIdleSoundRef`) 1.0)
                (`KismetSystemLibrary.Delay` 0.07)
                (`NiagaraFunctionLibrary.SpawnSystemAtLocation` "/Game/VFX/Choc/NS_ChocGround.NS_ChocGround" (+ (`SceneComponent.K2_GetComponentLocation` (`self.CollisionShape`)) (0.0 0.0 200.0)) (struct) (5.0 5.0 5.0))
                (`KismetSystemLibrary.Delay` 0.3)
                (`AudioComponent.SetVolumeMultiplier` (`self.OutIdleSoundRef`) 0.0)
                (`GameplayStatics.PlaySoundAtLocation` "/Game/Audio/Sounds/SFX/Boss/SC_Boss_P2_MoveIn.SC_Boss_P2_MoveIn" (`self.K2_GetActorLocation`) (struct) 1.0 1.0 0.0 null null null null)
                (`self.ChooseHole`)
                (`ActorSequenceComponent.PlaySequence` (`self.Dive Out`))
                (`GameplayStatics.PlaySoundAtLocation` "/Game/Audio/Sounds/SFX/Boss/SC_Boss_P2_Feint.SC_Boss_P2_Feint" (`self.K2_GetActorLocation`) (struct) 1.0 1.0 0.0 null null null null)
                (`PrimitiveComponent.SetCollisionResponseToAllChannels` (`self.CollisionShape`) "ECR_Block")
                (`KismetSystemLibrary.Delay` 2.6)
                (if (not (`self.hit`))
                  (`self.Tauping`)))
              (:`then_1`
                (goto _label_9 :!via `Open`))))))
      (:`then_1`
        (`/Engine/EditorBlueprintResources/StandardMacros.Gate` true :!label _label_9
          (:`Exit`
            (if (`KismetMathLibrary.RandomBoolWithWeight` (`self.FINTEWHEIGHT`))
              (goto _label_8)
              (else
                (`SceneComponent.K2_SetWorldLocation` _ns_exclamation _returnvalue false false :!label _label_10)
                (`ActorComponent.Activate` _ns_exclamation true)
                (`GameplayStatics.PlaySoundAtLocation` "/Game/Audio/Sounds/SFX/Boss/SC_Boss_P2_Exclamation.SC_Boss_P2_Exclamation" _returnvalue (struct) 1.0 1.0 0.0 null null null null)
                (`KismetSystemLibrary.Delay` 1.2)
                (`ActorComponent.Deactivate` _ns_exclamation)
                (`NiagaraFunctionLibrary.SpawnSystemAtLocation` "/Game/VFX/Choc/NS_ChocGround.NS_ChocGround" (+ (`SceneComponent.K2_GetComponentLocation` (`self.CollisionShape`)) (0.0 0.0 200.0)) (struct) (2.0 2.0 2.0))
                (`AudioComponent.SetVolumeMultiplier` (`self.OutIdleSoundRef`) 0.0)
                (`GameplayStatics.PlaySoundAtLocation` "/Game/Audio/Sounds/SFX/Boss/SC_Boss_P2_MoveIn.SC_Boss_P2_MoveIn" (`self.K2_GetActorLocation`) (struct) 1.0 1.0 0.0 null null null null)
                (`ActorSequenceComponent.PlaySequence` (`self.Dive Out`))
                (`PrimitiveComponent.SetCollisionResponseToAllChannels` (`self.CollisionShape`) "ECR_Block")
                (`KismetSystemLibrary.Delay` 2.6)
                (if (not (`self.hit`))
                  (`self.Tauping`))))))))
    (else
      (goto _label_10))))

(event `Panick`
  ;[1 0.3021 0.5254 0.5 50] Phase 2
  (`self.SetFace` "NewEnumerator5" "NewEnumerator1")
  (if (not (>= (`self.HitCount`) 5))
    (`/Engine/EditorBlueprintResources/StandardMacros.DoOnce` false :!label _label_11
      (:`Completed`
        (set `self.panickrepeat` 0)
        (if (<= (`self.panickrepeat`) 8) :!label _label_12
          (`self.ChooseHole`)
          (`ActorSequenceComponent.PlaySequence` (`self.Dive outanin`))
          (`PrimitiveComponent.SetCollisionResponseToAllChannels` (`self.CollisionShape`) "ECR_Ignore")
          (`KismetSystemLibrary.Delay` 0.07)
          (`NiagaraFunctionLibrary.SpawnSystemAtLocation` "/Game/VFX/Choc/NS_ChocGround.NS_ChocGround" (+ (`SceneComponent.K2_GetComponentLocation` (`self.CollisionShape`)) (0.0 0.0 200.0)) (struct) (5.0 5.0 5.0))
          (`GameplayStatics.PlaySoundAtLocation` "/Game/Audio/Sounds/SFX/Boss/SC_Boss_P2_MoveOut.SC_Boss_P2_MoveOut" (`self.K2_GetActorLocation`) (struct) 1.0 1.0 0.0 null null null null)
          (`AudioComponent.SetVolumeMultiplier` (`self.OutIdleSoundRef`) 1.0)
          (`KismetSystemLibrary.Delay` 0.23)
          (`AudioComponent.SetVolumeMultiplier` (`self.OutIdleSoundRef`) 0.0)
          (`NiagaraFunctionLibrary.SpawnSystemAtLocation` "/Game/VFX/Choc/NS_ChocGround.NS_ChocGround" (+ (`SceneComponent.K2_GetComponentLocation` (`self.CollisionShape`)) (0.0 0.0 200.0)) (struct) (5.0 5.0 5.0))
          (`GameplayStatics.PlaySoundAtLocation` "/Game/Audio/Sounds/SFX/Boss/SC_Boss_P2_MoveOut.SC_Boss_P2_MoveOut" (`self.K2_GetActorLocation`) (struct) 1.0 1.0 0.0 null null null null)
          (`KismetSystemLibrary.Delay` 0.3)
          (set `self.panickrepeat` (+ (`self.panickrepeat`) 1))
          (goto _label_12)
          (else
            (`ActorSequenceComponent.PlaySequence` (`self.Dive Out`))
            (`GameplayStatics.PlaySoundAtLocation` "/Game/Audio/Sounds/SFX/Boss/SC_Boss_P2_MoveOut.SC_Boss_P2_MoveOut" (`self.K2_GetActorLocation`) (struct) 1.0 1.0 0.0 null null null null)
            (`KismetSystemLibrary.Delay` 1.3)
            (set `self.hit` false)
            (`self.Tauping`)
            (goto _label_11 :!via `Reset`)))))))

(fn `ChooseHole`
  (bind _prechole (`self.PrecHole`))
  (bind _holepicked (`self.HolePicked`))
  (bind _outitem (`KismetArrayLibrary.Array_Random` (`self.Trou`)))
  (`/Engine/EditorBlueprintResources/StandardMacros.IsValid` _outitem
    (:`Is Valid`
      (set `self.HolePicked` _outitem))
    (:`Is Not Valid`
      _))
  (`self.K2_SetActorLocation` (+ (`self.K2_GetActorLocation` (`self.HolePicked`)) (0.0 0.0 -120.0)))
  (`/Engine/EditorBlueprintResources/StandardMacros.IsValid` _prechole
    (:`Is Valid`
      (`KismetArrayLibrary.Array_Add` (`self.Trou`) _prechole))
    (:`Is Not Valid`
      _))
  (set `self.PrecHole` _holepicked)
  (`KismetArrayLibrary.Array_RemoveItem` (`self.Trou`) _holepicked))

(fn `UserConstructionScript`
  (`parent.UserConstructionScript`))