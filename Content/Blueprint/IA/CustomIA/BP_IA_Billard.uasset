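; Billiard ball actor for a pool minigame, knocked horizontally away from the player's rock by a velocity-change impulse on hit.
; Construction stores its start transform and applies its color.
; Enter marks it in and counts pocketed Boule balls: black entering last unlocks an achievement and completes target actors, otherwise all Boule balls return to start with zeroed velocity.
; Dehors resets only this ball.
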(event `Enter`
  (set `self.IsIn?` true)
  (set `self.NewVar_0` 0)
  (for _array_element (`self.Boule`)
    (if (`/Game/Blueprint/IA/CustomIA/BP_IA_Billard.IsIn?` _array_element)
      (set `self.NewVar_0` (+ (`self.NewVar_0`) 1))))
  (if (and (`self.Black`) (>= (`self.NewVar_0`) (- (`KismetArrayLibrary.Array_Length` (`self.Boule`)) 1)))
    (`/Game/Blueprint/IMPORTED/BFL_Rock.PushAchievement` 8)
    (bind _outactors (`GameplayStatics.GetAllActorsOfClass` null))
    (for _array_element_2 _outactors
      (`self.Complete` _array_element_2))
    (else
      (for _array_element_3 (`self.Boule`)
        (bind _collisionshape (`/Game/Blueprint/IA/BP_IARock.CollisionShape` _array_element_3))
        (`PrimitiveComponent.SetPhysicsLinearVelocity` _collisionshape (0.0 0.0 0.0) false "None")
        (`PrimitiveComponent.SetPhysicsAngularVelocityInDegrees` _collisionshape (0.0 0.0 0.0) false "None")
        (`SceneComponent.K2_SetWorldLocationAndRotation` _collisionshape (`/Game/Blueprint/IA/CustomIA/BP_IA_Billard.InitialPos` _array_element_3) (`/Game/Blueprint/IA/CustomIA/BP_IA_Billard.InitialRot` _array_element_3) false false)))))

(event `Dehors`
  (bind _collisionshape (`self.CollisionShape`))
  (`PrimitiveComponent.SetPhysicsLinearVelocity` _collisionshape (0.0 0.0 0.0) false "None")
  (`PrimitiveComponent.SetPhysicsAngularVelocityInDegrees` _collisionshape (0.0 0.0 0.0) false "None")
  (`SceneComponent.K2_SetWorldLocationAndRotation` _collisionshape (`self.InitialPos`) (`self.InitialRot`) false false))

(event `self.CollisionShape.OnComponentHit`
  (params (HitComponent :type "PrimitiveComponent Object Reference") (OtherActor :type "Actor Object Reference") (OtherComp :type "PrimitiveComponent Object Reference") (NormalImpulse :type "Vector Structure") (Hit :type "HitResult Structure (by ref)"))
  (bind (_returnvalue_x _returnvalue_y) (`KismetMathLibrary.BreakVector` (* (`KismetMathLibrary.Normal` (- (`SceneComponent.K2_GetComponentLocation` (`self.CollisionShape`)) (`SceneComponent.K2_GetComponentLocation` (`/Game/Blueprint/IMPORTED/BFL_Rock.GetPhysicPlayerRef`)))) 1800.0)))
  (cast `/Game/Blueprint/Player/BP_PlayerRock` OtherActor)
  (`PrimitiveComponent.AddImpulse` (`self.CollisionShape`) (`KismetMathLibrary.MakeVector` _returnvalue_x _returnvalue_y) "None" true))

(fn `UserConstructionScript`
  (bind _collisionshape (`self.CollisionShape`))
  (`parent.UserConstructionScript`)
  (`MeshComponent.SetVectorParameterValueOnMaterials` (`self.SM_Rock`) "Color" (`self.Color`))
  (set `self.InitialPos` (`SceneComponent.K2_GetComponentLocation` _collisionshape))
  (set `self.InitialRot` (`SceneComponent.K2_GetComponentRotation` _collisionshape)))