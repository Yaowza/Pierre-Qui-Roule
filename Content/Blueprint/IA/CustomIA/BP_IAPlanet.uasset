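; BP_IAPlanet is a physics-driven AI actor that appears to be an unfinished prototype for revolving around a point.
; Its construction script builds and debug-draws a ring of waypoints around RevolveAroundPoint, using radius, resolution and the collision shape's forward vector.
; Tick prints the direction to the current waypoint but applies a constant world-X force, never advancing the waypoint index.
; Hits print the other component's class name.
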(event `self.ReceiveHit`
  (params (MyComp :type "PrimitiveComponent Object Reference") (Other :type "Actor Object Reference") (OtherComp :type "PrimitiveComponent Object Reference") (bSelfMoved :type Boolean) (HitLocation :type "Vector Structure") (HitNormal :type "Vector Structure") (NormalImpulse :type "Vector Structure") (Hit :type "HitResult Structure (by ref)"))
  (`KismetSystemLibrary.PrintString` (`KismetSystemLibrary.GetClassDisplayName` (`GameplayStatics.GetObjectClass` OtherComp))))

(event `self.ReceiveTick`
  (params (DeltaSeconds :type "Float (single-precision)"))
  (bind _returnvalue_location (`KismetMathLibrary.BreakTransform` (`self.GetTransform` self)))
  (`parent.ReceiveTick` DeltaSeconds)
  (`KismetSystemLibrary.PrintString` (`KismetStringLibrary.Conv_VectorToString` (* (`KismetMathLibrary.GetDirectionUnitVector` _returnvalue_location (`|GetArrayItem` (`self.Points`) (`self.currentPointId`))) 100.0)))
  (`PrimitiveComponent.AddForce` (`self.CollisionShape`) (100.0 0.0 0.0) "None" false))

(fn `UserConstructionScript`
  (bind _revolveresolution (`self.RevolveResolution`))
  (`parent.UserConstructionScript`)
  (`KismetArrayLibrary.Array_Clear` (`self.Points`))
  (for _index (range (+ _revolveresolution 1))
    (bind _returnvalue (+ (`self.RevolveAroundPoint`) (* (`KismetMathLibrary.GreaterGreater_VectorRotator` (`SceneComponent.GetForwardVector` (`self.CollisionShape`)) (`KismetMathLibrary.MakeRotator` 0.0 0.0 (* _index (/ 360.0 (+ _revolveresolution 1))))) (`self.RevolveRadius`))))
    (`KismetSystemLibrary.DrawDebugSphere` _returnvalue 10.0)
    (`KismetArrayLibrary.Array_Add` (`self.Points`) _returnvalue)))