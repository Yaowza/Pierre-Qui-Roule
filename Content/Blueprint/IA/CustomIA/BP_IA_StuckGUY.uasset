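; BP_IA_StuckGUY is an AI-themed actor that can jitter in place and swaps visibility when the player rock reaches it.
; While Shaking is set, Tick uses a short random Delay to throttle small random yaw nudges on CollisionShape.
; When BP_PlayerRock begins overlapping the Sphere, the actor unhides itself and hides every actor in OtherREFS.
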(event `self.ReceiveTick`
  (params (DeltaSeconds :type "Float (single-precision)"))
  (bind _collisionshape (`self.CollisionShape`))
  (bind (_returnvalue_roll _returnvalue_pitch _returnvalue_yaw) (`KismetMathLibrary.BreakRotator` (`SceneComponent.K2_GetComponentRotation` _collisionshape)))
  (`parent.ReceiveTick` DeltaSeconds)
  (if (`self.Shaking`)
    (`KismetSystemLibrary.Delay` (`KismetMathLibrary.RandomFloatInRange` 0.0 0.1))
    (`SceneComponent.K2_SetWorldRotation` _collisionshape (`KismetMathLibrary.MakeRotator` _returnvalue_roll _returnvalue_pitch (+ _returnvalue_yaw (`KismetMathLibrary.RandomFloatInRange` -5.0 5.0))) false false)))

(event `self.Sphere.OnComponentBeginOverlap`
  (params (OverlappedComponent :type "PrimitiveComponent Object Reference") (OtherActor :type "Actor Object Reference") (OtherComp :type "PrimitiveComponent Object Reference") (OtherBodyIndex :type Integer) (bFromSweep :type Boolean) (SweepResult :type "HitResult Structure (by ref)"))
  (cast `/Game/Blueprint/Player/BP_PlayerRock` OtherActor)
  (`self.SetActorHiddenInGame` false)
  (for _array_element (`self.OtherREFS`)
    (`self.SetActorHiddenInGame` _array_element true)))

(fn `UserConstructionScript`
  (`parent.UserConstructionScript`))