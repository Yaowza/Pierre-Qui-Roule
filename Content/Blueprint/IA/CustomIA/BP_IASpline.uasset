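; BP_IASpline is an actor that repeatedly rolls a mesh along its spline, with a happy face material applied on BeginPlay.
; A looping 0.01-second timer advances distance by world delta times SpeedMultiplier, moving the mesh and adding pitch spin.
; At the spline's end, it hides the mesh, waits a random delay of up to five seconds, then restarts.
; The construction script sets mesh size from Scale.
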(event `self.ReceiveBeginPlay`
  (`self.FollowSpline`)
  (bind _returnvalue (`KismetMaterialLibrary.CreateDynamicMaterialInstance` "/Game/Art/Material/Face/M_Face.M_Face"))
  (set `self.FaceMaterial` _returnvalue)
  (`MaterialInstanceDynamic.SetTextureParameterValue` (`self.FaceMaterial`) "eyes_texture" "/Game/Art/Material/Face/e_happy.e_happy")
  (`MaterialInstanceDynamic.SetTextureParameterValue` (`self.FaceMaterial`) "mouth_texture" "/Game/Art/Material/Face/m_happy.m_happy")
  (`PrimitiveComponent.SetMaterial` (`self.SM_Face`) 0 (`self.FaceMaterial`)))

(event `FollowSpline`
  (`SceneComponent.SetHiddenInGame` (`self.StaticMesh`) false false)
  (set `self.Distance` 0.0)
  (bind _returnvalue (`KismetSystemLibrary.K2_SetTimerDelegate` (delegate `Following`) 0.01 true true)))

(event `Following`
  (bind _staticmesh (`self.StaticMesh`))
  (if (<= (`self.Distance`) (`SplineComponent.GetSplineLength` (`self.Spline`)))
    (set `self.Distance` (+ (`self.Distance`) (* (`GameplayStatics.GetWorldDeltaSeconds`) (`self.SpeedMultiplier`))))
    (`SceneComponent.K2_SetWorldLocation` _staticmesh (`SplineComponent.GetLocationAtDistanceAlongSpline` (`self.Spline`) (`self.Distance`) "World") false false)
    (`SceneComponent.K2_AddLocalRotation` _staticmesh (`KismetMathLibrary.MakeRotator` 0.0 (/ (`self.SpeedMultiplier`) 100.0)) false false)
    (else
      (`KismetSystemLibrary.K2_ClearAndInvalidateTimerHandle` (stale `FollowSpline` _returnvalue))
      (`SceneComponent.SetHiddenInGame` (`self.StaticMesh`) true false)
      (`KismetSystemLibrary.Delay` (`KismetMathLibrary.RandomFloatInRange` 0.0 5.0))
      (`self.FollowSpline`))))

(fn `UserConstructionScript`
  (`SceneComponent.SetWorldScale3D` (`self.StaticMesh`) (`KismetMathLibrary.Conv_DoubleToVector` (`self.Scale`))))