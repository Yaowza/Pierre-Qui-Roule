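; Decorative jumping character that loops the JumpingGuy1 level sequence and talks through a speech bubble widget.
; Jump and Explosion events spawn Niagara effects at the rock mesh, while StartDialogue and EndDialogue show or hide the bubble.
; Bonjour and Aurevoir write greeting and farewell lines; once Trigger01 sets Passé, both share a one-time cheer instead.
; The construction script builds a dynamic face material with happy eyes and mouth.
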(event `self.ReceiveBeginPlay`
  (bind (_outactor _returnvalue) (`LevelSequencePlayer.CreateLevelSequencePlayer` "/Game/Cinematic/TrucsRigolosDansLaMap/JumpingGuy1.JumpingGuy1"))
  (`MovieSceneSequencePlayer.PlayLooping` _returnvalue -1)
  (`MovieSceneSequencePlayer.PlayLooping` (`LevelSequenceActor.SequencePlayer` _outactor) -1)
  (`MovieSceneSequencePlayer.Play` (`LevelSequenceActor.SequencePlayer` _outactor))
  (`self.Bonjour`)
  (set `Widget.RenderOpacity` 0.0 (`WidgetComponent.GetWidget` (`self.WBP_Bubble`))))

(event `Explosion`
  (`NiagaraFunctionLibrary.SpawnSystemAtLocation` "/Game/VFX/Dash/NS_DashGroundSoft.NS_DashGroundSoft" (`SceneComponent.K2_GetComponentLocation` (`self.SM_Rock`))))

(event `Jump`
  (`NiagaraFunctionLibrary.SpawnSystemAtLocation` "/Game/VFX/Jump/NS_Jump2.NS_Jump2" (`SceneComponent.K2_GetComponentLocation` (`self.SM_Rock`))))

(event `Bonjour`
  (bind _aswbp_bubble (cast `/Game/UI/WBP/WBP_Bubble` (`WidgetComponent.GetWidget` (`self.WBP_Bubble`)) :!pure true))
  (bind _aswbp_bubble_2 (cast `/Game/UI/WBP/WBP_Bubble` (`WidgetComponent.GetWidget` (`self.WBP_Bubble`)) :!pure true))
  (if (`self.Passé`)
    (`/Engine/EditorBlueprintResources/StandardMacros.DoOnce` false :!label _label
      (:`Completed`
        (set `/Game/UI/WBP/WBP_Bubble.DialogueWrintingSpeed` 0.01 _aswbp_bubble)
        (set `/Game/UI/WBP/WBP_Bubble.DialogueText` "Youpiiiiiiiiiii !!" _aswbp_bubble)
        (set `/Game/UI/WBP/WBP_Bubble.With Sound` false _aswbp_bubble)
        (`/Game/UI/WBP/WBP_Bubble.PlayDialogue` _aswbp_bubble)))
    (else
      (set `/Game/UI/WBP/WBP_Bubble.DialogueWrintingSpeed` 0.01 _aswbp_bubble_2)
      (set `/Game/UI/WBP/WBP_Bubble.DialogueText` "Bonjour !" _aswbp_bubble_2)
      (set `/Game/UI/WBP/WBP_Bubble.With Sound` false _aswbp_bubble_2)
      (`/Game/UI/WBP/WBP_Bubble.PlayDialogue` _aswbp_bubble_2))))

(event `Aurevoir`
  (bind _aswbp_bubble (cast `/Game/UI/WBP/WBP_Bubble` (`WidgetComponent.GetWidget` (`self.WBP_Bubble`)) :!pure true))
  (if (`self.Passé`)
    (goto _label)
    (else
      (set `/Game/UI/WBP/WBP_Bubble.DialogueWrintingSpeed` 0.01 _aswbp_bubble)
      (set `/Game/UI/WBP/WBP_Bubble.DialogueText` "Aurevoir !" _aswbp_bubble)
      (set `/Game/UI/WBP/WBP_Bubble.With Sound` false _aswbp_bubble)
      (`/Game/UI/WBP/WBP_Bubble.PlayDialogue` _aswbp_bubble))))

(event `/Game/Blueprint/Interface/BPI_Rock.StartDialogue`
  (set `Widget.RenderOpacity` 1.0 (`WidgetComponent.GetWidget` (`self.WBP_Bubble`))))

(event `/Game/Blueprint/Interface/BPI_Rock.EndDialogue`
  (set `Widget.RenderOpacity` 0.0 (`WidgetComponent.GetWidget` (`self.WBP_Bubble`))))

(event `/Game/Blueprint/Interface/BPI_Rock.Trigger01`
  (set `self.Passé` true))

(fn `UserConstructionScript`
  (bind _returnvalue (`KismetMaterialLibrary.CreateDynamicMaterialInstance` "/Game/Art/Material/Face/M_Face.M_Face"))
  (set `self.FaceMaterial` _returnvalue)
  (`MaterialInstanceDynamic.SetTextureParameterValue` (`self.FaceMaterial`) "eyes_texture" (select `/Game/Art/Material/Face/E_eyes` "NewEnumerator0" :`NewEnumerator0` (`self.eyes_happy_texture`)))
  (`MaterialInstanceDynamic.SetTextureParameterValue` (`self.FaceMaterial`) "mouth_texture" (select `/Game/Art/Material/Face/E_mouth` "NewEnumerator0" :`NewEnumerator0` (`self.mouth_happy_texture`)))
  (`PrimitiveComponent.SetMaterial` (`self.SM_Face`) 0 (`self.FaceMaterial`)))