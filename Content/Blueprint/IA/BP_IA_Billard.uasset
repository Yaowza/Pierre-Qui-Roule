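; Billiard ball actor for a billiard puzzle that reacts when its Enter event marks it as in.
; Enter counts in balls in its Boule list; if this is the black ball and all but at most one are in, it pushes an achievement and completes every BP_Billard.
; Otherwise, it stops the listed balls and returns them to starting transforms, leaving IsIn unchanged.
; Construction tints the mesh and records that transform.
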(event `Enter`
  (set `self.IsIn?` true)
  (set `self.NewVar_0` 0)
  (for _array_element (`self.Boule`)
    (if (`/Game/Blueprint/IA/BP_IA_Billard.IsIn?` _array_element)
      (set `self.NewVar_0` (+ (`self.NewVar_0`) 1))))
  (if (and (`self.Black`) (>= (`self.NewVar_0`) (- (`KismetArrayLibrary.Array_Length` (`self.Boule`)) 1)))
    (`/Game/Blueprint/BFL_Rock.PushAchievement` 8)
    (bind _outactors (`GameplayStatics.GetAllActorsOfClass` "/Game/Blueprint/BP_Billard.BP_Billard_C"))
    (for _array_element_2 _outactors
      (`/Game/Blueprint/BP_Billard.Complete` _array_element_2))
    (else
      (for _array_element_3 (`self.Boule`)
        (bind _collisionshape (`/Game/Blueprint/IA/BP_IARock.CollisionShape` _array_element_3))
        (`PrimitiveComponent.SetPhysicsLinearVelocity` _collisionshape (0.0 0.0 0.0) false "None")
        (`PrimitiveComponent.SetPhysicsAngularVelocityInDegrees` _collisionshape (0.0 0.0 0.0) false "None")
        (`SceneComponent.K2_SetWorldLocationAndRotation` _collisionshape (`/Game/Blueprint/IA/BP_IA_Billard.InitialPos` _array_element_3) (`/Game/Blueprint/IA/BP_IA_Billard.InitialRot` _array_element_3) false false)))))

(fn `UserConstructionScript`
  (bind _collisionshape (`self.CollisionShape`))
  (`parent.UserConstructionScript`)
  (`MeshComponent.SetVectorParameterValueOnMaterials` (`self.SM_Rock`) "Color" (`self.Color`))
  (set `self.InitialPos` (`SceneComponent.K2_GetComponentLocation` _collisionshape))
  (set `self.InitialRot` (`SceneComponent.K2_GetComponentRotation` _collisionshape)))