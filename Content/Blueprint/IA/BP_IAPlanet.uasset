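; Celestial body actor that acts either as a slowly spinning sun or as a physics-driven planet orbiting a point, taken from SunRef when set.
; BeginPlay stores the orbit radius and gives a perpendicular launch impulse, with physics simulation enabled only for planets.
; Each Tick applies a centripetal force plus a smaller perpendicular one, both scaled by radius and Scale.
; The construction script previews the orbit as a debug circle and applies any material override.
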(event `self.ReceiveBeginPlay`
  (bind _sunref (`self.SunRef`))
  (bind _materialoverride (`self.MaterialOverride`))
  (`parent.ReceiveBeginPlay`)
  (`PrimitiveComponent.SetSimulatePhysics` (`self.CollisionShape`) (not (`self.IsSun`)))
  (if (`KismetSystemLibrary.IsValid` _sunref)
    (set `self.RevolveAroundPoint` (`self.K2_GetActorLocation` _sunref))
    (if (`KismetSystemLibrary.IsValid` _materialoverride)
      (`PrimitiveComponent.SetMaterial` (`self.SM_Rock`) 0 _materialoverride)))
  (set `self.RevolveRadius` (`KismetMathLibrary.Vector_Distance` (`SceneComponent.K2_GetComponentLocation` (`self.CollisionShape`)) (`self.RevolveAroundPoint`)))
  (`PrimitiveComponent.AddImpulse` (`self.CollisionShape`) (* (`KismetMathLibrary.GreaterGreater_VectorRotator` (`KismetMathLibrary.GetDirectionUnitVector` (`SceneComponent.K2_GetComponentLocation` (`self.CollisionShape`)) (`self.RevolveAroundPoint`)) (struct :`Yaw` -90.0)) (* (`self.RevolveRadius`) 200.0 (`self.Scale`))) "None" false))

(event `self.ReceiveTick`
  (params (DeltaSeconds :type "Float (single-precision)"))
  (bind _revolvearoundpoint (`self.RevolveAroundPoint`))
  (bind _collisionshape (`self.CollisionShape`))
  (bind _returnvalue (`SceneComponent.K2_GetComponentLocation` (`self.CollisionShape`)))
  (`parent.ReceiveTick` DeltaSeconds)
  (if (`self.IsSun`)
    (`SceneComponent.K2_AddWorldRotation` (`self.CollisionShape`) (struct :`Yaw` 0.15) false false)
    (else
      (`PrimitiveComponent.AddForce` _collisionshape (* (`KismetMathLibrary.GetDirectionUnitVector` _returnvalue _revolvearoundpoint) 200.0 (`self.RevolveRadius`) (`self.Scale`)) "None" false)
      (`PrimitiveComponent.AddForce` _collisionshape (* (`KismetMathLibrary.GreaterGreater_VectorRotator` (`KismetMathLibrary.GetDirectionUnitVector` _revolvearoundpoint _returnvalue) (struct :`Yaw` 90.0)) 20.0 (`self.RevolveRadius`) (`self.Scale`)) "None" false))))

(fn `UserConstructionScript`
  (bind _revolvearoundpoint (`self.RevolveAroundPoint`))
  (bind _materialoverride (`self.MaterialOverride`))
  (`parent.UserConstructionScript`)
  (bind _output_get (set `self.RevolveRadius` (`KismetMathLibrary.Vector_Distance` _revolvearoundpoint (`SceneComponent.K2_GetComponentLocation` (`self.CollisionShape`)))))
  (`KismetSystemLibrary.DrawDebugCircle` _revolvearoundpoint _output_get 32 (struct :`R` 1.0 :`G` 1.0 :`B` 1.0 :`A` 1.0) 0.0 0.0 (0.0 1.0 0.0) (1.0 0.0 0.0))
  (if (`KismetSystemLibrary.IsValid` _materialoverride)
    (`PrimitiveComponent.SetMaterial` (`self.SM_Rock`) 0 _materialoverride)))