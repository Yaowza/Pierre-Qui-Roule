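; AI aviator actor that flies its collision shape along a plane spline in an endless loop.
; A timeline drives the distance along the spline, turning the shape toward a point slightly ahead.
; A sliding altitude window of AppexRange height scales the timeline play rate each update, slowing climbs and speeding up dives to mimic momentum.
; The window recenters on the actor's height when each lap restarts.
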(event `self.ReceiveBeginPlay`
  (bind (_returnvalue_x _returnvalue_y _returnvalue_z) (`KismetMathLibrary.BreakVector` (`self.K2_GetActorLocation`)))
  (bind (_returnvalue_x_2 _returnvalue_y_2 _returnvalue_z_2) (`KismetMathLibrary.BreakVector` (`self.K2_GetActorLocation`)))
  (bind _appexrange (`self.AppexRange`))
  (bind _appexrange_2 (`self.AppexRange`))
  (bind _appexrange_3 (`self.AppexRange`))
  (bind (_returnvalue_x_3 _returnvalue_y_3 _returnvalue_z_3) (`KismetMathLibrary.BreakVector` (`SceneComponent.K2_GetComponentLocation` (`self.CollisionShape`))))
  (bind (_returnvalue_x_4 _returnvalue_y_4 _returnvalue_z_4) (`KismetMathLibrary.BreakVector` (`SceneComponent.K2_GetComponentLocation` (`self.CollisionShape`))))
  (bind (_returnvalue_x_5 _returnvalue_y_5 _returnvalue_z_5) (`KismetMathLibrary.BreakVector` (`SceneComponent.K2_GetComponentLocation` (`self.CollisionShape`))))
  (bind (_returnvalue_x_6 _returnvalue_y_6 _returnvalue_z_6) (`KismetMathLibrary.BreakVector` (`SceneComponent.K2_GetComponentLocation` (`self.CollisionShape`))))
  (`parent.ReceiveBeginPlay`)
  (`TimelineComponent.SetPlayRate` (`self.Timeline`) (`self.PlayRate`))
  (set `self.ZTopApex` (+ _returnvalue_z _appexrange))
  (set `self.ZBotApex` (- _returnvalue_z _appexrange))
  (bind (_direction _newtrack_0) (`Timeline|Timeline` :!label _label)
    (:`Update`
      (set `self.lastZpos` _returnvalue_z_4)
      (bind _returnvalue (* _newtrack_0 (`SplineComponent.GetSplineLength` (`self.PlaneSpline`))))
      (`SceneComponent.K2_SetWorldLocation` (`self.CollisionShape`) (+ (`SplineComponent.GetLocationAtDistanceAlongSpline` (`self.PlaneSpline`) _returnvalue "Local") (`self.K2_GetActorLocation`)) false false)
      (`SceneComponent.K2_SetWorldRotation` (`self.CollisionShape`) (`KismetMathLibrary.FindLookAtRotation` (`SceneComponent.K2_GetComponentLocation` (`self.CollisionShape`)) (`SplineComponent.GetLocationAtDistanceAlongSpline` (`self.PlaneSpline`) (+ _returnvalue 1.0) "World")) false false)
      (if (< _returnvalue_z_6 (`self.ZBotApex`))
        (set `self.ZBotApex` _returnvalue_z_6)
        (set `self.ZTopApex` (+ _returnvalue_z_6 (`self.AppexRange`))))
      (if (> _returnvalue_z_3 (`self.ZTopApex`))
        (set `self.ZTopApex` _returnvalue_z_3)
        (set `self.ZBotApex` (- _returnvalue_z_3 (`self.AppexRange`))))
      (`TimelineComponent.SetPlayRate` (`self.Timeline`) (* (`self.PlayRate`) (select `bool` (> (- _returnvalue_z_5 (`self.lastZpos`)) 0.0) :`false` (`KismetMathLibrary.MapRangeClamped` (- (`self.ZTopApex`) (`self.lastZpos`)) 0.0 _appexrange_2 0.4 1.0) :`true` (`KismetMathLibrary.MapRangeClamped` (- (`self.lastZpos`) (`self.ZBotApex`)) 0.0 _appexrange_2 1.0 0.4) :!type "Float (single-precision)"))))
    (:`Finished`
      (set `self.ZTopApex` (+ _returnvalue_z_2 _appexrange_3))
      (set `self.ZBotApex` (- _returnvalue_z_2 _appexrange_3))
      (`self.Loop`))))

(event `Loop`
  (goto _label :!via `PlayFromStart`))

(fn `UserConstructionScript`
  (`parent.UserConstructionScript`))