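; BP_Pool is a scalable mesh that scatters randomly sized rocks with faces inside a box volume.
; The construction script scales the mesh, flashes the debug bounds, then adds paired rock and face HISM instances, clearing only the rocks beforehand.
; A random stream seeds position and scale, while rotation and three per-rock custom data values are unseeded.
; On BeginPlay, a dynamic material gives all faces happy eye and mouth textures.
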(event `self.ReceiveBeginPlay`
  (bind _returnvalue (`KismetMaterialLibrary.CreateDynamicMaterialInstance` "/Game/Art/Material/Face/M_Face.M_Face"))
  (set `self.FaceMaterial` _returnvalue)
  (`MaterialInstanceDynamic.SetTextureParameterValue` (`self.FaceMaterial`) "eyes_texture" "/Game/Art/Material/Face/e_happy.e_happy")
  (`MaterialInstanceDynamic.SetTextureParameterValue` (`self.FaceMaterial`) "mouth_texture" "/Game/Art/Material/Face/m_happy.m_happy")
  (`PrimitiveComponent.SetMaterial` (`self.HISM_Face`) 0 (`self.FaceMaterial`)))

(fn `UserConstructionScript`
  (bind (_spawntransform_location _spawntransform_rotation _spawntransform_scale) (`KismetMathLibrary.BreakTransform` (`self.SpawnTransform`)))
  (bind _stream (`self.Stream`))
  (bind _hism_rock (`self.HISM_Rock`))
  (bind _returnvalue (`SceneComponent.K2_GetComponentLocation` (`self.HISM_Rock`)))
  (bind _returnvalue_2 (* (`self.Half Size`) (`self.New Scale`)))
  (`SceneComponent.SetWorldScale3D` (`self.StaticMesh`) (`self.New Scale`))
  (`InstancedStaticMeshComponent.ClearInstances` (`self.HISM_Rock`))
  (`KismetSystemLibrary.DrawDebugBox` _returnvalue _returnvalue_2 (struct :`R` 1.0 :`B` 0.037968 :`A` 1.0) (struct) 0.2 2.0)
  (for _ (range (+ (`self.RockNumber`) 1))
    (set `self.SpawnTransform` (`KismetMathLibrary.MakeTransform` (`KismetMathLibrary.RandomPointInBoundingBoxFromStream` _stream _returnvalue _returnvalue_2) (`KismetMathLibrary.RandomRotator` false) (`KismetMathLibrary.Conv_DoubleToVector` (`KismetMathLibrary.RandomFloatInRangeFromStream` _stream 0.5 2.0))))
    (`InstancedStaticMeshComponent.AddInstance` (`self.HISM_Face`) (`KismetMathLibrary.MakeTransform` _spawntransform_location _spawntransform_rotation (/ _spawntransform_scale 10.0)) true)
    (bind _returnvalue_3 (`InstancedStaticMeshComponent.AddInstance` (`self.HISM_Rock`) (`self.SpawnTransform`) true))
    (`InstancedStaticMeshComponent.SetCustomDataValue` _hism_rock _returnvalue_3 0 (`KismetMathLibrary.RandomFloatInRange` 0.0 1.0) false)
    (`InstancedStaticMeshComponent.SetCustomDataValue` _hism_rock _returnvalue_3 1 (`KismetMathLibrary.RandomFloatInRange` 0.0 1.0) false)
    (`InstancedStaticMeshComponent.SetCustomDataValue` _hism_rock _returnvalue_3 2 (`KismetMathLibrary.RandomFloatInRange` 0.0 1.0) false)))