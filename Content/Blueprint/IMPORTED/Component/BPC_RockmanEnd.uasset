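; BPC_RockmanEnd is a component that plays the exit sequence for the Rockman actor (BP_IA_Rockman).
; On BeginPlay it plays the Rockman sound, finds the actor in the level, stops its bubble dialogue system and resets its rotation.
; A fast looping timer then spins and slides the actor along world X in fixed per-tick steps until a delay ends and the actor is destroyed.
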(event `self.ReceiveBeginPlay`
  (`GameplayStatics.PlaySound2D` "/Game/Audio/Sounds/SFX/Rockman/SC_Rockman.SC_Rockman" 1.0 1.0 0.0 null null)
  (bind _returnvalue (`GameplayStatics.GetActorOfClass` "/Game/Blueprint/IA/CustomIA/BP_IA_Rockman.BP_IA_Rockman_C"))
  (bind _output_get (set `self.RockmanRef` _returnvalue))
  (bind _bpc_bubble (`/Game/Blueprint/IA/BP_IARock.BPC_Bubble` _output_get))
  (`/Game/Blueprint/IMPORTED/Component/BPC_Bubble.StopDialogue` _bpc_bubble)
  (`/Game/Blueprint/IMPORTED/Component/BPC_IA.StopSystem` _bpc_bubble)
  (`Actor.K2_SetActorRotation` :`self` (`self.RockmanRef`))
  (bind _returnvalue_2 (`KismetSystemLibrary.K2_SetTimerDelegate` (delegate `Anim`) 0.01 true true))
  (`KismetSystemLibrary.Delay` 5.0)
  (`KismetSystemLibrary.K2_ClearAndInvalidateTimerHandle` _returnvalue_2)
  (`Actor.K2_DestroyActor` (`self.RockmanRef`)))

(event `Anim`
  (bind _rockmanref (`self.RockmanRef`))
  (`Actor.K2_AddActorLocalRotation` _rockmanref (struct :`Pitch` 3.5) false false)
  (`Actor.K2_AddActorWorldOffset` _rockmanref (-3.0 0.0 0.0) false false))