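; BPC_IA is a base component for BP_IARock actors that detects whether the player is within a radius of its owner.
; On BeginPlay it caches the owning rock and optionally auto-starts.
; Start and stop events control a fast looping timer that compares the rock's distance to the player against SystemRadius.
; Each check fires PlayerInRange or PlayerOutRange, both empty hooks, and a getter exposes the rock and its collision shape.
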(event `self.ReceiveBeginPlay`
  ;[0 1 0.5794] Begin Play
  (bind _asbp_iarock (cast `/Game/Blueprint/IA/BP_IARock` (`self.GetOwner`)))
  (set `self.ParentRef` _asbp_iarock)
  (if (`self.AutoStart?`)
    (`self.StartSystem`)))

(event `StopSystem`
  ;[1 0.2165 0.7284] Start & Stop Component Systems
  (`self.ClearCheckingPlayer`)
  (set `self.SystemActive?` false))

(event `StartSystem`
  ;[1 0.2165 0.7284] Start & Stop Component Systems
  (`self.StartCHeckingPlayer`)
  (set `self.SystemActive?` true))

(event `StartCHeckingPlayer`
  ;[1 0.2165 0.7284] System Update
  (bind _returnvalue (`KismetSystemLibrary.K2_SetTimerDelegate` (delegate `CheckingPlayer`) 0.01 true true)))

(event `ClearCheckingPlayer`
  ;[1 0.2165 0.7284] System Update
  (`KismetSystemLibrary.K2_ClearAndInvalidateTimerHandle` (stale `StartCHeckingPlayer` _returnvalue)))

(event `CheckingPlayer`
  ;[1 0.2165 0.7284] System Update
  (if (<= (`/Game/Blueprint/IA/BP_IARock.GetDistanceToPlayer` (`self.ParentRef`)) (`self.SystemRadius`))
    (`self.PlayerInRange`)
    (else
      (`self.PlayerOutRange`))))

(event `PlayerInRange`
  ;[1 0.2165 0.7284] System Update
)

(event `PlayerOutRange`
  ;[1 0.2165 0.7284] System Update
)

(fn `GetParentRef`
  (returns (ParentRef :type "/Game/Blueprint/IA/BP_IARock Object Reference") (CollisionShape :type "StaticMeshComponent Object Reference"))
  (bind _parentref (`self.ParentRef`))
  (return _parentref (`/Game/Blueprint/IA/BP_IARock.CollisionShape` _parentref)))