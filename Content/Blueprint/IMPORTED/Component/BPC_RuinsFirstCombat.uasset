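; Actor component that kicks off the first combat encounter in the Ruins, expected on a BP_IARock owner.
; One second after BeginPlay, it calls StartSystem on the owner's BPCCombatSystem.
; It then does the same on the first BP_IARock found with the FirstCombat tag, with no check that one exists.
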(event `self.ReceiveBeginPlay`
  (bind _asbp_iarock (cast `/Game/Blueprint/IA/BP_IARock` (`self.GetOwner`)))
  (set `self.As BP IARock` _asbp_iarock)
  (`KismetSystemLibrary.Delay` 1.0)
  (`/Game/Blueprint/IMPORTED/Component/BPC_IA.StartSystem` (`/Game/Blueprint/IA/BP_IARock.BPC_CombatSystem` (`self.As BP IARock`)))
  (bind _outactors (`GameplayStatics.GetAllActorsOfClassWithTag` "/Game/Blueprint/IA/BP_IARock.BP_IARock_C" "FirstCombat"))
  (`/Game/Blueprint/IMPORTED/Component/BPC_IA.StartSystem` (`/Game/Blueprint/IA/BP_IARock.BPC_CombatSystem` (`|GetArrayItem` _outactors))))