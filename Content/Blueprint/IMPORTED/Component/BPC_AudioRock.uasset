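; Audio component for a rolling rock that drives its rolling and impact sounds.
; Initialize attaches a looping rolling sound and moves the audio listener to the player's camera; Tick sets its volume and pitch from speed while grounded, muting it otherwise.
; Impact picks a sound by collision profile or hit actor class (bell, wood/foliage, rock, default), with bells also spawning a Niagara effect.
; MapVelocity scales these values from the moving component's parent velocity.
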(event `Initialize`
  (params (MovingComponent :type "StaticMeshComponent Object Reference") (MaxSpeed :type "Float (double-precision)"))
  (set `self.Moving Component` MovingComponent)
  (bind _returnvalue (`GameplayStatics.SpawnSoundAttached` "/Game/Audio/Sounds/SFX/Rolling/SC_Rolling.SC_Rolling" (`self.Moving Component`) "None" (0.0 0.0 0.0) (struct) "SnapToTarget" false 1.0 1.0 0.0 null null false))
  (set `self.RollingSoundRef` _returnvalue)
  (`AudioComponent.Play` _returnvalue 0.0)
  (set `self.MaxSpeed` MaxSpeed)
  (set `self.Initialised?` true)
  (`PlayerController.SetAudioListenerOverride` :`self` (`GameplayStatics.GetPlayerController` 0) :`AttachToComponent` (`/Game/Blueprint/Player/BP_PlayerRock.GetCurrentCameraUsed` (`/Game/Blueprint/IMPORTED/BFL_Rock.GetPlayerActorRef`))))

(event `self.ReceiveTick`
  (params (DeltaSeconds :type "Float (single-precision)"))
  (bind _maxspeed (`self.MaxSpeed`))
  (bind _rollingsoundref (`self.RollingSoundRef`))
  (if (`self.Initialised?`)
    (if (`self.Grounded?`)
      (`AudioComponent.SetFloatParameter` _rollingsoundref "RollingVolume" (`self.MapVelocity` 0.0 _maxspeed 0.0 3.0))
      (`AudioComponent.SetFloatParameter` _rollingsoundref "RollingPitch" (`self.MapVelocity` 0.0 _maxspeed 0.0 2.0))
      (else
        (`AudioComponent.SetFloatParameter` (`self.RollingSoundRef`) "RollingVolume" 0.0)
        (`AudioComponent.SetFloatParameter` (`self.RollingSoundRef`) "RollingFoliageVolume" 0.0)))))

(event `Impact`
  (params (Hit :type "HitResult Structure (by ref)"))
  (bind (_bblockinghit _binitialoverlap _time _distance _location _impactpoint _normal _impactnormal _physmat _hitactor) (`GameplayStatics.BreakHitResult` Hit))
  (bind _maxspeed (`self.MaxSpeed`))
  (bind _maxspeed_2 (`self.MaxSpeed`))
  (bind _maxspeed_3 (`self.MaxSpeed`))
  (bind _returnvalue (`self.MapVelocity` 0.0 (`self.MaxSpeed`) 0.0 2.0))
  (bind _returnvalue_2 (`self.MapVelocity` 0.0 _maxspeed 0.0 2.0))
  (set `self.Location` _location)
  (bind _asstatic_mesh_actor (cast `StaticMeshActor` _hitactor)
    (:`then`
      (bind _returnvalue_3 (`PrimitiveComponent.GetCollisionProfileName` (`StaticMeshActor.StaticMeshComponent` _asstatic_mesh_actor)))
      (if (== _returnvalue_3 "Bell")
        (`GameplayStatics.PlaySoundAtLocation` "/Game/Audio/Sounds/SFX/Bell/SC_Bell.SC_Bell" (`self.Location`) (struct) _returnvalue_2 (`self.MapVelocity` 0.0 _maxspeed 0.0 4.0) 0.0 null null null null)
        (`NiagaraFunctionLibrary.SpawnSystemAtLocation` "/Game/ART_Imported/VFX/Cloches/NS_ClochesSound.NS_ClochesSound" (`self.Location`) (struct) (`KismetMathLibrary.Conv_DoubleToVector` _returnvalue_2))
        (elif (== _returnvalue_3 "Wood")
          (`GameplayStatics.PlaySoundAtLocation` "/Game/Audio/Sounds/SFX/Impact/SC_WoodImpact.SC_WoodImpact" (`self.Location`) (struct) (`self.MapVelocity` 0.0 _maxspeed_3 0.0 2.0) (`self.MapVelocity` 0.0 _maxspeed_3 0.0 2.0) 0.0 null null null null :!label _label)
          (else
            (`GameplayStatics.PlaySoundAtLocation` "/Game/Audio/Sounds/SFX/Landing/SC_Impact.SC_Impact" (`self.Location`) (struct) (`self.MapVelocity` 0.0 _maxspeed_2 0.0 2.0) (`self.MapVelocity` 0.0 _maxspeed_2 0.0 4.0) 0.0 null null null null :!label _label_2)))))
    (:`CastFailed`
      (cast `InstancedFoliageActor` _hitactor
        (:`then`
          (goto _label))
        (:`CastFailed`
          (cast `/Game/Blueprint/Player/BP_PlayerRock` _hitactor
            (:`then`
              _)
            (:`CastFailed`
              (cast `/Game/Blueprint/IA/BP_IARock` _hitactor
                (:`then`
                  _)
                (:`CastFailed`
                  (goto _label_2)))))
          (`GameplayStatics.PlaySoundAtLocation` "/Game/Audio/Sounds/SFX/Impact/SC_Rock_Impact.SC_Rock_Impact" (`self.Location`) (struct) _returnvalue _returnvalue 0.0 null null null null))))))

(fn `MapVelocity`
  (params (InRangeA :type "Float (double-precision)") (InRangeB :type "Float (double-precision)") (OutRangeA :type "Float (double-precision)") (OutRangeB :type "Float (double-precision)"))
  (returns (ReturnValue :type "Float (double-precision)"))
  (return (`KismetMathLibrary.MapRangeClamped` (`KismetMathLibrary.VSize` (`SceneComponent.GetComponentVelocity` (`|GetArrayItem` (`SceneComponent.GetParentComponents` (`self.Moving Component`))))) InRangeA InRangeB OutRangeA OutRangeB)))