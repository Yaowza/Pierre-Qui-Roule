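; Blueprint function library of shared helpers for a game with a BP_PlayerRock pawn.
; Player getters return player 0's pawn, or its moving component when that simulates physics.
; Achievement and level-data helpers forward to GM_Rock, reading and writing its Levels array.
; CameraBlend lerps location in a loop without delays, so it finishes within one frame, using the unnormalized counter as alpha.
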(fn `CameraBlend`
  (params (CamStart :type "CameraComponent Object Reference") (CamTarget :type "CameraComponent Object Reference") (BlendDuration :type "Float (double-precision)"))
  (locals (BlendVal :type "Float (double-precision)") (StartCamLocation :type "Vector Structure" :default (0.0 0.0 0.0)))
  (set `local.StartCamLocation` (`SceneComponent.K2_GetComponentLocation` CamStart))
  (set `local.BlendVal` 0.0)
  (if (not (>= (`local.BlendVal`) BlendDuration)) :!label _label
    (set `local.BlendVal` (+ (`local.BlendVal`) 0.01))
    (`SceneComponent.K2_SetWorldLocation` CamStart (`KismetMathLibrary.VLerp` (`local.StartCamLocation`) (`SceneComponent.K2_GetComponentLocation` CamTarget) (`local.BlendVal`)) false false)
    (goto _label)))

(fn `Get Level Data`
  (params (`Level Index` :type Integer))
  (returns (`Level Data` :type "/Game/Blueprint/Player/F_LevelData Structure"))
  (bind _asgm_rock (cast `/Game/Blueprint/Player/GM_Rock` (`GameplayStatics.GetGameMode` null)))
  (return (`|GetArrayItem` (`/Game/Blueprint/Player/GM_Rock.Levels` _asgm_rock) `Level Index`)))

(fn `GetPhysicPlayerRef`
  (returns (MovingComponent :type "SphereComponent Object Reference"))
  (bind _asbp_player_rock (cast `/Game/Blueprint/Player/BP_PlayerRock` (`GameplayStatics.GetPlayerPawn` null)))
  (bind _movingcomponent (`/Game/Blueprint/Player/BP_PlayerRock.GetMovingComponent` _asbp_player_rock))
  (if (`SceneComponent.IsSimulatingPhysics` _movingcomponent "None")
    (return _movingcomponent)))

(fn `GetPlayerActorRef`
  (returns (`AsBP Player Rock` :type "/Game/Blueprint/Player/BP_PlayerRock Object Reference"))
  (bind _asbp_player_rock (cast `/Game/Blueprint/Player/BP_PlayerRock` (`GameplayStatics.GetPlayerPawn` null)))
  (return _asbp_player_rock))

(fn `PushAchievement`
  (params (Index :type Integer))
  (bind _asgm_rock (cast `/Game/Blueprint/Player/GM_Rock` (`GameplayStatics.GetGameMode` null)))
  (`/Game/Blueprint/Player/GM_Rock.Push Achievement` _asgm_rock Index))

(fn `SetLevelData`
  (params (Index :type Integer) (Item :type "/Game/Blueprint/Player/F_LevelData Structure (by ref)"))
  (bind _asgm_rock (cast `/Game/Blueprint/Player/GM_Rock` (`GameplayStatics.GetGameMode` null)))
  (`KismetArrayLibrary.Array_Set` (`/Game/Blueprint/Player/GM_Rock.Levels` _asgm_rock) Index Item))