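; BP_TrailGrass is an actor that builds a tapered chain of static mesh trail segments, named for interactive grass.
; Its construction script clears and rebuilds the segments along local X, shrinking Y and Z scale magnitude toward zero.
; BeginPlay detaches the segments in world space.
; Tick is empty; the lerp-based follow logic and the MPC_GrassInteractive player-position write are unconnected, so the trail never updates.
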(event `self.ReceiveBeginPlay`
  (for _array_element (`self.TrailObjects`)
    (`SceneComponent.K2_DetachFromComponent` _array_element "KeepWorld" "KeepWorld" "KeepWorld" true)))

(event `self.ReceiveTick`
  (params (DeltaSeconds :type "Float (single-precision)")))

(fn `AddTrailObjects`
  (params (TrailSegmentCount :type Integer :default 10) (`Trail Width` :type "Float (double-precision)" :default 100.0))
  (bind _trailsegmentcount (`local.TrailSegmentCount`))
  (bind _trail_width (`local.Trail Width`))
  (bind _returnvalue (/ _trail_width (`self.TrailObjectScale`)))
  (`self.ClearTrailObject`)
  (for _index (range (+ TrailSegmentCount 1))
    (bind _returnvalue_2 (* _returnvalue (/ (- _index _trailsegmentcount) _trailsegmentcount)))
    (bind _returnvalue_3 (`AddComponent|NODE_AddStaticMeshComponent-0` :`RelativeTransform` (`KismetMathLibrary.MakeTransform` (`KismetMathLibrary.MakeVector` (* _index _trail_width)) (struct) (`KismetMathLibrary.MakeVector` _returnvalue _returnvalue_2 _returnvalue_2))))
    (`KismetArrayLibrary.Array_Add` (`self.TrailObjects`) _returnvalue_3)))

(fn `ClearTrailObject`
  (bind _trailobjects (`self.TrailObjects`))
  (for _array_element _trailobjects
    (`ActorComponent.K2_DestroyComponent` _array_element))
  (`KismetArrayLibrary.Array_Clear` _trailobjects))

(fn `UserConstructionScript`
  (`self.AddTrailObjects` 10))