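; BP_Fountain is a fountain actor that awards an achievement when the player rock (BP_PlayerRock) stays inside its sphere trigger for about a second.
; Begin and end overlap update an IsIn flag and share a retriggerable delay, so leaving early restarts the timer and fails the check.
; If the rock is still inside when it expires, the Blueprint pushes the achievement, activates confetti and plays a fountain sound shortly after.
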(event `self.Sphere.OnComponentBeginOverlap`
  (params (OverlappedComponent :type "PrimitiveComponent Object Reference") (OtherActor :type "Actor Object Reference") (OtherComp :type "PrimitiveComponent Object Reference") (OtherBodyIndex :type Integer) (bFromSweep :type Boolean) (SweepResult :type "HitResult Structure (by ref)"))
  (cast `/Game/Blueprint/Player/BP_PlayerRock` OtherActor)
  (set `self.IsIn?` true)
  (`KismetSystemLibrary.RetriggerableDelay` 1.0 :!label _label)
  (if (`self.IsIn?`)
    (`/Game/Blueprint/IMPORTED/BFL_Rock.PushAchievement` 2)
    (`ActorComponent.Activate` (`self.NS_Confettis`) true)
    (`KismetSystemLibrary.Delay` 0.25)
    (`GameplayStatics.PlaySoundAtLocation` "/Game/Audio/Sounds/SFX/Firework/SC_Fountain.SC_Fountain" (`SceneComponent.K2_GetComponentLocation` (`self.NS_Confettis`)) (struct) 1.0 1.0 0.0 null null null null)))

(event `self.Sphere.OnComponentEndOverlap`
  (params (OverlappedComponent :type "PrimitiveComponent Object Reference") (OtherActor :type "Actor Object Reference") (OtherComp :type "PrimitiveComponent Object Reference") (OtherBodyIndex :type Integer))
  (cast `/Game/Blueprint/Player/BP_PlayerRock` OtherActor)
  (set `self.IsIn?` false)
  (goto _label))

(fn `UserConstructionScript`)