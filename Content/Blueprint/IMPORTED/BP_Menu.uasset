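; Menu actor that shows the main menu through its own camera and hands control over to the player.
; InitializeCamera makes itself the view target, creates WBP_MainMenu and enables the cursor.
; Play closes the widget, blends to the player's third-person camera, then initializes the player after the blend.
; OpenWidget and CloseWidget toggle the same widget and input mode, with closing gated by CanClose and hiding delayed.
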(event `InitializeCamera`
  (bind _returnvalue (`GameplayStatics.GetPlayerController` 0))
  (`PlayerController.SetViewTargetWithBlend` (`GameplayStatics.GetPlayerController` 0) self 0.0 "VTBlend_Linear" 0.0 true)
  (`/Game/Blueprint/Player/BP_PlayerRock.SetCurrentCameraUsed` (`/Game/Blueprint/IMPORTED/BFL_Rock.GetPlayerActorRef`) (`self.Camera`))
  (bind _returnvalue_2 (`|CreateWidget` "/Game/ART_Imported/UI/WBP/WBP_MainMenu.WBP_MainMenu_C"))
  (`UserWidget.AddToViewport` _returnvalue_2 0)
  (bind _output_get (set `self.WBP_MenuRef` _returnvalue_2))
  (`WidgetBlueprintLibrary.SetInputMode_GameAndUIEx` _returnvalue _output_get)
  (set `PlayerController.bShowMouseCursor` true _returnvalue))

(event `Play`
  (bind _returnvalue (`GameplayStatics.GetPlayerController` 0))
  (bind _asbp_player_rock (`/Game/Blueprint/IMPORTED/BFL_Rock.GetPlayerActorRef`))
  (`/Game/ART_Imported/UI/WBP/WBP_MainMenu.Close` (`self.WBP_MenuRef`))
  (`WidgetBlueprintLibrary.SetInputMode_GameOnly` _returnvalue)
  (set `PlayerController.bShowMouseCursor` false _returnvalue)
  (`PlayerController.SetViewTargetWithBlend` (`GameplayStatics.GetPlayerController` 0) _asbp_player_rock 1.0 "VTBlend_Linear" 0.0 true)
  (`/Game/Blueprint/Player/BP_PlayerRock.SetCurrentCameraUsed` _asbp_player_rock (`/Game/Blueprint/Player/BP_PlayerRock.ThirdPersonCamera` _asbp_player_rock))
  (`KismetSystemLibrary.Delay` 1.0)
  (`/Game/Blueprint/Player/BP_PlayerRock.InitializePlayer` (`/Game/Blueprint/IMPORTED/BFL_Rock.GetPlayerActorRef`))
  (`Widget.SetVisibility` (`self.WBP_MenuRef`) "Collapsed"))

(event `OpenWidget`
  (bind _returnvalue (`GameplayStatics.GetPlayerController` 0))
  (bind _wbp_menuref (`self.WBP_MenuRef`))
  (`WidgetBlueprintLibrary.SetInputMode_GameAndUIEx` _returnvalue (`self.WBP_MenuRef`))
  (set `PlayerController.bShowMouseCursor` true _returnvalue)
  (`Widget.SetVisibility` _wbp_menuref "Visible")
  (`/Game/ART_Imported/UI/WBP/WBP_MainMenu.Open` _wbp_menuref))

(event `CloseWidget`
  (bind _returnvalue (`GameplayStatics.GetPlayerController` 0))
  (bind _wbp_menuref (`self.WBP_MenuRef`))
  (if (`/Game/ART_Imported/UI/WBP/WBP_MainMenu.CanClose` _wbp_menuref)
    (`KismetSystemLibrary.PrintString` "Hello")
    (`/Game/ART_Imported/UI/WBP/WBP_MainMenu.Close` _wbp_menuref)
    (`WidgetBlueprintLibrary.SetInputMode_GameOnly` _returnvalue)
    (set `PlayerController.bShowMouseCursor` false _returnvalue)
    (`KismetSystemLibrary.Delay` 0.5)
    (`Widget.SetVisibility` (`self.WBP_MenuRef`) "Collapsed")))

(fn `UserConstructionScript`)