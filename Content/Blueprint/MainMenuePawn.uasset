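; MainMenuePawn is a pawn Blueprint that brings up the main menu through its STARTM event.
; The event creates the WBP_MainMenue widget once, adds it to the viewport, and switches player 0 to UI-only input with a visible cursor.
; It then hands the widget references to itself and to PlayerREF.
; Possessed and Tick are empty, and two CS_MainMen camera shake calls are left unconnected.
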(event `self.ReceivePossessed`
  (params (NewController :type "Controller Object Reference")))

(event `STARTM`
  (bind _returnvalue (`GameplayStatics.GetPlayerController` 0))
  (`|ExecutionSequence`
    (:`then_0`
      (`/Engine/EditorBlueprintResources/StandardMacros.DoOnce` false
        (:`Completed`
          (bind _returnvalue_2 (`|CreateWidget` "/Game/UI/WBP/WBP_MainMenue.WBP_MainMenue_C"))
          (`UserWidget.AddToViewport` _returnvalue_2 0))))
    (:`then_1`
      (`/Engine/EditorBlueprintResources/StandardMacros.IsValid` _returnvalue
        (:`Is Valid`
          (`WidgetBlueprintLibrary.SetInputMode_UIOnlyEx` _returnvalue null)
          (set `PlayerController.bShowMouseCursor` true _returnvalue))))
    (:`then_2`
      (set `/Game/UI/WBP/WBP_MainMenue.MainMenuBPREF` self _returnvalue_2)
      (set `/Game/UI/WBP/WBP_MainMenue.PlayerREF` (`self.PlayerREF`) _returnvalue_2))))

(event `self.ReceiveTick`
  (params (DeltaSeconds :type "Float (single-precision)")))

(fn `UserConstructionScript`)