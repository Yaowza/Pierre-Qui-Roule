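; Sound manager Blueprint that holds the ambient and music audio components and crossfades between music tracks.
; BeginPlay sets ambient volume to full and registers the hub music as the current track.
; ChangeMusic starts the new track and runs a looping UpdateMusic timer for four seconds, then makes that track current.
; UpdateMusic uses FInterpTo on volume multipliers to fade the current track out and the new one in.
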(event `self.ReceiveBeginPlay`
  (`AudioComponent.SetVolumeMultiplier` (`self.SC_Ambiant`) 1.0)
  (set `self.CurrentMusicPlayed` (`self.SC_HubMusic`)))

(event `ChangeMusic`
  (params (NewMusic :type "AudioComponent Object Reference"))
  (bind _output_get (set `self.NewMusic` NewMusic))
  (`AudioComponent.Play` _output_get 0.0)
  (bind _returnvalue (`KismetSystemLibrary.K2_SetTimer` null "UpdateMusic" 0.01 true true))
  (`KismetSystemLibrary.Delay` 4.0)
  (`KismetSystemLibrary.K2_ClearAndInvalidateTimerHandle` _returnvalue)
  (set `self.CurrentMusicPlayed` (`self.NewMusic`)))

(fn `UpdateMusic`
  (locals (CurrentMusicVolume :type "Float (single-precision)" :default 0.0))
  (bind _currentmusicplayed (`self.CurrentMusicPlayed`))
  (bind _newmusic (`self.NewMusic`))
  (`/Engine/EditorBlueprintResources/StandardMacros.IsValid` _currentmusicplayed
    (:`Is Valid`
      (`AudioComponent.SetVolumeMultiplier` _currentmusicplayed (`KismetMathLibrary.FInterpTo` (`AudioComponent.VolumeMultiplier` _currentmusicplayed) 0.0 (`GameplayStatics.GetWorldDeltaSeconds`) 3.0)))
    (:`Is Not Valid`
      _))
  (`/Engine/EditorBlueprintResources/StandardMacros.IsValid` _newmusic
    (:`Is Valid`
      (`AudioComponent.SetVolumeMultiplier` _newmusic (`KismetMathLibrary.FInterpTo` (`AudioComponent.VolumeMultiplier` _newmusic) 1.0 (`GameplayStatics.GetWorldDeltaSeconds`) 3.0)))
    (:`Is Not Valid`
      (`KismetSystemLibrary.PrintString` "ERROR : NEW MUSIC INVALID" true true (struct :`R` 1.0 :`A` 1.0) 10.0))))

(fn `UserConstructionScript`)