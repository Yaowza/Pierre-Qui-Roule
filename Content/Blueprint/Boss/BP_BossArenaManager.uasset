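; Boss arena manager that reshapes the level around the rock player and the boss fight.
; Left and right trigger boxes swap each side's mesh visibility, collision and FX overlaps, while paired gates track the side that CloseEntrance blocks.
; PlayerStop destroys the bridge, and BreakGround removes floor meshes and kill-zone actors.
; CallFX grows a timeline-scaled sphere from the boss, sending ActivateRockMessage to whatever it overlaps.
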(event `self.BoxR.OnComponentBeginOverlap`
  (params (OverlappedComponent :type "PrimitiveComponent Object Reference") (OtherActor :type "Actor Object Reference") (OtherComp :type "PrimitiveComponent Object Reference") (OtherBodyIndex :type Integer) (bFromSweep :type Boolean) (SweepResult :type "HitResult Structure (by ref)"))
  (cast `/Game/Blueprint/Player/BP_PlayerRock` OtherActor)
  (`|ExecutionSequence`
    (:`then_0`
      (for _array_element (`self.MeshesLeft`)
        (`self.F_HideMeshes` _array_element)))
    (:`then_1`
      (for _array_element_2 (`self.MeshesRight`)
        (`self.F_ShowMeshes` _array_element_2)))
    (:`then_2`
      (for _array_element_3 (`self.FXS_R`)
        (set `PrimitiveComponent.bGenerateOverlapEvents` true (`/Game/Blueprint/Boss/RockFallFX.Sphere` _array_element_3))))
    (:`then_3`
      (for _array_element_4 (`self.FXS_L`)
        (set `PrimitiveComponent.bGenerateOverlapEvents` false (`/Game/Blueprint/Boss/RockFallFX.Sphere` _array_element_4))))
    (:`then_4`
      (`/Engine/EditorBlueprintResources/StandardMacros.Gate` false :!label _label
        (:`Exit`
          (`|ExecutionSequence`
            (:`then_0`
              (set `self.BlockSideName` "R"))
            (:`then_1`
              (goto _label_2 :!via `Open`))
            (:`then_2`
              (goto _label :!via `Close`))))))))

(event `self.ReceiveBeginPlay`
  (`|ExecutionSequence`
    (:`then_0`
      (for _array_element (`self.MeshesLeft_Block`)
        (`self.F_HideMeshes` _array_element)))
    (:`then_1`
      (for _array_element_2 (`self.MeshesRight_Block`)
        (`self.F_HideMeshes` _array_element_2)))))

(event `self.PlayerStop.OnComponentBeginOverlap`
  (params (OverlappedComponent :type "PrimitiveComponent Object Reference") (OtherActor :type "Actor Object Reference") (OtherComp :type "PrimitiveComponent Object Reference") (OtherBodyIndex :type Integer) (bFromSweep :type Boolean) (SweepResult :type "HitResult Structure (by ref)"))
  (bind _asbp_player_rock (cast `/Game/Blueprint/Player/BP_PlayerRock` OtherActor))
  (for _array_element (`self.BridgeDestroymesh`)
    (`/Engine/EditorBlueprintResources/StandardMacros.IsValid` _array_element
      (:`Is Valid`
        (`self.K2_DestroyActor` _array_element))))
  (`ActorComponent.K2_DestroyComponent` (`self.PlayerStop`)))

(event `self.BoxL.OnComponentBeginOverlap`
  (params (OverlappedComponent :type "PrimitiveComponent Object Reference") (OtherActor :type "Actor Object Reference") (OtherComp :type "PrimitiveComponent Object Reference") (OtherBodyIndex :type Integer) (bFromSweep :type Boolean) (SweepResult :type "HitResult Structure (by ref)"))
  (cast `/Game/Blueprint/Player/BP_PlayerRock` OtherActor)
  (`|ExecutionSequence`
    (:`then_0`
      (for _array_element (`self.MeshesRight`)
        (`self.F_HideMeshes` _array_element)))
    (:`then_1`
      (for _array_element_2 (`self.MeshesLeft`)
        (`self.F_ShowMeshes` _array_element_2)))
    (:`then_2`
      (for _array_element_3 (`self.FXS_R`)
        (set `PrimitiveComponent.bGenerateOverlapEvents` false (`/Game/Blueprint/Boss/RockFallFX.Sphere` _array_element_3))))
    (:`then_3`
      (for _array_element_4 (`self.FXS_L`)
        (set `PrimitiveComponent.bGenerateOverlapEvents` true (`/Game/Blueprint/Boss/RockFallFX.Sphere` _array_element_4))))
    (:`then_4`
      (`/Engine/EditorBlueprintResources/StandardMacros.Gate` false :!label _label_2
        (:`Exit`
          (`|ExecutionSequence`
            (:`then_0`
              (set `self.BlockSideName` "L"))
            (:`then_1`
              (goto _label :!via `Open`))
            (:`then_2`
              (goto _label_2 :!via `Close`))))))))

(event `MoveTowardEnd`
  (bind _movingcomponent (`/Game/Blueprint/Player/BP_PlayerRock.GetMovingComponent` (`/Game/Blueprint/BFL_Rock.GetPlayerActorRef`)))
  (`PrimitiveComponent.AddForce` _movingcomponent (* (`KismetMathLibrary.GetDirectionUnitVector` (`SceneComponent.K2_GetComponentLocation` _movingcomponent) (`SceneComponent.K2_GetComponentLocation` (`self.Player go to loc`))) 500000.0) "None" false))

(event `Close Entrance`
  (`KismetSystemLibrary.PrintString` "Close" true false)
  (switch `name` (`self.BlockSideName`)
    (:`L`
      (for _array_element (`self.MeshesLeft_Block`)
        (`self.F_ShowMeshes` _array_element)))
    (:`R`
      (for _array_element_2 (`self.MeshesRight_Block`)
        (`self.F_ShowMeshes` _array_element_2)))))

(event `BreakGround`
  (for _array_element (`self.GroundDestroyedMeshes`)
    (`self.K2_DestroyActor` _array_element))
  (for _array_element_2 (`self.KillZonesToActivate`)
    (`self.K2_DestroyActor` _array_element_2)))

(event `CallFX`
  (bind _outactors (`GameplayStatics.GetAllActorsWithTag` "BossBoss"))
  (bind _asbp_iarock_boss (cast `/Game/Blueprint/IA/CustomIA/BP_IARockBoss` (`|GetArrayItem` _outactors)))
  (`SceneComponent.K2_SetWorldLocation` (`self.FXTriggerer`) (`self.K2_GetActorLocation` _asbp_iarock_boss) false false)
  (bind (_direction _newtrack_0) (`Timeline|ScaleSphere` :!via `PlayFromStart`)
    (:`Update`
      (`SceneComponent.SetWorldScale3D` (`self.FXTriggerer`) (`KismetMathLibrary.Conv_DoubleToVector` (* (* _newtrack_0 170.0) 1.6))))))

(event `self.FXTriggerer.OnComponentBeginOverlap`
  (params (OverlappedComponent :type "PrimitiveComponent Object Reference") (OtherActor :type "Actor Object Reference") (OtherComp :type "PrimitiveComponent Object Reference") (OtherBodyIndex :type Integer) (bFromSweep :type Boolean) (SweepResult :type "HitResult Structure (by ref)"))
  (message `/Game/Blueprint/Interface/BPI_Boss.ActivateRock` OtherActor))

(fn `F_HideMeshes`
  (params (Mesh :type "StaticMeshActor Object Reference"))
  (bind _rootcomponent (`Actor.RootComponent` Mesh))
  (`/Engine/EditorBlueprintResources/StandardMacros.IsValid` _rootcomponent
    (:`Is Valid`
      (`SceneComponent.SetVisibility` _rootcomponent false false)
      (`self.SetActorEnableCollision` Mesh false))))

(fn `F_ShowMeshes`
  (params (Mesh :type "StaticMeshActor Object Reference"))
  (bind _rootcomponent (`Actor.RootComponent` Mesh))
  (`/Engine/EditorBlueprintResources/StandardMacros.IsValid` _rootcomponent
    (:`Is Valid`
      (`SceneComponent.SetVisibility` _rootcomponent true false))
    (:`Is Not Valid`
      _))
  (`self.SetActorEnableCollision` Mesh true))

(fn `UserConstructionScript`)