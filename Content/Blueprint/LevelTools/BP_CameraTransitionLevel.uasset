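; BP_CameraTransitionLevel is a camera actor that takes over and releases the player's view, likely for level transitions.
; Shortly after BeginPlay it snaps onto the physics player while keeping world rotation.
; UseCamera blends the view to itself, registers it as the current camera, and starts a fast looping timer that replays a moving shake and enforces TargetRot.
; StopCamera blends back to the third-person camera and clears the timer.
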(event `self.ReceiveBeginPlay`
  (`KismetSystemLibrary.Delay` 0.2)
  (`self.K2_AttachToComponent` (`/Game/Blueprint/BFL_Rock.GetPhysicPlayerRef`) "None" "SnapToTarget" "KeepWorld" "KeepRelative"))

(event `UseCamera`
  (`PlayerController.SetViewTargetWithBlend` (`GameplayStatics.GetPlayerController` 0) self 0.75 "VTBlend_Linear" 0.0 true)
  (bind _returnvalue (`KismetSystemLibrary.K2_SetTimerDelegate` (delegate `CameraShake`) 0.01 true true))
  (`/Game/Blueprint/Player/BP_PlayerRock.SetCurrentCameraUsed` (`/Game/Blueprint/BFL_Rock.GetPlayerActorRef`) (`self.Camera`)))

(event `StopCameraShake`
  (`KismetSystemLibrary.K2_ClearAndInvalidateTimerHandle` (stale `UseCamera` _returnvalue))
  (`KismetSystemLibrary.PrintString` "Hello"))

(event `CameraShake`
  (`LegacyCameraShake.StartLegacyCameraShake` (`GameplayStatics.GetPlayerCameraManager` 0) "/Game/Blueprint/Player/CameraShakePlayer/CS_Moving.CS_Moving_C" 1.5)
  (`self.K2_SetActorRotation` (`self.TargetRot`)))

(event `StopCamera`
  (bind _asbp_player_rock (`/Game/Blueprint/BFL_Rock.GetPlayerActorRef`))
  (`PlayerController.SetViewTargetWithBlend` (`GameplayStatics.GetPlayerController` 0) (`/Game/Blueprint/BFL_Rock.GetPlayerActorRef`) 1.0 "VTBlend_Linear" 0.0 true)
  (`self.StopCameraShake`)
  (`/Game/Blueprint/Player/BP_PlayerRock.SetCurrentCameraUsed` _asbp_player_rock (`/Game/Blueprint/Player/BP_PlayerRock.ThirdPersonCamera` _asbp_player_rock)))

(fn `UserConstructionScript`)