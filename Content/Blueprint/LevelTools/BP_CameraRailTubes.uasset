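; Level camera rail that blends the view from BP_PlayerRock's third-person camera to its own spline-following camera.
; Start triggers toggle the rail view, leaving StartBox re-enables it, and end triggers return to the player.
; While active, Tick eases the camera toward the spline point nearest CamRailTarget, aims it at the physics player and resets cannon camera rotation.
; ResetCameraSnap restores the player view and the camera's initial transform; trigger-to-spline placement code is unconnected.
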(event `self.StartBox.OnComponentEndOverlap`
  (params (OverlappedComponent :type "PrimitiveComponent Object Reference") (OtherActor :type "Actor Object Reference") (OtherComp :type "PrimitiveComponent Object Reference") (OtherBodyIndex :type Integer))
  (cast `/Game/Blueprint/Player/BP_PlayerRock` OtherActor)
  (if (not (`self.cam`))
    (`PlayerController.SetViewTargetWithBlend` (`GameplayStatics.GetPlayerController` 0) self 1.0 "VTBlend_Linear" 0.0 true :!label _label)
    (set `self.cam` true)
    (`/Game/Blueprint/Player/BP_PlayerRock.SetCurrentCameraUsed` (`/Game/Blueprint/BFL_Rock.GetPlayerActorRef`) (`self.Camera`))))

(event `self.StartBox.OnComponentBeginOverlap`
  (params (OverlappedComponent :type "PrimitiveComponent Object Reference") (OtherActor :type "Actor Object Reference") (OtherComp :type "PrimitiveComponent Object Reference") (OtherBodyIndex :type Integer) (bFromSweep :type Boolean) (SweepResult :type "HitResult Structure (by ref)"))
  (bind _asbp_player_rock (`/Game/Blueprint/BFL_Rock.GetPlayerActorRef`))
  (bind _asbp_player_rock_2 (`/Game/Blueprint/BFL_Rock.GetPlayerActorRef`))
  (cast `/Game/Blueprint/Player/BP_PlayerRock` OtherActor)
  (if (`self.cam`) :!label _label_2
    (`PlayerController.SetViewTargetWithBlend` (`GameplayStatics.GetPlayerController` 0) _asbp_player_rock 1.0 "VTBlend_Linear" 0.0 true :!label _label_3)
    (set `self.cam` false)
    (`/Game/Blueprint/Player/BP_PlayerRock.ResetCameraRotation_Canon` _asbp_player_rock)
    (`/Game/Blueprint/Player/BP_PlayerRock.SetCurrentCameraUsed` _asbp_player_rock_2 (`/Game/Blueprint/Player/BP_PlayerRock.ThirdPersonCamera` _asbp_player_rock_2))
    (else
      (goto _label))))

(event `self.StartTrigerBox.OnComponentBeginOverlap`
  (params (OverlappedComponent :type "PrimitiveComponent Object Reference") (OtherActor :type "Actor Object Reference") (OtherComp :type "PrimitiveComponent Object Reference") (OtherBodyIndex :type Integer) (bFromSweep :type Boolean) (SweepResult :type "HitResult Structure (by ref)"))
  (cast `/Game/Blueprint/Player/BP_PlayerRock` OtherActor)
  (goto _label_2))

(event `self.EndTrigerBox.OnComponentBeginOverlap`
  (params (OverlappedComponent :type "PrimitiveComponent Object Reference") (OtherActor :type "Actor Object Reference") (OtherComp :type "PrimitiveComponent Object Reference") (OtherBodyIndex :type Integer) (bFromSweep :type Boolean) (SweepResult :type "HitResult Structure (by ref)"))
  (cast `/Game/Blueprint/Player/BP_PlayerRock` OtherActor)
  (if (`self.cam`) :!label _label_4
    (goto _label_3)))

(event `self.EndBox.OnComponentBeginOverlap`
  (params (OverlappedComponent :type "PrimitiveComponent Object Reference") (OtherActor :type "Actor Object Reference") (OtherComp :type "PrimitiveComponent Object Reference") (OtherBodyIndex :type Integer) (bFromSweep :type Boolean) (SweepResult :type "HitResult Structure (by ref)"))
  (cast `/Game/Blueprint/Player/BP_PlayerRock` OtherActor)
  (goto _label_4))

(event `self.ReceiveBeginPlay`
  (bind _camera (`self.Camera`))
  (set `self.BaseLoc` (`SceneComponent.K2_GetComponentLocation` _camera))
  (set `self.BaseRot` (`SceneComponent.K2_GetComponentRotation` _camera)))

(event `self.ReceiveTick`
  (params (DeltaSeconds :type "Float (single-precision)"))
  (if (`self.cam`)
    (`|ExecutionSequence`
      (:`then_0`
        (`SceneComponent.K2_SetWorldLocationAndRotation` (`self.Camera`) (`KismetMathLibrary.VInterpTo` (`SceneComponent.K2_GetComponentLocation` (`self.Camera`)) (`SplineComponent.FindLocationClosestToWorldLocation` (`self.Spline`) (`SceneComponent.K2_GetComponentLocation` (`/Game/Blueprint/Player/BP_PlayerRock.CamRailTarget` (`/Game/Blueprint/BFL_Rock.GetPlayerActorRef`))) "World") (`GameplayStatics.GetWorldDeltaSeconds`) 5.0) (`KismetMathLibrary.FindLookAtRotation` (`SceneComponent.K2_GetComponentLocation` (`self.Camera`)) (`SceneComponent.K2_GetComponentLocation` (`/Game/Blueprint/BFL_Rock.GetPhysicPlayerRef`))) false false)
        (`/Game/Blueprint/Player/BP_PlayerRock.ResetCameraRotation_Canon` (`/Game/Blueprint/BFL_Rock.GetPlayerActorRef`))))))

(event `ResetCameraSnap`
  (bind _asbp_player_rock (`/Game/Blueprint/BFL_Rock.GetPlayerActorRef`))
  (bind _asbp_player_rock_2 (`/Game/Blueprint/BFL_Rock.GetPlayerActorRef`))
  (`PlayerController.SetViewTargetWithBlend` (`GameplayStatics.GetPlayerController` 0) _asbp_player_rock_2 1.0 "VTBlend_Linear" 0.0 true)
  (set `self.cam` false)
  (`/Game/Blueprint/Player/BP_PlayerRock.ResetCameraRotation_Canon` _asbp_player_rock_2)
  (`SceneComponent.K2_SetWorldLocationAndRotation` (`self.Camera`) (`self.BaseLoc`) (`self.BaseRot`) false false)
  (`/Game/Blueprint/Player/BP_PlayerRock.SetCurrentCameraUsed` _asbp_player_rock (`/Game/Blueprint/Player/BP_PlayerRock.ThirdPersonCamera` _asbp_player_rock)))

(fn `UserConstructionScript`)