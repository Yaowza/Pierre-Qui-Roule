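; Level-tool cannon that captures the player rock on trigger overlap and launches it with an impulse and boost.
; When no BOSS is set, capture locks the player, pins it to RockSocket with a looping timer and blends to the cannon camera, optionally sliding along a spline.
; Firing is automatic or on interact, optionally restoring control and camera afterwards.
; Timelines drive the lid and optional barrel swing; construction selects mesh and lid visibility.
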(event `CloseClappet`
  (`TimelineComponent.SetPlayRate` (`self.Clappet`) (/ 1.0 0.5))
  (bind (_direction _newtrack_0) (`Timeline|Clappet` :!via `PlayFromStart` :!label _label)
    (:`Update`
      (`SceneComponent.K2_SetRelativeRotation` (`self.CanonLid`) (`KismetMathLibrary.MakeRotator` (`KismetMathLibrary.Lerp` 140.0 0.0 _newtrack_0)) false false))))

(event `OpentClappet`
  (`TimelineComponent.SetPlayRate` (`self.Clappet`) (/ 1.0 0.5))
  (goto _label :!via `Reverse`))

(event `RotateCanon`
  (bind _returnvalue (* (/ (`self.SwingAngle`) 2.0) -1.0))
  (`/Engine/EditorBlueprintResources/StandardMacros.FlipFlop`
    (:`A`
      (set `self.SwingRight?` false))
    (:`B`
      (set `self.SwingRight?` true)))
  (`TimelineComponent.SetPlayRate` (`self.SwingTimling`) (/ 1.0 (`self.SwingSpeed`)))
  (`SceneComponent.K2_SetRelativeRotation` (`self.CanonSocket`) (`KismetMathLibrary.MakeRotator` 0.0 _returnvalue) false false)
  (set `self.Relative Rotation Y (Pitch)` _returnvalue)
  (set `self.RL` true :!label _label_2)
  (bind (_direction _newtrack_0) (`Timeline|SwingTimling` :!via `PlayFromStart` :!label _label_3)
    (:`Update`
      (`SceneComponent.K2_SetRelativeRotation` (`self.CanonSocket`) (`KismetMathLibrary.MakeRotator` 0.0 (`KismetMathLibrary.Lerp` (`self.Relative Rotation Y (Pitch)`) (/ (`self.SwingAngle`) 2.0) _newtrack_0)) false false))
    (:`Finished`
      (`KismetSystemLibrary.Delay` (`self.DelayBeforeNextSwing`))
      (if (`self.RL`)
        (set `self.RL` false)
        (goto _label_3 :!via `Reverse`)
        (else
          (goto _label_2))))))

(event `self.ReceiveBeginPlay`
  (bind _swingangle (`self.SwingAngle`))
  (bind (_relativerotation_roll _relativerotation_pitch _relativerotation_yaw) (`KismetMathLibrary.BreakRotator` (`SceneComponent.RelativeRotation` (`self.CanonSocket`))))
  (if (`self.Swing?`)
    (set `self.StartXRot` _relativerotation_roll)
    (set `self.StartZRot` _relativerotation_yaw)
    (set `self.RightTarget` (+ _relativerotation_pitch _swingangle))
    (set `self.LeftTarget` (- _relativerotation_pitch _swingangle))
    (`SceneComponent.K2_SetRelativeRotation` (`self.CanonSocket`) (`KismetMathLibrary.MakeRotator` (`self.StartXRot`) (`self.RightTarget`) (`self.StartZRot`)) false false)
    (`self.RotateCanon`)))

(event `self.TrigerBox.OnComponentBeginOverlap`
  (params (OverlappedComponent :type "PrimitiveComponent Object Reference") (OtherActor :type "Actor Object Reference") (OtherComp :type "PrimitiveComponent Object Reference") (OtherBodyIndex :type Integer) (bFromSweep :type Boolean) (SweepResult :type "HitResult Structure (by ref)"))
  (bind _boss (`self.BOSS`))
  (bind _spline (`self.Spline`))
  (bind _camera (`self.Camera`))
  (bind (_returnvalue_roll _returnvalue_pitch _returnvalue_yaw) (`KismetMathLibrary.BreakRotator` (`KismetMathLibrary.FindLookAtRotation` (`SceneComponent.K2_GetComponentLocation` (`self.Camera`)) (`SceneComponent.K2_GetComponentLocation` (`self.ShootSocket`)))))
  (bind _asbp_player_rock (cast `/Game/Blueprint/Player/BP_PlayerRock` OtherActor))
  (`/Engine/EditorBlueprintResources/StandardMacros.DoOnce` false :!label _label_4
    (:`Completed`
      (set `self.cam` true)
      (`GameplayStatics.PlaySound2D` "/Game/Audio/Sounds/SFX/Canon/SC_CanonEnter.SC_CanonEnter" 1.0 1.0 0.0 null null)
      (`/Engine/EditorBlueprintResources/StandardMacros.IsValid` _boss
        (:`Is Valid`
          (`/Game/Blueprint/IA/BP_IARock.Ignoreplayer` _boss true))
        (:`Is Not Valid`
          (`/Game/Blueprint/Player/BP_PlayerRock.Cancel Down Dash` _asbp_player_rock)
          (`PrimitiveComponent.SetCollisionResponseToChannel` (`self.Sphere`) "ECC_GameTraceChannel2" "ECR_Block")
          (`/Game/Blueprint/Player/BP_PlayerRock.LockPlayer` (`/Game/Blueprint/BFL_Rock.GetPlayerActorRef`))
          (`PlayerController.SetViewTargetWithBlend` (`GameplayStatics.GetPlayerController` 0) self (`self.BlendSpeed`) "VTBlend_Linear" 0.0 true)
          (`/Game/Blueprint/Player/BP_PlayerRock.SetCurrentCameraUsed` (`/Game/Blueprint/BFL_Rock.GetPlayerActorRef`) (`self.Camera`))
          (`|ExecutionSequence`
            (:`then_0`
              (bind _returnvalue (`KismetSystemLibrary.K2_SetTimerDelegate` (delegate `SnapPlayer`) 0.01 true true))
              (if (`self.SnapCam ?`)
                _
                (elif (`self.AutoShoot?`)
                  (`KismetSystemLibrary.Delay` 1.0)
                  (`self.Shoot`))))
            (:`then_1`
              (`KismetSystemLibrary.Delay` 0.2)
              (if (`self.SnapCam ?`)
                (`TimelineComponent.SetPlayRate` (`self.SlideCAM`) (/ 1.0 (`self.SlideCamSpeed`)))
                (bind (_direction _newtrack_0) (`Timeline|SlideCAM` :!via `PlayFromStart`)
                  (:`Update`
                    (bind _returnvalue_location (`KismetMathLibrary.BreakTransform` (`SplineComponent.GetTransformAtDistanceAlongSpline` _spline (`KismetMathLibrary.Lerp` 0.0 (`SplineComponent.GetSplineLength` _spline) _newtrack_0) "Local" false)))
                    (`SceneComponent.K2_SetRelativeTransform` _camera (`KismetMathLibrary.MakeTransform` _returnvalue_location) false false)
                    (`SceneComponent.K2_SetWorldRotation` _camera (`SplineComponent.GetRotationAtTime` _spline _newtrack_0 "World" false) false false))
                  (:`Finished`
                    (`SceneComponent.K2_SetWorldRotation` _camera (`KismetMathLibrary.MakeRotator` _returnvalue_roll _returnvalue_pitch _returnvalue_yaw) false false)
                    (if (`self.AutoShoot?`)
                      (`KismetSystemLibrary.Delay` (`self.ShootDelay`))
                      (`self.Shoot`))))))
            (:`then_3`
              (`KismetSystemLibrary.Delay` (`self.ClappetDelay`))
              (`self.CloseClappet`))))))))

(event `ClearSnapPlayer`
  (`KismetSystemLibrary.K2_ClearAndInvalidateTimerHandle` (stale `self.TrigerBox.OnComponentBeginOverlap` _returnvalue)))

(event `SnapPlayer`
  (bind _rocksocket (`self.RockSocket`))
  (`SceneComponent.K2_SetWorldLocationAndRotation` (`/Game/Blueprint/BFL_Rock.GetPhysicPlayerRef`) (`SceneComponent.K2_GetComponentLocation` _rocksocket) (`SceneComponent.K2_GetComponentRotation` _rocksocket) false false)
  (if (and (`/Game/Blueprint/Player/BP_PlayerRock.GetInteracted?` (`/Game/Blueprint/BFL_Rock.GetPlayerActorRef`)) (not (`self.AutoShoot?`)))
    (`self.Shoot`)))

(event `self.TrigerBox.OnComponentEndOverlap`
  (params (OverlappedComponent :type "PrimitiveComponent Object Reference") (OtherActor :type "Actor Object Reference") (OtherComp :type "PrimitiveComponent Object Reference") (OtherBodyIndex :type Integer))
  (cast `/Game/Blueprint/Player/BP_PlayerRock` OtherActor)
  (goto _label_4 :!via `Reset`))

(event `Shoot`
  (bind _asbp_player_rock (`/Game/Blueprint/BFL_Rock.GetPlayerActorRef`))
  (bind _asbp_player_rock_2 (`/Game/Blueprint/BFL_Rock.GetPlayerActorRef`))
  (bind _asbp_player_rock_3 (`/Game/Blueprint/BFL_Rock.GetPlayerActorRef`))
  (bind _shootsocket (`self.ShootSocket`))
  (bind _boss (`self.BOSS`))
  (`/Game/Blueprint/Player/BP_PlayerRock.ResetCameraRotation_CamLock` (`/Game/Blueprint/BFL_Rock.GetPlayerActorRef`))
  (`GameplayStatics.PlaySound2D` "/Game/Audio/Sounds/SFX/Canon/SC_CanonShoot.SC_CanonShoot" 1.0 1.0 0.0 null null)
  (`/Engine/EditorBlueprintResources/StandardMacros.IsValid` _boss
    (:`Is Valid`
      (`/Game/Blueprint/IA/BP_IARock.Ignoreplayer` _boss false))
    (:`Is Not Valid`
      _))
  (`self.ClearSnapPlayer`)
  (`SceneComponent.K2_SetWorldLocationAndRotation` (`/Game/Blueprint/BFL_Rock.GetPhysicPlayerRef`) (`SceneComponent.K2_GetComponentLocation` _shootsocket) (`SceneComponent.K2_GetComponentRotation` _shootsocket) false false)
  (`/Game/Blueprint/Player/BP_PlayerRock.UnlockPlayer` _asbp_player_rock)
  (`self.DisableInput` _asbp_player_rock (`GameplayStatics.GetPlayerController` 0))
  (`PrimitiveComponent.AddImpulse` (`/Game/Blueprint/BFL_Rock.GetPhysicPlayerRef`) (* (`SceneComponent.GetForwardVector` (`self.RockSocket`)) 5000000.0) "None" false)
  (`ActorComponent.Activate` (`self.NS_Jump2`) true)
  (`/Game/Blueprint/Player/BP_PlayerRock.StartBoost` (`/Game/Blueprint/BFL_Rock.GetPlayerActorRef`) (`self.Boost`))
  (`KismetSystemLibrary.Delay` 0.25)
  (if (`self.ShouldFree`)
    (if (`self.cam`)
      (`self.EnableInput` (`/Game/Blueprint/BFL_Rock.GetPlayerActorRef`) (`GameplayStatics.GetPlayerController` 0))
      (`PlayerController.SetViewTargetWithBlend` (`GameplayStatics.GetPlayerController` 0) _asbp_player_rock_3 0.0 "VTBlend_Linear" 0.0 false)
      (set `self.cam` false)
      (`/Game/Blueprint/Player/BP_PlayerRock.SetCurrentCameraUsed` _asbp_player_rock_2 (`/Game/Blueprint/Player/BP_PlayerRock.ThirdPersonCamera` _asbp_player_rock_2))
      (`SceneComponent.K2_SetWorldRotation` (`/Game/Blueprint/Player/BP_PlayerRock.GetMovingComponent` _asbp_player_rock_2) (`SceneComponent.K2_GetComponentRotation` (`self.Sphere1`)) false false)
      (`/Game/Blueprint/Player/BP_PlayerRock.ResetCameraRotation_CamLock` _asbp_player_rock_3))
    (else
      (`KismetSystemLibrary.Delay` 0.5)
      (`self.OpentClappet`))))

(event `Cameraaaaaaaa`
  (`SceneComponent.K2_SetWorldLocationAndRotation` (`self.Camera`) (`KismetMathLibrary.VInterpTo` (`SceneComponent.K2_GetComponentLocation` (`self.Camera`)) (`SplineComponent.FindLocationClosestToWorldLocation` (`self.SplineRail`) (`SceneComponent.K2_GetComponentLocation` (`/Game/Blueprint/Player/BP_PlayerRock.ThirdPersonCamera` (`/Game/Blueprint/BFL_Rock.GetPlayerActorRef`))) "World") (`GameplayStatics.GetWorldDeltaSeconds`) 5.0) (`KismetMathLibrary.FindLookAtRotation` (`SceneComponent.K2_GetComponentLocation` (`self.Camera`)) (`SceneComponent.K2_GetComponentLocation` (`/Game/Blueprint/BFL_Rock.GetPhysicPlayerRef`))) false false))

(fn `SwingCanon`
  (bind _returnvalue (`KismetMathLibrary.SelectFloat` (`self.RightTarget`) (`self.LeftTarget`) (`self.SwingRight?`)))
  (bind (_relativerotation_roll _relativerotation_pitch) (`KismetMathLibrary.BreakRotator` (`SceneComponent.RelativeRotation` (`self.CanonSocket`))))
  (`SceneComponent.K2_SetRelativeRotation` (`self.CanonSocket`) (`KismetMathLibrary.MakeRotator` (`self.StartXRot`) (`KismetMathLibrary.FInterpTo_Constant` _relativerotation_pitch _returnvalue (`GameplayStatics.GetWorldDeltaSeconds`) (`self.SwingSpeed`)) (`self.StartZRot`)) false false)
  (`KismetSystemLibrary.PrintString` (`KismetStringLibrary.Conv_DoubleToString` _returnvalue) true false (struct :`G` 0.66 :`B` 1.0 :`A` 1.0) 0.0))

(fn `UserConstructionScript`
  (`SceneComponent.K2_SetRelativeLocation` (`self.Camera`) (`.Position` (break `SplinePoint` (`SplineComponent.GetSplinePointAt` (`self.Spline`) 0 "Local"))) false false)
  (`SceneComponent.K2_SetWorldRotation` (`self.Camera`) (`SplineComponent.GetRotationAtSplinePoint` (`self.Spline`) 0 "World") false false)
  (`|ExecutionSequence`
    (:`then_0`
      (if (`self.Swing?`)
        (`SceneComponent.SetVisibility` (`self.CanonA`) true false)
        (`SceneComponent.SetVisibility` (`self.CanonB`) false false)
        (else
          (`SceneComponent.SetVisibility` (`self.CanonA`) false false)
          (`SceneComponent.SetVisibility` (`self.CanonB`) true false))))
    (:`then_1`
      (if (`self.WithDoor?`)
        (`SceneComponent.SetVisibility` (`self.CanonLid`) true false)
        (else
          (`SceneComponent.SetVisibility` (`self.CanonLid`) false false))))))