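; BP_CheckPoint is a level-tool checkpoint volume that records a respawn transform for the rolling-rock player.
; When BP_PlayerRock overlaps its box, or TrigerCheckpoint is called, it overwrites LastCheckPointLocation in GI_PierreQuiRouleGameInstance.
; The saved value is a single-entry map pairing the RespawnPivot component's world location with its rotation.
; The construction script sizes the box from an extent variable.
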(event `TrigerCheckpoint`
  (bind _respawnpivot (`self.RespawnPivot`))
  (bind _asgi_pierre_qui_roule_game_instance (cast `/Game/Blueprint/GameInstance/GI_PierreQuiRouleGameInstance` (`GameplayStatics.GetGameInstance`) :!label _label))
  (set `/Game/Blueprint/GameInstance/GI_PierreQuiRouleGameInstance.LastCheckPointLocation` (`|MakeMap` (`SceneComponent.K2_GetComponentLocation` _respawnpivot) (`SceneComponent.K2_GetComponentRotation` _respawnpivot)) _asgi_pierre_qui_roule_game_instance))

(event `self.Box.OnComponentBeginOverlap`
  (params (OverlappedComponent :type "PrimitiveComponent Object Reference") (OtherActor :type "Actor Object Reference") (OtherComp :type "PrimitiveComponent Object Reference") (OtherBodyIndex :type Integer) (bFromSweep :type Boolean) (SweepResult :type "HitResult Structure (by ref)"))
  (bind _asbp_player_rock (cast `/Game/Blueprint/Player/BP_PlayerRock` OtherActor))
  (set `self.PlayerREF` _asbp_player_rock)
  (goto _label))

(fn `UserConstructionScript`
  (`BoxComponent.SetBoxExtent` (`self.Box`) (`self.In Box Extent`) true))