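; BP_CameraRail is a level camera trigger that blends the BP_PlayerRock player's view to a spline-bound rail camera.
; OnlyIN selects Box enter/exit switching, or an In trigger that toggles plus an Out trigger that exits.
; While active, a looping timer eases the camera toward the spline point nearest the physics player, facing the player or keeping its starting rotation.
; The construction script applies trigger size and rail arrow placement.
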(event `self.ReceiveBeginPlay`
  ;[0 1 0.5794] Begin Play
  (set `self.StartRot` (`SceneComponent.K2_GetComponentRotation` (`self.CameraOnRail`))))

(event `self.Box.OnComponentEndOverlap`
  (params (OverlappedComponent :type "PrimitiveComponent Object Reference") (OtherActor :type "Actor Object Reference") (OtherComp :type "PrimitiveComponent Object Reference") (OtherBodyIndex :type Integer))
  (bind _asbp_player_rock (`/Game/Blueprint/BFL_Rock.GetPlayerActorRef`))
  ;[1 0.217 0] End Overlap
  (if (`self.OnlyIN`)
    (bind _asbp_player_rock_2 (cast `/Game/Blueprint/Player/BP_PlayerRock` OtherActor))
    (set `self.PlayerROck` _asbp_player_rock_2)
    (`self.ClearRailUpdate` :!label _label)
    (`PlayerController.SetViewTargetWithBlend` (`GameplayStatics.GetPlayerController` 0) (`self.PlayerROck`) (`self.BlendTimeOut`) "VTBlend_Linear" 0.0 true)
    (`/Game/Blueprint/Player/BP_PlayerRock.SetCurrentCameraUsed` _asbp_player_rock (`/Game/Blueprint/Player/BP_PlayerRock.ThirdPersonCamera` (`/Game/Blueprint/BFL_Rock.GetPlayerActorRef`)))
    (`/Game/Blueprint/Player/BP_PlayerRock.ResetCameraRotationCustomRot` _asbp_player_rock 0.0 -50.0)))

(event `self.Out.OnComponentBeginOverlap`
  (params (OverlappedComponent :type "PrimitiveComponent Object Reference") (OtherActor :type "Actor Object Reference") (OtherComp :type "PrimitiveComponent Object Reference") (OtherBodyIndex :type Integer) (bFromSweep :type Boolean) (SweepResult :type "HitResult Structure (by ref)"))
  ;[1 0.217 0] End Overlap
  (if (not (`self.OnlyIN`))
    (bind _asbp_player_rock (cast `/Game/Blueprint/Player/BP_PlayerRock` OtherActor))
    (set `self.PlayerROck` _asbp_player_rock)
    (goto _label)))

(event `ClearRailUpdate`
  ;[1 0.2165 0.7284] Clear Rail Update
  (`KismetSystemLibrary.K2_ClearAndInvalidateTimerHandle` (stale `self.Box.OnComponentBeginOverlap` _returnvalue)))

(event `self.Box.OnComponentBeginOverlap`
  (params (OverlappedComponent :type "PrimitiveComponent Object Reference") (OtherActor :type "Actor Object Reference") (OtherComp :type "PrimitiveComponent Object Reference") (OtherBodyIndex :type Integer) (bFromSweep :type Boolean) (SweepResult :type "HitResult Structure (by ref)"))
  ;[1 0.217 0] Begin Overlap
  (if (`self.OnlyIN`)
    (cast `/Game/Blueprint/Player/BP_PlayerRock` OtherActor)
    (`PlayerController.SetViewTargetWithBlend` (`GameplayStatics.GetPlayerController` 0) self (`self.BlendTimeIn`) "VTBlend_Linear" 0.0 true :!label _label_2)
    (`/Game/Blueprint/Player/BP_PlayerRock.SetCurrentCameraUsed` (`/Game/Blueprint/BFL_Rock.GetPlayerActorRef`) (`self.CameraOnRail`))
    (bind _returnvalue (`KismetSystemLibrary.K2_SetTimerDelegate` (delegate `FollowPlayerOnRail`) 0.001 true true))))

(event `self.In.OnComponentBeginOverlap`
  (params (OverlappedComponent :type "PrimitiveComponent Object Reference") (OtherActor :type "Actor Object Reference") (OtherComp :type "PrimitiveComponent Object Reference") (OtherBodyIndex :type Integer) (bFromSweep :type Boolean) (SweepResult :type "HitResult Structure (by ref)"))
  ;[1 0.217 0] Begin Overlap
  (if (not (`self.OnlyIN`))
    (bind _asbp_player_rock (cast `/Game/Blueprint/Player/BP_PlayerRock` OtherActor))
    (set `self.PlayerROck` _asbp_player_rock)
    (if (`self.IN!`)
      (set `self.IN!` false)
      (goto _label)
      (else
        (set `self.IN!` true)
        (goto _label_2)))))

(event `FollowPlayerOnRail`
  ;[1 0.2165 0.7284] Follow Player On Rail
  (`SceneComponent.K2_SetWorldLocationAndRotation` (`self.CameraOnRail`) (`KismetMathLibrary.VInterpTo` (`SceneComponent.K2_GetComponentLocation` (`self.CameraOnRail`)) (`SplineComponent.FindLocationClosestToWorldLocation` (`self.Spline`) (`SceneComponent.K2_GetComponentLocation` (`/Game/Blueprint/BFL_Rock.GetPhysicPlayerRef`)) "World") (`GameplayStatics.GetWorldDeltaSeconds`) 5.0) (`KismetMathLibrary.RInterpTo` (`SceneComponent.K2_GetComponentRotation` (`self.CameraOnRail`)) (`KismetMathLibrary.SelectRotator` (`KismetMathLibrary.FindLookAtRotation` (`SceneComponent.K2_GetComponentLocation` (`self.CameraOnRail`)) (`SceneComponent.K2_GetComponentLocation` (`/Game/Blueprint/BFL_Rock.GetPhysicPlayerRef`))) (`self.StartRot`) (`self.LookAtPlayer?`)) (`GameplayStatics.GetWorldDeltaSeconds`) 5.0) false false))

(fn `UserConstructionScript`
  ;[1 1 1] Update Triger box size
  (`BoxComponent.SetBoxExtent` (`self.Box`) (`self.TrigerBoxSize`) false)
  (`ShapeComponent.SetLineThickness` (`self.Box`) (/ (`KismetMathLibrary.VSize` (`self.TrigerBoxSize`)) 24.0))
  ;[1 1 1] Update Rail Loc & Rot
  (`SceneComponent.K2_SetRelativeLocation` (`self.Arrow`) (`self.RailStartLocation`) false false)
  (`SceneComponent.K2_SetWorldRotation` (`self.Arrow`) (`KismetMathLibrary.ComposeRotators` (`self.RailRotation`) (`self.K2_GetActorRotation`)) false false))