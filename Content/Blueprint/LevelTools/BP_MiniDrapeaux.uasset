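; Level-building actor that strings mini flags along a spline on a rope, built entirely in the construction script.
; Flags are instanced into HISMBell, spaced by mesh width with unseeded random jitter, skipping both end indices, each with three random custom data values.
; The rope is a second HISM with one instance per unit of spline length.
; Bell sound and mesh-vertex scattering logic is left unconnected.
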(event `self.Attack`)

(fn `UserConstructionScript`
  (locals (LoopIndex :type Integer))
  (bind _spline (`self.Spline`))
  (bind _spline_2 (`self.Spline`))
  (bind _hism_bell (`self.HISM_Bell`))
  (bind (_returnvalue_min _returnvalue_max) (break `Box` (`StaticMesh.GetBoundingBox` (`self.Drapeaux`))))
  (bind _returnvalue (* (`self.SplineMeshIndex`) 1.0))
  (bind _returnvalue_2 (+ (`self.Instances`) 1))
  (bind _returnvalue_x (`KismetMathLibrary.BreakVector` (- _returnvalue_max _returnvalue_min)))
  (bind _returnvalue_3 (+ (* _returnvalue_x (`local.LoopIndex`)) (`KismetMathLibrary.RandomFloatInRange` -100.0 100.0)))
  (bind (_returnvalue_roll _returnvalue_pitch _returnvalue_yaw) (`KismetMathLibrary.BreakRotator` (`SplineComponent.GetRotationAtDistanceAlongSpline` _spline _returnvalue_3 "World")))
  (`KismetMathLibrary.SetRandomStreamSeed` (`self.Random Stream`) (`self.New Seed`))
  (`InstancedStaticMeshComponent.ClearInstances` (`self.HISM_Bell`))
  (`InstancedStaticMeshComponent.ClearInstances` (`self.HISM_Rope`))
  (bind _returnvalue_4 (`KismetMaterialLibrary.CreateDynamicMaterialInstance` (`StaticMesh.GetMaterial` (`self.Drapeaux`) 0)))
  (`StaticMeshComponent.SetStaticMesh` (`self.HISM_Bell`) (`self.Drapeaux`))
  (`PrimitiveComponent.SetMaterial` (`self.HISM_Bell`) 0 _returnvalue_4)
  (`|ExecutionSequence`
    (:`then_0`
      (for _index (range (+ _returnvalue_2 1))
        (bind _output_get (set `local.LoopIndex` _index))
        (if (not (or (== _output_get 0) (== _output_get _returnvalue_2)))
          (bind _returnvalue_5 (`InstancedStaticMeshComponent.AddInstance` (`self.HISM_Bell`) (`KismetMathLibrary.MakeTransform` (`SplineComponent.GetLocationAtDistanceAlongSpline` _spline _returnvalue_3 "World") (`KismetMathLibrary.MakeRotator` _returnvalue_roll _returnvalue_pitch _returnvalue_yaw) (`KismetMathLibrary.Conv_DoubleToVector` (`self.InstanceScale`))) true))
          (`InstancedStaticMeshComponent.SetCustomDataValue` _hism_bell _returnvalue_5 0 (`KismetMathLibrary.RandomFloatInRange` 0.0 1.0) false)
          (`InstancedStaticMeshComponent.SetCustomDataValue` _hism_bell _returnvalue_5 1 (`KismetMathLibrary.RandomFloatInRange` 0.0 1.0) false)
          (`InstancedStaticMeshComponent.SetCustomDataValue` _hism_bell _returnvalue_5 2 (`KismetMathLibrary.RandomFloatInRange` 0.0 1.0) false)))
      (for _index_2 (range (+ (`KismetMathLibrary.FTrunc` (`SplineComponent.GetSplineLength` _spline_2)) 1))
        (set `self.SplineMeshIndex` _index_2)
        (`InstancedStaticMeshComponent.AddInstance` (`self.HISM_Rope`) (`KismetMathLibrary.MakeTransform` (`SplineComponent.GetLocationAtDistanceAlongSpline` _spline_2 _returnvalue "Local") (`SplineComponent.GetRotationAtDistanceAlongSpline` _spline_2 _returnvalue "Local") (`KismetMathLibrary.Conv_DoubleToVector` (`self.InstanceRopeScale`))) false)))))