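; Level-tool platform that sets a chosen mesh and strings bells and rope along a spline.
; When SpawnProcMesh is on, the construction script rebuilds both instanced meshes: a bell at each spline point and a rope instance every unit of spline length.
; An Attack event plays the bell sound at SoundLoc.
; Seeded random scattering of bells and spline points over mesh vertices is left unconnected.
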(event `/Game/Blueprint/Interface/BPI_Rock.Attack`
  (`GameplayStatics.PlaySoundAtLocation` "/Game/Audio/Sounds/SFX/Bell/SC_Bell.SC_Bell" (`SceneComponent.K2_GetComponentLocation` (`self.SoundLoc`)) (struct) 1.0 1.0 0.0 null null null null))

(fn `UserConstructionScript`
  (bind _spline (`self.Spline`))
  (bind _spline_2 (`self.Spline`))
  (bind _returnvalue (* (`self.SplineMeshIndex`) 1.0))
  (`KismetMathLibrary.SetRandomStreamSeed` (`self.Random Stream`) (`self.New Seed`))
  (`StaticMeshComponent.SetStaticMesh` (`self.StaticMesh`) (`self.PlatformMesh`))
  (if (`self.SpawnProcMesh?`)
    (`InstancedStaticMeshComponent.ClearInstances` (`self.HISM_Bell`))
    (`InstancedStaticMeshComponent.ClearInstances` (`self.HISM_Rope`))
    (for _index (range (+ (`SplineComponent.GetNumberOfSplinePoints` _spline) 1))
      (bind _returnvalue_2 (`SplineComponent.GetSplinePointAt` _spline _index "Local"))
      (`InstancedStaticMeshComponent.AddInstance` (`self.HISM_Bell`) (`KismetMathLibrary.MakeTransform` (`.Position` (break `SplinePoint` _returnvalue_2)) (`KismetMathLibrary.MakeRotator` 0.0 (.roll (`.Rotation` (break `SplinePoint` _returnvalue_2))) (+ (.yaw (`.Rotation` (break `SplinePoint` _returnvalue_2))) -90.0)) (`KismetMathLibrary.Conv_DoubleToVector` (`self.InstanceScale`))) false))
    (for _index_2 (range (+ (`KismetMathLibrary.FTrunc` (`SplineComponent.GetSplineLength` _spline_2)) 1))
      (set `self.SplineMeshIndex` _index_2)
      (`InstancedStaticMeshComponent.AddInstance` (`self.HISM_Rope`) (`KismetMathLibrary.MakeTransform` (`SplineComponent.GetLocationAtDistanceAlongSpline` _spline_2 _returnvalue "Local") (`SplineComponent.GetRotationAtDistanceAlongSpline` _spline_2 _returnvalue "Local") (`KismetMathLibrary.Conv_DoubleToVector` (`self.InstanceRopeScale`))) false))))