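; BP_FunnyTriggerer is a level-tool trigger that relays BP_PlayerRock overlaps to ActorToTrigger as dialogue and trigger messages.
; Entering the Sphere starts dialogue, and leaving it ends dialogue and clears the timer.
; With Tracing on, a fast looping timer line-traces from ActorToTrigger to the player's moving component, repeatedly sending start when clear and end when blocked.
; Entering the separate Box sends Trigger01Message.
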(event `self.Sphere.OnComponentBeginOverlap`
  (params (OverlappedComponent :type "PrimitiveComponent Object Reference") (OtherActor :type "Actor Object Reference") (OtherComp :type "PrimitiveComponent Object Reference") (OtherBodyIndex :type Integer) (bFromSweep :type Boolean) (SweepResult :type "HitResult Structure (by ref)"))
  (cast `/Game/Blueprint/Player/BP_PlayerRock` OtherActor)
  (if (`self.Tracing`)
    (bind _returnvalue (`KismetSystemLibrary.K2_SetTimerDelegate` (delegate `LineTrace`) 0.001 true true))
    (else
      (message `/Game/Blueprint/Interface/BPI_Rock.StartDialogue` (`self.ActorToTrigger`)))))

(event `LineTrace`
  (bind _outhit (`KismetSystemLibrary.LineTraceSingle` (`self.K2_GetActorLocation` (`self.ActorToTrigger`)) (`SceneComponent.K2_GetComponentLocation` (`/Game/Blueprint/Player/BP_PlayerRock.GetMovingComponent` (`/Game/Blueprint/BFL_Rock.GetPlayerActorRef`))) "TraceTypeQuery6"))
  (if (`GameplayStatics.BreakHitResult` _outhit)
    (message `/Game/Blueprint/Interface/BPI_Rock.EndDialogue` (`self.ActorToTrigger`))
    (else
      (message `/Game/Blueprint/Interface/BPI_Rock.StartDialogue` (`self.ActorToTrigger`)))))

(event `self.Sphere.OnComponentEndOverlap`
  (params (OverlappedComponent :type "PrimitiveComponent Object Reference") (OtherActor :type "Actor Object Reference") (OtherComp :type "PrimitiveComponent Object Reference") (OtherBodyIndex :type Integer))
  (cast `/Game/Blueprint/Player/BP_PlayerRock` OtherActor)
  (message `/Game/Blueprint/Interface/BPI_Rock.EndDialogue` (`self.ActorToTrigger`))
  (`KismetSystemLibrary.K2_ClearAndInvalidateTimerHandle` (stale `self.Sphere.OnComponentBeginOverlap` _returnvalue)))

(event `self.Box.OnComponentBeginOverlap`
  (params (OverlappedComponent :type "PrimitiveComponent Object Reference") (OtherActor :type "Actor Object Reference") (OtherComp :type "PrimitiveComponent Object Reference") (OtherBodyIndex :type Integer) (bFromSweep :type Boolean) (SweepResult :type "HitResult Structure (by ref)"))
  (cast `/Game/Blueprint/Player/BP_PlayerRock` OtherActor)
  (message `/Game/Blueprint/Interface/BPI_Rock.Trigger01` (`self.ActorToTrigger`)))

(fn `UserConstructionScript`)