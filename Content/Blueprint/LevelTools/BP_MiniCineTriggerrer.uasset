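; BP_MiniCineTriggerrer is a one-shot trigger volume that plays a short cinematic when the player rock enters its box.
; It locks the player, blends to its own camera while the Level Sequence plays, then blends back, unlocks and starts the referenced enemy's combat system.
; Separate events, not called within this graph, turn the enemy via timeline and reveal it with thunder VFX, camera shake and sound.
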(event `self.Box.OnComponentBeginOverlap`
  (params (OverlappedComponent :type "PrimitiveComponent Object Reference") (OtherActor :type "Actor Object Reference") (OtherComp :type "PrimitiveComponent Object Reference") (OtherBodyIndex :type Integer) (bFromSweep :type Boolean) (SweepResult :type "HitResult Structure (by ref)"))
  (bind _asbp_player_rock (`/Game/Blueprint/BFL_Rock.GetPlayerActorRef`))
  (bind _asbp_player_rock_2 (`/Game/Blueprint/BFL_Rock.GetPlayerActorRef`))
  (bind _ennemyref (`self.EnnemyREF`))
  (bind _camblendspeed_out (`self.CamBlendSpeed_Out`))
  (cast `/Game/Blueprint/Player/BP_PlayerRock` OtherActor)
  (`/Engine/EditorBlueprintResources/StandardMacros.DoOnce` false
    (:`Completed`
      (`/Game/Blueprint/Player/BP_PlayerRock.LockPlayer` _asbp_player_rock)
      (`PlayerController.SetViewTargetWithBlend` (`GameplayStatics.GetPlayerController` 0) self (`self.CamBlendSpeed_In`) "VTBlend_Linear" 0.0 false)
      (`/Game/Blueprint/Player/BP_PlayerRock.SetCurrentCameraUsed` _asbp_player_rock (`self.Camera`))
      (bind _outactor (`LevelSequencePlayer.CreateLevelSequencePlayer` (`self.Level Sequence`)))
      (bind _sequenceplayer (`LevelSequenceActor.SequencePlayer` _outactor))
      (`MovieSceneSequencePlayer.Play` _sequenceplayer)
      (`KismetSystemLibrary.Delay` (`self.SequenceLength`))
      (`MovieSceneSequencePlayer.Pause` _sequenceplayer)
      (`PlayerController.SetViewTargetWithBlend` (`GameplayStatics.GetPlayerController` 0) (`/Game/Blueprint/BFL_Rock.GetPlayerActorRef`) _camblendspeed_out "VTBlend_Linear" 0.0 false)
      (`/Game/Blueprint/Player/BP_PlayerRock.SetCurrentCameraUsed` _asbp_player_rock_2 (`/Game/Blueprint/Player/BP_PlayerRock.ThirdPersonCamera` _asbp_player_rock_2))
      (`KismetSystemLibrary.Delay` _camblendspeed_out)
      (`/Game/Blueprint/Player/BP_PlayerRock.UnlockPlayer` (`/Game/Blueprint/BFL_Rock.GetPlayerActorRef`))
      (`/Engine/EditorBlueprintResources/StandardMacros.IsValid` _ennemyref
        (:`Is Valid`
          (`/Game/Blueprint/Component/BPC_IA.StartSystem` (`/Game/Blueprint/IA/BP_IARock.BPC_CombatSystem` _ennemyref)))))))

(event `EndMini ciné`)

(event `/Game/Blueprint/Interface/BPI_Rock.Trigger01`
  (`TimelineComponent.SetPlayRate` (`self.Rotate`) (/ 1.0 0.4))
  (bind (_direction _newtrack_0) (`Timeline|Rotate` :!via `PlayFromStart`)
    (:`Update`
      (`self.K2_SetActorRotation` (`self.EnnemyREF`) (`KismetMathLibrary.RLerp` (struct) (struct :`Yaw` 175.0) _newtrack_0) false))))

(event `/Game/Blueprint/Interface/BPI_Rock.Shazam`
  (bind _returnvalue (- (`SceneComponent.K2_GetComponentLocation` (`self.Arrow`)) (0.0 0.0 80.0)))
  (`NiagaraFunctionLibrary.SpawnSystemAtLocation` "/Game/VFX/Thunderz/Thunder/Thunder.Thunder" _returnvalue)
  (`self.SetActorHiddenInGame` (`self.EnnemyREF`) false)
  (`GameplayStatics.PlayWorldCameraShake` "/Game/Blueprint/Player/CameraShakePlayer/CS_ImpactBoss.CS_ImpactBoss_C" _returnvalue 1000000000000.0)
  (`GameplayStatics.PlaySound2D` "/Game/Audio/Sounds/SFX/horizon-thunder-sphere-2.horizon-thunder-sphere-2" 1.0 1.0 0.0 null null))

(fn `UserConstructionScript`)