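; Boost volume that propels BP_PlayerRock along its arrow direction while the rock is inside the box.
; Overlap starts a looping 0.01s timer applying StartBoost and a physics impulse, plus sound, rumble and faster flower material animation.
; Exit clears the timer and slows the flowers after a delay.
; Construction script toggles tube, plane and Niagara visuals; box resizing and trace-based flower scattering are disconnected.
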(event `self.Box.OnComponentBeginOverlap`
  (params (OverlappedComponent :type "PrimitiveComponent Object Reference") (OtherActor :type "Actor Object Reference") (OtherComp :type "PrimitiveComponent Object Reference") (OtherBodyIndex :type Integer) (bFromSweep :type Boolean) (SweepResult :type "HitResult Structure (by ref)"))
  (bind _asbp_player_rock (cast `/Game/Blueprint/Player/BP_PlayerRock` OtherActor))
  (bind _returnvalue (`KismetSystemLibrary.K2_SetTimerDelegate` (delegate `Boosting`) 0.01 true true))
  (`GameplayStatics.PlaySound2D` "/Game/Audio/Sounds/SFX/FlowerBoost/SC_FlowerBoost.SC_FlowerBoost" 1.0 1.0 0.0 null null)
  (`MeshComponent.SetScalarParameterValueOnMaterials` (`self.HISM_Flower`) "Speed" 100.0)
  (`|ExecutionSequence`
    (:`then_0`
      (bind (_direction _newtrack_0) (`Timeline|Timeline` :!via `PlayFromStart`)))
    (:`then_1`
      (`PlayerController.PlayDynamicForceFeedback` (`GameplayStatics.GetPlayerController` 0) (`KismetMathLibrary.Lerp` 0.4 0.0 _newtrack_0) 0.6 true true true true))))

(event `Boosting`
  (`/Game/Blueprint/Player/BP_PlayerRock.StartBoost` (stale `self.Box.OnComponentBeginOverlap` _asbp_player_rock))
  (`PrimitiveComponent.AddImpulse` (`/Game/Blueprint/BFL_Rock.GetPhysicPlayerRef`) (* (`SceneComponent.GetForwardVector` (`self.Arrow`)) 300000.0 1.0) "None" false))

(event `self.Box.OnComponentEndOverlap`
  (params (OverlappedComponent :type "PrimitiveComponent Object Reference") (OtherActor :type "Actor Object Reference") (OtherComp :type "PrimitiveComponent Object Reference") (OtherBodyIndex :type Integer))
  (cast `/Game/Blueprint/Player/BP_PlayerRock` OtherActor)
  (`KismetSystemLibrary.K2_ClearAndInvalidateTimerHandle` (stale `self.Box.OnComponentBeginOverlap` _returnvalue))
  (`KismetSystemLibrary.Delay` 2.0)
  (`MeshComponent.SetScalarParameterValueOnMaterials` (`self.HISM_Flower`) "Speed" 10.0))

(fn `UserConstructionScript`
  (bind _niagara (`self.Niagara`))
  (`|ExecutionSequence`
    (:`then_0`
      (if (`self.Tube`)
        (`SceneComponent.SetVisibility` (`self.Niagara`) false false)
        (`SceneComponent.SetVisibility` (`self.Plane`) false false)
        (`SceneComponent.SetVisibility` (`self.Cylindre_Booster`) true false)
        (else
          (`SceneComponent.SetVisibility` (`self.Niagara`) true false)
          (`SceneComponent.SetVisibility` (`self.Plane`) true false)
          (`SceneComponent.SetVisibility` (`self.Cylindre_Booster`) false false))))
    (:`then_1`
      (if (`self.Flowers ?`)
        (`SceneComponent.SetVisibility` _niagara true false)
        (else
          (`SceneComponent.SetVisibility` _niagara false false))))))