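; Level start actor, tagged with its level name, that runs the transition into a level.
; StartLevel launches the player rock toward it, updates GM_Rock score, timer and level, then swaps streamed levels in blocking loops behind a transition.
; It then starts music and timer, moving the rock backward along a spline on a looping timer until control returns.
; With Cine set, it instead plays the plot-twist sequence, unlocks level data and triggers a checkpoint afterward.
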(event `IntroStopped`
  (bind _asbp_player_rock (`/Game/Blueprint/BFL_Rock.GetPlayerActorRef`))
  (bind _asbp_player_rock_2 (`/Game/Blueprint/BFL_Rock.GetPlayerActorRef`))
  (bind _fadecinescreen (`self.FadeCineScreen`))
  (set `self.cineend` true)
  (`PlayerController.SetViewTargetWithBlend` (`GameplayStatics.GetPlayerController` 0) _asbp_player_rock_2 1.0 "VTBlend_Linear" 0.0 true)
  (`/Game/Blueprint/Player/BP_PlayerRock.SetCurrentCameraUsed` _asbp_player_rock_2 (`/Game/Blueprint/Player/BP_PlayerRock.ThirdPersonCamera` _asbp_player_rock_2))
  (set `/Game/Blueprint/Player/BP_PlayerRock.ActualCinePlaying` null (`/Game/Blueprint/BFL_Rock.GetPlayerActorRef`))
  (`GameplayStatics.UnloadStreamLevelBySoftObjectPtr` "/Game/Level/Sublevel/SL_cinematic.SL_cinematic")
  (`/Game/Blueprint/Player/BP_PlayerRock.TrigerSleep` (`/Game/Blueprint/BFL_Rock.GetPlayerActorRef`))
  (`/Game/Blueprint/BFL_Rock.CloseCineDialogue`)
  (`self.SetActorHiddenInGame` (`/Game/Blueprint/BFL_Rock.GetPlayerActorRef`) false)
  (`KismetMaterialLibrary.SetScalarParameterValue` "/Game/Blueprint/Player/MPC_SEeThgh.MPC_SEeThgh" "Active" 1.0)
  (set `/Game/Blueprint/Player/BP_PlayerRock.ClampVelocity?` true (`/Game/Blueprint/BFL_Rock.GetPlayerActorRef`))
  (for _array_element (`self.KillZoneToActivate`)
    (set `/Game/Blueprint/LevelTools/BP_KillZone.Used?` true _array_element))
  (`/Game/Blueprint/Player/BP_PlayerRock.SetCurrentCameraUsed` _asbp_player_rock (`/Game/Blueprint/Player/BP_PlayerRock.ThirdPersonCamera` _asbp_player_rock))
  (`/Game/Blueprint/LevelTools/BP_CheckPoint.TrigerCheckpoint` (`self.Checkpoint`))
  (`KismetSystemLibrary.Delay` 1.0)
  (`/Game/Blueprint/Player/BP_PlayerRock.UnlockPlayer` (`/Game/Blueprint/BFL_Rock.GetPlayerActorRef`))
  (`UserWidget.PlayAnimation` _fadecinescreen (`/Game/UI/WBP/WBP_CineFade.FadeOut` _fadecinescreen) 0.0 1 "Forward" 1.0 false)
  (`/Game/Blueprint/Player/BP_PlayerRock.FadeBackOut` (`/Game/Blueprint/BFL_Rock.GetPlayerActorRef`))
  (`KismetSystemLibrary.Delay` 0.5)
  (`Widget.RemoveFromParent` _fadecinescreen))

(event `self.ReceiveBeginPlay`
  (set `self.Tags` (`|MakeArray` (`self.LevelName`)))
  (bind _returnvalue (`GameplayStatics.GetActorOfClass` "/Game/Blueprint/BP_SoundManager.BP_SoundManager_C"))
  (set `self.SoundManagerRef` _returnvalue)
  (bind _returnvalue_2 (`GameplayStatics.GetActorOfClass` "/Game/Blueprint/LevelTools/BP_CameraTransitionLevel.BP_CameraTransitionLevel_C"))
  (set `self.CameraTransitionRef` _returnvalue_2))

(event `StartLevel`
  (params (`Current Level` :type Integer))
  (bind _asbp_player_rock (`/Game/Blueprint/BFL_Rock.GetPlayerActorRef`))
  (bind _movingcomponent (`/Game/Blueprint/BFL_Rock.GetPhysicPlayerRef`))
  (bind (_level_data_levelname _level_data_levelunlocked _level_data_levelmaxmoss _level_data_levelmosstounlock _level_data_playermossscore _level_data_playertimesec _level_data_playertimemin _level_data_playercurrentmoss) (break `/Game/Blueprint/Player/F_LevelData` (`/Game/Blueprint/BFL_Rock.Get Level Data` 5)))
  (bind _asbp_player_rock_2 (`/Game/Blueprint/BFL_Rock.GetPlayerActorRef`))
  (bind _asbp_player_rock_3 (`/Game/Blueprint/BFL_Rock.GetPlayerActorRef`))
  (bind _soundmanagerref (`self.SoundManagerRef`))
  (bind _fadecinescreen (`self.FadeCineScreen`))
  (bind _leveltoload (`self.LevelToLoad`))
  (bind _fadecinescreen_2 (`self.FadeCineScreen`))
  (bind _leveltounload (`self.LevelToUnload`))
  (bind _soundmanagerref_2 (`self.SoundManagerRef`))
  (bind _asgm_rock (cast `/Game/Blueprint/Player/GM_Rock` (`GameplayStatics.GetGameMode`) :!pure true))
  (bind _mossquantity (`/Game/Blueprint/Player/BP_PlayerRock.MossQuantity` _asbp_player_rock))
  (bind _current_level (`/Game/Blueprint/Player/GM_Rock.Current Level` (cast `/Game/Blueprint/Player/GM_Rock` (`GameplayStatics.GetGameMode`) :!pure true)))
  (bind (_level_data_levelname_2 _level_data_levelunlocked_2 _level_data_levelmaxmoss_2 _level_data_levelmosstounlock_2 _level_data_playermossscore_2) (break `/Game/Blueprint/Player/F_LevelData` (`/Game/Blueprint/BFL_Rock.Get Level Data` (`/Game/Blueprint/Player/GM_Rock.Current Level` _asgm_rock))))
  (bind (_level_data_levelname_3 _level_data_levelunlocked_3 _level_data_levelmaxmoss_3 _level_data_levelmosstounlock_3 _level_data_playermossscore_3 _level_data_playertimesec_2 _level_data_playertimemin_2) (break `/Game/Blueprint/Player/F_LevelData` (`/Game/Blueprint/BFL_Rock.Get Level Data` _current_level)))
  ;[1 0.2165 0.7284] Start Level
  (set `/Game/Blueprint/LevelTools/BP_CameraTransitionLevel.TargetRot` (`SceneComponent.K2_GetComponentRotation` (`self.Arrow`)) (`self.CameraTransitionRef`))
  (`KismetSystemLibrary.DelayUntilNextTick`)
  (`self.LaunchPlayer`)
  (`KismetSystemLibrary.Delay` 1.0)
  (`GameplayStatics.PlaySound2D` "/Game/Audio/Sounds/SFX/LevelTransition/SC_LevelTransition_In.SC_LevelTransition_In" 1.0 1.0 0.0 null null)
  (`/Game/Blueprint/Player/BP_PlayerRock.CloseBlackScreen` _asbp_player_rock)
  (`/Game/Blueprint/Player/GM_Rock.Update Current Score` _asgm_rock (`KismetMathLibrary.SelectInt` _mossquantity _level_data_playermossscore_2 (> _mossquantity _level_data_playermossscore_2)))
  (`/Game/Blueprint/Player/GM_Rock.StopTimer` _asgm_rock true)
  (`/Game/Blueprint/Player/GM_Rock.UpdateTimer` _asgm_rock)
  (`/Game/Blueprint/Player/GM_Rock.Change Level` _asgm_rock `Current Level`)
  (`/Game/Blueprint/HUD/PQR_HUD.Set Max Moss` (cast `/Game/Blueprint/HUD/PQR_HUD` (`PlayerController.GetHUD` (`GameplayStatics.GetPlayerController` 0)) :!pure true) _level_data_levelmaxmoss_2)
  (`KismetSystemLibrary.Delay` 1.0)
  (set `self.AngularVelocity` (`PrimitiveComponent.GetPhysicsAngularVelocityInRadians` (`/Game/Blueprint/BFL_Rock.GetPhysicPlayerRef`) "None"))
  (`/Game/Blueprint/Player/BP_PlayerRock.LockPlayer` (`/Game/Blueprint/BFL_Rock.GetPlayerActorRef`))
  (`PrimitiveComponent.SetAngularDamping` _movingcomponent 0.0)
  (`PrimitiveComponent.SetPhysicsAngularVelocityInRadians` _movingcomponent (`self.AngularVelocity`) false "None")
  (`/Game/Blueprint/LevelTools/BP_CameraTransitionLevel.StopCameraShake` (`self.CameraTransitionRef`))
  (if (> (`self.LevelLoadLoopIndex`) (`KismetArrayLibrary.Array_Length` _leveltounload)) :!label _label
    (set `self.LevelLoadLoopIndex` 0)
    (`KismetSystemLibrary.Delay` 1.0)
    (if (> (`self.LevelLoadLoopIndex`) (`KismetArrayLibrary.Array_Length` _leveltoload)) :!label _label_2
      (set `self.LevelLoadLoopIndex` 0)
      (`KismetSystemLibrary.Delay` 1.0)
      (if (`self.Cine?`)
        (`/Engine/EditorBlueprintResources/StandardMacros.DoOnce` false
          (:`Completed`
            (`/Game/Blueprint/Player/BP_PlayerRock.LockPlayer` (`/Game/Blueprint/BFL_Rock.GetPlayerActorRef`))
            (`self.EnableInput` (`/Game/Blueprint/BFL_Rock.GetPlayerActorRef`) (`GameplayStatics.GetPlayerController` 0))
            (`/Game/Blueprint/BP_SoundManager.ChangeMusic` _soundmanagerref (`/Game/Blueprint/BP_SoundManager.SC_HubMusic` _soundmanagerref))
            (bind _returnvalue (`|CreateWidget` "/Game/UI/WBP/WBP_CineFade.WBP_CineFade_C"))
            (bind _output_get (set `self.FadeCineScreen` _returnvalue))
            (`UserWidget.AddToViewport` _output_get 0)
            (`/Game/Blueprint/Player/BP_PlayerRock.OpenBlackScreen` (`/Game/Blueprint/BFL_Rock.GetPlayerActorRef`) false)
            (`|ExecutionSequence`
              (:`then_0`
                (set `self.cineend` false)
                (`GameplayStatics.LoadStreamLevelBySoftObjectPtr` "/Game/Level/Sublevel/SL_cinematic.SL_cinematic" true)
                (`/Game/Blueprint/Player/BP_PlayerRock.RemoveMoss` _asbp_player_rock_3 (`/Game/Blueprint/Player/BP_PlayerRock.MossQuantity` _asbp_player_rock_3))
                (`self.SetActorHiddenInGame` (`/Game/Blueprint/BFL_Rock.GetPlayerActorRef`) true)
                (bind (_outactor _returnvalue_2) (`LevelSequencePlayer.CreateLevelSequencePlayer` "/Game/Cinematic/SEQ_2_PlotTwist/MS_plottwistnew.MS_plottwistnew"))
                (`/Engine/EditorBlueprintResources/StandardMacros.IsValid` _returnvalue_2
                  (:`Is Valid`
                    (bind _sequenceplayer (`LevelSequenceActor.SequencePlayer` _outactor))
                    (`MovieSceneSequencePlayer.Play` _sequenceplayer)
                    (bind _output_get_2 (set `/Game/Blueprint/Player/BP_PlayerRock.ActualCinePlaying` _sequenceplayer (`/Game/Blueprint/BFL_Rock.GetPlayerActorRef`)))
                    (`KismetMaterialLibrary.SetScalarParameterValue` "/Game/Blueprint/Player/MPC_SEeThgh.MPC_SEeThgh" "Active")
                    (add `MovieSceneSequencePlayer.OnStop` _returnvalue_2 (delegate `IntroStopped`))
                    (`PlayerController.SetViewTargetWithBlend` (`GameplayStatics.GetPlayerController` 0) _asbp_player_rock_2 1.0 "VTBlend_Linear" 0.0 true)
                    (`/Game/Blueprint/Player/BP_PlayerRock.SetCurrentCameraUsed` _asbp_player_rock_2 (`/Game/Blueprint/Player/BP_PlayerRock.ThirdPersonCamera` _asbp_player_rock_2))
                    (`SceneComponent.K2_SetWorldLocation` (`/Game/Blueprint/BFL_Rock.GetPhysicPlayerRef`) (487.982117 9632.643555 428.62381) false false)
                    (`/Game/Blueprint/Player/BP_PlayerRock.LockPlayer` (`/Game/Blueprint/BFL_Rock.GetPlayerActorRef`))
                    (`/Game/Blueprint/BFL_Rock.SetLevelData` 5 (make `/Game/Blueprint/Player/F_LevelData` _level_data_levelname true _level_data_levelmaxmoss _level_data_levelmosstounlock _level_data_playermossscore _level_data_playertimesec _level_data_playertimemin _level_data_playercurrentmoss))
                    (bind _returnvalue_3 (- (`TimeManagementBlueprintLibrary.Conv_QualifiedFrameTimeToSeconds` (`MovieSceneSequencePlayer.GetDuration` _output_get_2)) 1.0))
                    (`KismetSystemLibrary.PrintString` (`KismetStringLibrary.Conv_DoubleToString` _returnvalue_3))
                    (`KismetSystemLibrary.Delay` _returnvalue_3)
                    (`/Engine/EditorBlueprintResources/StandardMacros.IsValid` _returnvalue_2
                      (:`Is Valid`
                        (`KismetSystemLibrary.PrintString` "fadefin" true false)
                        (if (not (`self.cineend`))
                          (`UserWidget.PlayAnimation` _fadecinescreen_2 (`/Game/UI/WBP/WBP_CineFade.FadeIn` _fadecinescreen_2) 0.0 1 "Forward" 1.0 false)))))))
              (:`then_1`
                (`KismetSystemLibrary.Delay` 0.5)
                (`UserWidget.PlayAnimation` _fadecinescreen (`/Game/UI/WBP/WBP_CineFade.FadeOut` _fadecinescreen) 0.0 1 "Forward" 1.0 false)))))
        (else
          (`PlayerController.SetViewTargetWithBlend` (`GameplayStatics.GetPlayerController` 0) self 0.0 "VTBlend_Linear" 0.0 true)
          (`/Game/Blueprint/Player/BP_PlayerRock.SetCurrentCameraUsed` (`/Game/Blueprint/BFL_Rock.GetPlayerActorRef`) (`self.Camera`))
          (`/Game/Blueprint/Player/BP_PlayerRock.OpenBlackScreen` (`/Game/Blueprint/BFL_Rock.GetPlayerActorRef`) false)
          (`GameplayStatics.PlaySound2D` "/Game/Audio/Sounds/SFX/LevelTransition/SC_LevelTransition_Out.SC_LevelTransition_Out" 1.0 1.0 0.0 null null)
          (`/Game/Blueprint/Player/GM_Rock.StartTimer` (cast `/Game/Blueprint/Player/GM_Rock` (`GameplayStatics.GetGameMode`) :!pure true) (and (!= _current_level 0) (> (+ _level_data_playertimesec_2 _level_data_playertimemin_2) 0)))
          (`PrimitiveComponent.SetPhysicsAngularVelocityInRadians` (`/Game/Blueprint/BFL_Rock.GetPhysicPlayerRef`) (0.0 0.0 0.0) false "None")
          (set `self.Current` (`SplineComponent.GetSplineLength` (`self.Spline`)))
          (bind _returnvalue_4 (`KismetSystemLibrary.K2_SetTimerDelegate` (delegate `UpdateLanding`) 0.01 true true))
          (`/Game/Blueprint/BP_SoundManager.ChangeMusic` _soundmanagerref_2 (select `int` (`self.LevelMusic`) :`0` (`/Game/Blueprint/BP_SoundManager.SC_MushroomMusic` _soundmanagerref_2) :`1` (`/Game/Blueprint/BP_SoundManager.SC_RuinMusic` _soundmanagerref_2) :`2` (`/Game/Blueprint/BP_SoundManager.SC_HubMusic` _soundmanagerref_2)))
          (`/Game/Blueprint/Player/BP_PlayerRock.TrigerSleep` (`/Game/Blueprint/BFL_Rock.GetPlayerActorRef`))))
      (else
        (`GameplayStatics.LoadStreamLevelBySoftObjectPtr` (`|GetArrayItem` _leveltoload (`self.LevelLoadLoopIndex`)) true true)
        (set `self.LevelLoadLoopIndex` (+ (`self.LevelLoadLoopIndex`) 1))
        (goto _label_2)))
    (else
      (`GameplayStatics.UnloadStreamLevelBySoftObjectPtr` (`|GetArrayItem` _leveltounload (`self.LevelLoadLoopIndex`)) true)
      (set `self.LevelLoadLoopIndex` (+ (`self.LevelLoadLoopIndex`) 1))
      (goto _label))))

(event `ClearLanding`
  (bind _asbp_player_rock (`/Game/Blueprint/BFL_Rock.GetPlayerActorRef`))
  (bind _asbp_player_rock_2 (`/Game/Blueprint/BFL_Rock.GetPlayerActorRef`))
  ;[1 0.2165 0.7284] Start Level
  (`KismetSystemLibrary.K2_ClearAndInvalidateTimerHandle` (stale `StartLevel` _returnvalue_4))
  (`AudioComponent.SetFloatParameter` (`/Game/Blueprint/Player/BP_PlayerRock.WindSoundRef` _asbp_player_rock) "WindVolume" 0.0)
  (`/Game/Blueprint/Player/BP_PlayerRock.UnlockPlayer` _asbp_player_rock)
  (`self.EnableInput` (`/Game/Blueprint/BFL_Rock.GetPlayerActorRef`) (`GameplayStatics.GetPlayerController` 0))
  (set `/Game/Blueprint/Player/BP_PlayerRock.ClampVelocity?` true _asbp_player_rock)
  (for _array_element (`self.KillZoneToActivate`)
    (set `/Game/Blueprint/LevelTools/BP_KillZone.Used?` true _array_element))
  (`PlayerController.SetViewTargetWithBlend` (`GameplayStatics.GetPlayerController` 0) _asbp_player_rock_2 1.0 "VTBlend_Linear" 0.0 true)
  (`/Game/Blueprint/Player/BP_PlayerRock.SetCurrentCameraUsed` _asbp_player_rock_2 (`/Game/Blueprint/Player/BP_PlayerRock.ThirdPersonCamera` _asbp_player_rock_2)))

(event `UpdateLanding`
  (bind _current (`self.Current`))
  (bind _returnvalue (`KismetMathLibrary.FInterpTo_Constant` _current 0.0 (`GameplayStatics.GetWorldDeltaSeconds`) (* (`/Game/Blueprint/Player/BP_PlayerRock.MaxVelocity` (`/Game/Blueprint/BFL_Rock.GetPlayerActorRef`)) 1.5)))
  ;[1 0.2165 0.7284] Start Level
  (`KismetSystemLibrary.PrintString` (`KismetStringLibrary.Conv_DoubleToString` _current))
  (if (<= _current 250.0)
    (`self.ClearLanding`)
    (else
      (`SceneComponent.K2_SetWorldLocation` (`/Game/Blueprint/BFL_Rock.GetPhysicPlayerRef`) (`SplineComponent.GetLocationAtDistanceAlongSpline` (`self.Spline`) _returnvalue "World") false false)
      (set `self.Current` _returnvalue))))

(event `self.Box.OnComponentBeginOverlap`
  (params (OverlappedComponent :type "PrimitiveComponent Object Reference") (OtherActor :type "Actor Object Reference") (OtherComp :type "PrimitiveComponent Object Reference") (OtherBodyIndex :type Integer) (bFromSweep :type Boolean) (SweepResult :type "HitResult Structure (by ref)"))
  (cast `/Game/Blueprint/Player/BP_PlayerRock` OtherActor)
  (`/Engine/EditorBlueprintResources/StandardMacros.DoOnce` false :!label _label_3))

(event `self.Box.OnComponentEndOverlap`
  (params (OverlappedComponent :type "PrimitiveComponent Object Reference") (OtherActor :type "Actor Object Reference") (OtherComp :type "PrimitiveComponent Object Reference") (OtherBodyIndex :type Integer))
  (cast `/Game/Blueprint/Player/BP_PlayerRock` OtherActor)
  (goto _label_3 :!via `Reset`))

(fn `LandPlayer`
  (params (Distance :type "Float (single-precision)"))
  (`SceneComponent.K2_SetWorldLocation` (`/Game/Blueprint/BFL_Rock.GetPhysicPlayerRef`) (`SplineComponent.GetLocationAtDistanceAlongSpline` (`self.Spline`) Distance "World") false false))

(fn `LaunchPlayer`
  (bind _asbp_player_rock (`/Game/Blueprint/BFL_Rock.GetPlayerActorRef`))
  (bind (_tossvelocity _returnvalue) (`GameplayStatics.BlueprintSuggestProjectileVelocity` (`SceneComponent.K2_GetComponentLocation` (`/Game/Blueprint/Player/BP_PlayerRock.GetMovingComponent` (`/Game/Blueprint/BFL_Rock.GetPlayerActorRef`))) (`self.K2_GetActorLocation`) (`self.Launch Speed`) 0.0 "DoNotTrace" 0.0 false true))
  (`KismetSystemLibrary.PrintString` (`KismetStringLibrary.Conv_BoolToString` _returnvalue) true false (struct :`G` 0.66 :`B` 1.0 :`A` 1.0) 10.0)
  (`/Game/Blueprint/Player/BP_PlayerRock.UnlockPlayer` (`/Game/Blueprint/BFL_Rock.GetPlayerActorRef`))
  (set `/Game/Blueprint/Player/BP_PlayerRock.CanMove?` false _asbp_player_rock)
  (set `/Game/Blueprint/Player/BP_PlayerRock.ClampVelocity?` false _asbp_player_rock)
  (set `/Game/Blueprint/Player/BP_PlayerRock.CanLook?` false _asbp_player_rock)
  (`PrimitiveComponent.AddImpulse` (`/Game/Blueprint/BFL_Rock.GetPhysicPlayerRef`) _tossvelocity "None" true))

(fn `UserConstructionScript`
  (`BoxComponent.SetBoxExtent` (`self.Box`) (`self.In Box Extent`) true)
  (set `self.Tags` (`|MakeArray` (`self.LevelName`))))