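; Level-tool kill zone that kills the rolling rock player on entering its box and respawns it at the last checkpoint.
; When enabled, the overlap sets a death flag on the GameInstance to block re-entry, disables input and resets rail-tube cameras.
; Chained timelines drive a circle wipe through a UI material parameter collection.
; A black screen covers the teleport to the saved transform, then the wipe reopens and control returns.
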(event `self.PreviewBox.OnComponentBeginOverlap`
  (params (OverlappedComponent :type "PrimitiveComponent Object Reference") (OtherActor :type "Actor Object Reference") (OtherComp :type "PrimitiveComponent Object Reference") (OtherBodyIndex :type Integer) (bFromSweep :type Boolean) (SweepResult :type "HitResult Structure (by ref)"))
  (bind _movingcomponent (`/Game/Blueprint/BFL_Rock.GetPhysicPlayerRef`))
  (bind _playerref (`self.PlayerREF`))
  (bind _playerref_2 (`self.PlayerREF`))
  (bind (_key _value) (`BlueprintMapLibrary.Map_GetKeyValueByIndex` (`/Game/Blueprint/GameInstance/GI_PierreQuiRouleGameInstance.LastCheckPointLocation` (cast `/Game/Blueprint/GameInstance/GI_PierreQuiRouleGameInstance` (`GameplayStatics.GetGameInstance`) :!pure true))))
  (bind _asbp_player_rock (cast `/Game/Blueprint/Player/BP_PlayerRock` OtherActor))
  (set `self.PlayerREF` _asbp_player_rock)
  (if (`self.Used?`)
    (`KismetSystemLibrary.PrintString` (`KismetStringLibrary.Concat_StrStr` "HitKillzone : " (`KismetSystemLibrary.GetDisplayName` self)) true false (struct :`R` 1.0 :`B` 0.117776 :`A` 1.0))
    (if (`/Game/Blueprint/Player/BP_PlayerRock.ShouldTick?` (`/Game/Blueprint/BFL_Rock.GetPlayerActorRef`))
      (bind _asgi_pierre_qui_roule_game_instance (cast `/Game/Blueprint/GameInstance/GI_PierreQuiRouleGameInstance` (`GameplayStatics.GetGameInstance`)))
      (if (not (`/Game/Blueprint/GameInstance/GI_PierreQuiRouleGameInstance.Ded` _asgi_pierre_qui_roule_game_instance))
        (set `/Game/Blueprint/GameInstance/GI_PierreQuiRouleGameInstance.Ded` true _asgi_pierre_qui_roule_game_instance)
        (`KismetSystemLibrary.PrintString` (`KismetStringLibrary.Concat_StrStr` "kiled by :" (`KismetSystemLibrary.GetDisplayName` self)) true false (struct :`R` 1.0 :`B` 0.08985 :`A` 1.0))
        (`self.DisableInput` (`GameplayStatics.GetPlayerController` 0))
        (`|ExecutionSequence`
          (:`then_0`
            (`SceneComponent.SetVisibility` (`/Game/Blueprint/Player/BP_PlayerRock.Widget` (`self.PlayerREF`)) true false)
            (`/Game/Blueprint/Player/BP_PlayerRock.Cancel Down Dash` (`/Game/Blueprint/BFL_Rock.GetPlayerActorRef`))
            (`/Game/Blueprint/Player/BP_PlayerRock.ResetCameraRotation` (`self.PlayerREF`))
            (`TimelineComponent.SetPlayRate` (`self.ActivFade`) (/ 1.0 0.3))
            (`GameplayStatics.PlaySound2D` "/Game/Audio/Sounds/SFX/Death/SC_Death.SC_Death" 1.0 1.0 0.0 null null)
            (bind (_direction _newtrack_0) (`Timeline|ActivFade` :!via `PlayFromStart`)
              (:`Update`
                (`KismetMaterialLibrary.SetScalarParameterValue` "/Game/Art/Material/UI_Materials/MPC_UI.MPC_UI" "CircleSize" (`KismetMathLibrary.Lerp` 200.0 70.0 _newtrack_0))
                (`TimelineComponent.SetPlayRate` (`self.FadeIN`) (/ 1.0 0.8)))
              (:`Finished`
                (`TimelineComponent.SetPlayRate` (`self.FadeIN`) (/ 1.0 1.5))
                (bind (_direction_2 _newtrack_0_2) (`Timeline|FadeIN` :!via `PlayFromStart`)
                  (:`Update`
                    (`KismetMaterialLibrary.SetScalarParameterValue` "/Game/Art/Material/UI_Materials/MPC_UI.MPC_UI" "CircleSize" (`KismetMathLibrary.Lerp` 70.0 0.0 _newtrack_0_2)))
                  (:`Finished`
                    (`KismetSystemLibrary.DelayUntilNextTick`)
                    (bind _returnvalue (`|CreateWidget` "/Game/UI/WBP/WBP_BlackScreen.WBP_BlackScreen_C"))
                    (`UserWidget.AddToViewport` _returnvalue 0)
                    (`KismetSystemLibrary.Delay` 0.5)
                    (`/Game/Blueprint/Player/BP_PlayerRock.LockPlayer` _playerref)
                    (`SceneComponent.K2_SetWorldLocation` _movingcomponent _key false true)
                    (`SceneComponent.K2_SetWorldRotation` _movingcomponent _value false false)
                    (`/Game/Blueprint/Player/BP_PlayerRock.ResetCameraRotation_Death` _playerref)
                    (`KismetSystemLibrary.Delay` 1.5)
                    (`Widget.RemoveFromParent` _returnvalue)
                    (`GameplayStatics.PlaySound2D` "/Game/Audio/Sounds/SFX/Death/SC_Respawn.SC_Respawn" 1.0 1.0 0.0 null null)
                    (bind (_direction_3 _newtrack_0_3) (`Timeline|FadeOUT` :!via `PlayFromStart`)
                      (:`Update`
                        (`KismetMaterialLibrary.SetScalarParameterValue` "/Game/Art/Material/UI_Materials/MPC_UI.MPC_UI" "CircleSize" (`KismetMathLibrary.Lerp` 0.0 70.0 _newtrack_0_3)))
                      (:`Finished`
                        (`self.EnableInput` _playerref_2 (`GameplayStatics.GetPlayerController` 0))
                        (`/Game/Blueprint/Player/BP_PlayerRock.UnlockPlayer` _playerref_2)
                        (`SceneComponent.SetVisibility` (`/Game/Blueprint/Player/BP_PlayerRock.Widget` (`self.PlayerREF`)) false false)
                        (set `/Game/Blueprint/GameInstance/GI_PierreQuiRouleGameInstance.Ded` false (cast `/Game/Blueprint/GameInstance/GI_PierreQuiRouleGameInstance` (`GameplayStatics.GetGameInstance`) :!pure true)))))))))
          (:`then_1`
            (bind _outactors (`GameplayStatics.GetAllActorsOfClass` "/Game/Blueprint/LevelTools/BP_CameraRailTubes.BP_CameraRailTubes_C"))
            (for _array_element _outactors
              (`/Game/Blueprint/LevelTools/BP_CameraRailTubes.ResetCameraSnap` _array_element))))))))

(fn `UserConstructionScript`
  (`SceneComponent.SetHiddenInGame` (`self.PreviewBox`) (`self.HiddenInGame`) false))