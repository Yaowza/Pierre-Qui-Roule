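; BP_HubLanding is a hub landing trigger that plays the MS_plottwist cinematic when the player comes within landing range.
; Tick compares the player's physics location to the actor while ShouldCheck is set, firing through a DoOnce.
; It clamps velocity, unlocks the player and clears the check, then after a delay locks the player, hides itself and plays the sequence.
; When the sequence stops, it unlocks the player and unhides itself after a short delay.
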(event `self.ReceiveTick`
  (params (DeltaSeconds :type "Float (single-precision)"))
  (bind _asbp_player_rock (`/Game/Blueprint/BFL_Rock.GetPlayerActorRef`))
  (if (and (`self.ShouldCheck?`) (<= (`KismetMathLibrary.Vector_Distance` (`SceneComponent.K2_GetComponentLocation` (`/Game/Blueprint/BFL_Rock.GetPhysicPlayerRef`)) (`self.K2_GetActorLocation`)) (`self.LandingRange`)))
    (`/Engine/EditorBlueprintResources/StandardMacros.DoOnce` false :!label _label
      (:`Completed`
        (set `/Game/Blueprint/Player/BP_PlayerRock.ClampVelocity?` true _asbp_player_rock)
        (`/Game/Blueprint/Player/BP_PlayerRock.UnlockPlayer` _asbp_player_rock)
        (set `self.ShouldCheck?` false)
        (`KismetSystemLibrary.Delay` 2.0)
        (`/Game/Blueprint/Player/BP_PlayerRock.LockPlayer` (`/Game/Blueprint/BFL_Rock.GetPlayerActorRef`))
        (`self.SetActorHiddenInGame` true)
        (bind (_outactor _returnvalue) (`LevelSequencePlayer.CreateLevelSequencePlayer` "/Game/Cinematic/PlotTwist/MS_plottwist.MS_plottwist"))
        (`MovieSceneSequencePlayer.Play` (`LevelSequenceActor.SequencePlayer` _outactor))
        (add `MovieSceneSequencePlayer.OnStop` _returnvalue (delegate `CineStopped`))
        (`KismetSystemLibrary.Delay` 5.0)
        (goto _label :!via `Reset`)))))

(event `CineStopped`
  (`KismetSystemLibrary.Delay` 1.0)
  (`/Game/Blueprint/Player/BP_PlayerRock.UnlockPlayer` (`/Game/Blueprint/BFL_Rock.GetPlayerActorRef`))
  (`self.SetActorHiddenInGame` false))

(fn `UserConstructionScript`)