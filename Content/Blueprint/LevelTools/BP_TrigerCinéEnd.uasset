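; BP_TrigerCinéEnd is a level trigger volume that starts combat when the player enters it, apparently marking the end of a cinematic.
; The first BP_PlayerRock overlap on its Box calls StartSystem on the BPCCombatSystem of the referenced CombatREF, destroys MeshToDestroy, then destroys the trigger itself.
; The construction script sizes the Box from the InBoxExtent variable.
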(event `self.Box.OnComponentBeginOverlap`
  (params (OverlappedComponent :type "PrimitiveComponent Object Reference") (OtherActor :type "Actor Object Reference") (OtherComp :type "PrimitiveComponent Object Reference") (OtherBodyIndex :type Integer) (bFromSweep :type Boolean) (SweepResult :type "HitResult Structure (by ref)"))
  (cast `/Game/Blueprint/Player/BP_PlayerRock` OtherActor)
  (`/Engine/EditorBlueprintResources/StandardMacros.DoOnce` false
    (:`Completed`
      (`/Game/Blueprint/Component/BPC_IA.StartSystem` (`/Game/Blueprint/IA/BP_IARock.BPC_CombatSystem` (`self.CombatREF`)))
      (`self.K2_DestroyActor` (`self.MeshToDestroy`))
      (`self.K2_DestroyActor`))))

(fn `UserConstructionScript`
  (`BoxComponent.SetBoxExtent` (`self.Box`) (`self.In Box Extent`) true))