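; BP_ReturnHub is a level trigger that sends the player rock back to the hub when it overlaps the box.
; It clears the listed kill zones' Used flags, removes the player's moss, locks look and movement, and launches the physics body toward BP_HubLanding using a suggested projectile velocity impulse.
; It enables the landing's check, then after a delay unloads the streamed level, restores look and re-arms.
; The hub music change is disconnected.
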(event `self.ReceiveBeginPlay`
  (bind _returnvalue (`GameplayStatics.GetActorOfClass` "/Game/Blueprint/BP_SoundManager.BP_SoundManager_C"))
  (set `self.SoundManagerRef` _returnvalue))

(event `self.Box.OnComponentBeginOverlap`
  (params (OverlappedComponent :type "PrimitiveComponent Object Reference") (OtherActor :type "Actor Object Reference") (OtherComp :type "PrimitiveComponent Object Reference") (OtherBodyIndex :type Integer) (bFromSweep :type Boolean) (SweepResult :type "HitResult Structure (by ref)"))
  (bind _asbp_player_rock (`/Game/Blueprint/BFL_Rock.GetPlayerActorRef`))
  (cast `/Game/Blueprint/Player/BP_PlayerRock` OtherActor)
  (`/Engine/EditorBlueprintResources/StandardMacros.DoOnce` false :!label _label
    (:`Completed`
      (for _array_element (`self.KillZoneToDsactivate`)
        (set `/Game/Blueprint/LevelTools/BP_KillZone.Used?` false _array_element))
      (bind _returnvalue (`GameplayStatics.GetActorOfClass` "/Game/Blueprint/LevelTools/BP_HubLanding.BP_HubLanding_C"))
      (set `self.HubLandingRef` _returnvalue)
      (`KismetSystemLibrary.DelayUntilNextTick`)
      (set `/Game/Blueprint/Player/BP_PlayerRock.CanLook?` false _asbp_player_rock)
      (`/Game/Blueprint/Player/BP_PlayerRock.RemoveMoss` _asbp_player_rock (`/Game/Blueprint/Player/BP_PlayerRock.MossQuantity` _asbp_player_rock))
      (`self.LaunchPlayer`)
      (set `/Game/Blueprint/LevelTools/BP_HubLanding.ShouldCheck?` true (`self.HubLandingRef`))
      (`KismetSystemLibrary.Delay` 3.0)
      (`GameplayStatics.UnloadStreamLevelBySoftObjectPtr` (`self.Level`))
      (set `/Game/Blueprint/Player/BP_PlayerRock.CanLook?` true (`/Game/Blueprint/BFL_Rock.GetPlayerActorRef`))
      (goto _label :!via `Reset`))))

(fn `LaunchPlayer`
  (bind _asbp_player_rock (`/Game/Blueprint/BFL_Rock.GetPlayerActorRef`))
  (`/Game/Blueprint/Player/BP_PlayerRock.LockPlayer` (`/Game/Blueprint/BFL_Rock.GetPlayerActorRef`))
  (bind _tossvelocity (`GameplayStatics.BlueprintSuggestProjectileVelocity` (`SceneComponent.K2_GetComponentLocation` (`/Game/Blueprint/BFL_Rock.GetPhysicPlayerRef`)) (`self.K2_GetActorLocation` (`self.HubLandingRef`)) 50000.0 0.0 "DoNotTrace" 0.0 false true))
  (`/Game/Blueprint/Player/BP_PlayerRock.UnlockPlayer` (`/Game/Blueprint/BFL_Rock.GetPlayerActorRef`))
  (set `/Game/Blueprint/Player/BP_PlayerRock.CanMove?` false _asbp_player_rock)
  (set `/Game/Blueprint/Player/BP_PlayerRock.ClampVelocity?` false _asbp_player_rock)
  (`PrimitiveComponent.AddImpulse` (`/Game/Blueprint/BFL_Rock.GetPhysicPlayerRef`) _tossvelocity "None" true))

(fn `UserConstructionScript`)