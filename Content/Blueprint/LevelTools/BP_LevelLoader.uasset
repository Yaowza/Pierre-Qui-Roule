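; Level streaming trigger volume that swaps sublevels as the player rock enters or leaves its box.
; On begin overlap it unloads the LevelToUnload list and loads and shows the LevelToLoad list, without blocking.
; On end overlap it reverses the swap unless Once is set.
; Each direction has a DoOnce gate that resets after a short delay to debounce repeated overlaps.
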(event `self.Box.OnComponentBeginOverlap`
  (params (OverlappedComponent :type "PrimitiveComponent Object Reference") (OtherActor :type "Actor Object Reference") (OtherComp :type "PrimitiveComponent Object Reference") (OtherBodyIndex :type Integer) (bFromSweep :type Boolean) (SweepResult :type "HitResult Structure (by ref)"))
  (cast `/Game/Blueprint/Player/BP_PlayerRock` OtherActor)
  (`/Engine/EditorBlueprintResources/StandardMacros.DoOnce` false :!label _label
    (:`Completed`
      (`|ExecutionSequence`
        (:`then_0`
          (for _array_element (`self.LevelToUnload`)
            (`GameplayStatics.UnloadStreamLevelBySoftObjectPtr` _array_element)))
        (:`then_1`
          (for _array_element_2 (`self.LevelToLoad`)
            (`GameplayStatics.LoadStreamLevelBySoftObjectPtr` _array_element_2 true))
          (`KismetSystemLibrary.Delay` 0.25)
          (goto _label :!via `Reset`))))))

(event `self.Box.OnComponentEndOverlap`
  (params (OverlappedComponent :type "PrimitiveComponent Object Reference") (OtherActor :type "Actor Object Reference") (OtherComp :type "PrimitiveComponent Object Reference") (OtherBodyIndex :type Integer))
  (cast `/Game/Blueprint/Player/BP_PlayerRock` OtherActor)
  (if (not (`self.Once`))
    (`/Engine/EditorBlueprintResources/StandardMacros.DoOnce` false :!label _label_2
      (:`Completed`
        (`|ExecutionSequence`
          (:`then_0`
            (for _array_element (`self.LevelToLoad`)
              (`GameplayStatics.UnloadStreamLevelBySoftObjectPtr` _array_element)))
          (:`then_1`
            (for _array_element_2 (`self.LevelToUnload`)
              (`GameplayStatics.LoadStreamLevelBySoftObjectPtr` _array_element_2 true))
            (`KismetSystemLibrary.Delay` 0.25)
            (goto _label_2 :!via `Reset`)))))))

(fn `UserConstructionScript`)