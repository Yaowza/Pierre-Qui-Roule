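; Trigger volume that shifts Ultra Dynamic Sky lighting while BP_PlayerRock is inside its box.
; On overlap it finds the sky actor and plays the Switch timeline, lerping sun latitude, longitude and light intensity.
; On exit it reverses the timeline from its end at a faster play rate.
; A large set of cloud, fog, color, date and lens flare lerps is left disconnected and never runs.
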(event `self.ReceiveBeginPlay`)

(event `self.Box.OnComponentBeginOverlap`
  (params (OverlappedComponent :type "PrimitiveComponent Object Reference") (OtherActor :type "Actor Object Reference") (OtherComp :type "PrimitiveComponent Object Reference") (OtherBodyIndex :type Integer) (bFromSweep :type Boolean) (SweepResult :type "HitResult Structure (by ref)"))
  (cast `/Game/Blueprint/Player/BP_PlayerRock` OtherActor)
  (bind _returnvalue (`GameplayStatics.GetActorOfClass` "/Game/UltraDynamicSky/Blueprints/Ultra_Dynamic_Sky.Ultra_Dynamic_Sky_C"))
  (bind _output_get (set `self.lightref` _returnvalue))
  (`TimelineComponent.SetPlayRate` (`self.Switch`) (/ 1.0 0.1))
  (bind (_direction _newtrack_1) (`Timeline|Switch` :!via `PlayFromStart` :!label _label)
    (:`Update`
      (set `/Game/UltraDynamicSky/Blueprints/Ultra_Dynamic_Sky.Latitude` (`KismetMathLibrary.Lerp` -59.76007 0.720109 _newtrack_1) _output_get)
      (set `/Game/UltraDynamicSky/Blueprints/Ultra_Dynamic_Sky.Longitude` (`KismetMathLibrary.Lerp` 1.440153 -30.239874 _newtrack_1) _output_get)
      (set `/Game/UltraDynamicSky/Blueprints/Ultra_Dynamic_Sky.Sun Light Intensity` (`KismetMathLibrary.Lerp` 200.0 100.0 _newtrack_1) _output_get))))

(event `self.Box.OnComponentEndOverlap`
  (params (OverlappedComponent :type "PrimitiveComponent Object Reference") (OtherActor :type "Actor Object Reference") (OtherComp :type "PrimitiveComponent Object Reference") (OtherBodyIndex :type Integer))
  (cast `/Game/Blueprint/Player/BP_PlayerRock` OtherActor)
  (`TimelineComponent.SetPlayRate` (`self.Switch`) (/ 1.0 0.05))
  (goto _label :!via `ReverseFromEnd`))

(fn `UserConstructionScript`)