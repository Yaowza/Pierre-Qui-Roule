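; Level actor that drains the BP_PlayerRock player's moss on contact when its first tag is Boss.
; Overlap or hit starts a one-time, tick-by-tick loop that removes moss while growing the mesh, and hits also play a debounced bell.
; The construction script scatters seeded moss HISM instances around the mesh.
; Boss cinematic and older shred branches are unwired, leaving their player-unlock callbacks unbound.
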(event `self.ReceiveBeginPlay`
  (set `self.Tags` (`|MakeArray` (`self.Tag`))))

(event `CustomEvent`
  (`KismetSystemLibrary.Delay` 1.0)
  (`/Game/Blueprint/Player/BP_PlayerRock.UnlockPlayer` (`/Game/Blueprint/BFL_Rock.GetPlayerActorRef`))
  (`self.SetActorHiddenInGame` (`/Game/Blueprint/BFL_Rock.GetPlayerActorRef`) false))

(event `self.SphereAbsorber.OnComponentBeginOverlap`
  (params (OverlappedComponent :type "PrimitiveComponent Object Reference") (OtherActor :type "Actor Object Reference") (OtherComp :type "PrimitiveComponent Object Reference") (OtherBodyIndex :type Integer) (bFromSweep :type Boolean) (SweepResult :type "HitResult Structure (by ref)"))
  (bind _playerref (`self.playerref`))
  (bind _mossquantity (`/Game/Blueprint/Player/BP_PlayerRock.MossQuantity` _playerref))
  (bind _asbp_player_rock (cast `/Game/Blueprint/Player/BP_PlayerRock` OtherActor))
  (set `self.playerref` _asbp_player_rock)
  (if (> _mossquantity 0) :!label _label
    (switch `name` (`|GetArrayItem` (`self.Tags`))
      (:`Boss`
        (`/Engine/EditorBlueprintResources/StandardMacros.DoOnce` false
          (:`Completed`
            (`|ExecutionSequence`
              (:`then_0`
                (set `self.PreshredMoss` _mossquantity)
                (if (<= _mossquantity 2) :!label _label_2
                  (set `/Game/Blueprint/Player/BP_PlayerRock.MossQuantity` 0 _playerref)
                  (else
                    (`/Game/Blueprint/Player/BP_PlayerRock.RemoveMoss` _playerref 2)
                    (`SceneComponent.SetRelativeScale3D` (`self.StaticMesh`) (`KismetMathLibrary.Conv_DoubleToVector` (`KismetMathLibrary.MapRangeClamped` (`KismetMathLibrary.Conv_IntToDouble` _mossquantity) 1000.0 0.0 3.4 4.5)))
                    (`KismetSystemLibrary.DelayUntilNextTick`)
                    (goto _label_2)))))))))))

(event `self.Sphere.OnComponentHit`
  (params (HitComponent :type "PrimitiveComponent Object Reference") (OtherActor :type "Actor Object Reference") (OtherComp :type "PrimitiveComponent Object Reference") (NormalImpulse :type "Vector Structure") (Hit :type "HitResult Structure (by ref)"))
  (bind _asbp_player_rock (cast `/Game/Blueprint/Player/BP_PlayerRock` OtherActor))
  (set `self.playerref` _asbp_player_rock)
  (`|ExecutionSequence`
    (:`then_0`
      (goto _label))
    (:`then_1`
      (`/Engine/EditorBlueprintResources/StandardMacros.DoOnce` false :!label _label_3
        (:`Completed`
          (`GameplayStatics.PlaySoundAtLocation` "/Game/Audio/Sounds/SFX/Bell/SC_Bell.SC_Bell" (`SceneComponent.K2_GetComponentLocation` (`self.StaticMesh`)) (struct) 1.0 1.0 0.0 null null null null)
          (`KismetSystemLibrary.Delay` 0.2)
          (goto _label_3 :!via `Reset`))))))

(event `cine`
  (`KismetSystemLibrary.Delay` 1.0)
  (`/Game/Blueprint/Player/BP_PlayerRock.UnlockPlayer` (`/Game/Blueprint/BFL_Rock.GetPlayerActorRef`))
  (`self.SetActorHiddenInGame` (`/Game/Blueprint/BFL_Rock.GetPlayerActorRef`) false))

(fn `UserConstructionScript`
  (bind _hism_moss (`self.HISM_Moss`))
  (bind (_returnvalue_min _returnvalue_max) (break `Box` (`StaticMesh.GetBoundingBox` (`StaticMeshComponent.StaticMesh` (`self.StaticMesh`)))))
  (bind _returnvalue (* (`KismetMathLibrary.RandomUnitVectorFromStream` (`self.s`)) (`self.r`)))
  (bind (_returnvalue_roll _returnvalue_pitch _returnvalue_yaw) (`KismetMathLibrary.BreakRotator` (`KismetMathLibrary.MakeRotFromZ` (- _returnvalue (0.0 0.0 0.0)))))
  (bind _returnvalue_x (`KismetMathLibrary.BreakVector` (* (- _returnvalue_max _returnvalue_min) (`self.HISM_Moss_radmult`))))
  (`InstancedStaticMeshComponent.ClearInstances` (`self.HISM_Moss`))
  (for _ (range (+ (`self.MousseHISM`) 1))
    (set `self.r` _returnvalue_x)
    (`InstancedStaticMeshComponent.AddInstance` _hism_moss (`KismetMathLibrary.MakeTransform` _returnvalue (`KismetMathLibrary.MakeRotator` _returnvalue_roll _returnvalue_pitch _returnvalue_yaw) (* (1.0 1.0 1.0) (`self.hismMossScale`))) false)
    (`SceneComponent.K2_AttachToComponent` _hism_moss (`self.StaticMesh`) "None" "SnapToTarget" "SnapToTarget" "SnapToTarget" true)))