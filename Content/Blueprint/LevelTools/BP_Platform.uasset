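; Level-building platform actor that sets its mesh and, when SpawnProcMesh is on, procedurally decorates it with bells and rope in the Construction Script.
; It reads the mesh's first section and uses a seeded, weighted random test to pick vertices, placing HISM bells offset horizontally along their normals.
; Those positions also rebuild a spline, along which HISM rope segments repeat at slightly overlapping mesh-length intervals.
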(fn `UserConstructionScript`
  (bind _spline (`self.Spline`))
  (bind (_returnvalue_min _returnvalue_max) (break `Box` (`StaticMesh.GetBoundingBox` (`self.RopeMesh`))))
  (bind (_returnvalue_min_2 _returnvalue_max_2) (break `Box` (`StaticMesh.GetBoundingBox` (`self.RopeMesh`))))
  (bind _returnvalue_x (`KismetMathLibrary.BreakVector` (- _returnvalue_max _returnvalue_min)))
  (bind _returnvalue_x_2 (`KismetMathLibrary.BreakVector` (- _returnvalue_max_2 _returnvalue_min_2)))
  (bind _returnvalue (* (`self.SplineMeshIndex`) (- _returnvalue_x 5.0)))
  (`KismetMathLibrary.SetRandomStreamSeed` (`self.Random Stream`) (`self.New Seed`))
  (`StaticMeshComponent.SetStaticMesh` (`self.StaticMesh`) (`self.PlatformMesh`))
  (if (`self.SpawnProcMesh?`)
    (`InstancedStaticMeshComponent.ClearInstances` (`self.HISM_Bell`))
    (`InstancedStaticMeshComponent.ClearInstances` (`self.HISM_Rope`))
    (`SplineComponent.ClearSplinePoints` (`self.Spline`) true)
    (bind (_vertices _triangles _normals) (`KismetProceduralMeshLibrary.GetSectionFromStaticMesh` (`StaticMeshComponent.StaticMesh` (`self.StaticMesh`))))
    (for (_array_element _array_index) _vertices
      (if (`KismetMathLibrary.RandomBoolWithWeightFromStream` (`self.Random Stream`) (`self.SpawnWeight`))
        (bind _returnvalue_2 (`KismetMathLibrary.Normal` (`|GetArrayItem` _normals _array_index)))
        (bind (_returnvalue_x_3 _returnvalue_y) (`KismetMathLibrary.BreakVector` (+ _array_element (* _returnvalue_2 (`self.DistanceToVertice`)))))
        (bind _z (.z _array_element))
        (`InstancedStaticMeshComponent.AddInstance` (`self.HISM_Bell`) (`KismetMathLibrary.MakeTransform` (`KismetMathLibrary.MakeVector` _returnvalue_x_3 _returnvalue_y _z) (`KismetMathLibrary.Conv_VectorToRotator` _returnvalue_2) (0.25 0.25 0.25)) false)
        (`SplineComponent.AddSplinePoint` (`self.Spline`) (`KismetMathLibrary.MakeVector` _returnvalue_x_3 _returnvalue_y _z) "Local" true)))
    (for _index (range (+ (`KismetMathLibrary.FTrunc` (/ (`SplineComponent.GetSplineLength` (`self.Spline`)) (- _returnvalue_x_2 5.0))) 1))
      (set `self.SplineMeshIndex` _index)
      (`InstancedStaticMeshComponent.AddInstance` (`self.HISM_Rope`) (`KismetMathLibrary.MakeTransform` (`SplineComponent.GetLocationAtDistanceAlongSpline` _spline _returnvalue "Local") (`SplineComponent.GetRotationAtDistanceAlongSpline` _spline _returnvalue "Local")) false))))