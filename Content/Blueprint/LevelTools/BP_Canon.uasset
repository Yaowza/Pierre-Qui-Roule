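; Level-tool cannon actor that captures the rock player on trigger overlap, with optional lid, swinging barrel and automatic firing.
; Entry locks the player, blends to the cannon camera and snaps the body to a socket on a looping timer, unless a boss reference is valid.
; Interaction or AutoShoot triggers Shoot's sound, rumble and shake, then a delayed lid reopen and re-arm; the impulse launch logic is unconnected.
; Timelines drive lid and ping-pong swing.
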(event `CloseClappet`
  (`TimelineComponent.SetPlayRate` (`self.Clappet`) (/ 1.0 0.5))
  (bind (_direction _newtrack_0) (`Timeline|Clappet` :!via `PlayFromStart` :!label _label)
    (:`Update`
      (`SceneComponent.K2_SetRelativeRotation` (`self.CanonLid`) (`KismetMathLibrary.MakeRotator` (`KismetMathLibrary.Lerp` 140.0 0.0 _newtrack_0)) false false))))

(event `OpentClappet`
  (`TimelineComponent.SetPlayRate` (`self.Clappet`) (/ 1.0 0.5))
  (goto _label :!via `Reverse`))

(event `self.ReceiveBeginPlay`
  (bind _swingangle (`self.SwingAngle`))
  (bind (_relativerotation_roll _relativerotation_pitch _relativerotation_yaw) (`KismetMathLibrary.BreakRotator` (`SceneComponent.RelativeRotation` (`self.CanonSocket`))))
  (if (`self.Swing?`)
    (set `self.StartXRot` _relativerotation_roll)
    (set `self.StartZRot` _relativerotation_yaw)
    (set `self.RightTarget` (+ _relativerotation_pitch _swingangle))
    (set `self.LeftTarget` (- _relativerotation_pitch _swingangle))
    (`SceneComponent.K2_SetRelativeRotation` (`self.CanonSocket`) (`KismetMathLibrary.MakeRotator` (`self.StartXRot`) (`self.RightTarget`) (`self.StartZRot`)) false false)
    (`self.RotateCanon`)))

(event `RotateCanon`
  (bind _returnvalue (* (/ (`self.SwingAngle`) 2.0) -1.0))
  (`/Engine/EditorBlueprintResources/StandardMacros.FlipFlop`
    (:`A`
      (set `self.SwingRight?` false))
    (:`B`
      (set `self.SwingRight?` true)))
  (`TimelineComponent.SetPlayRate` (`self.SwingTimling`) (/ 1.0 (`self.SwingSpeed`)))
  (`SceneComponent.K2_SetRelativeRotation` (`self.CanonSocket`) (`KismetMathLibrary.MakeRotator` 0.0 _returnvalue) false false)
  (set `self.Relative Rotation Y (Pitch)` _returnvalue)
  (set `self.RL` true :!label _label_2)
  (bind (_direction _newtrack_0) (`Timeline|SwingTimling` :!via `PlayFromStart` :!label _label_3)
    (:`Update`
      (`SceneComponent.K2_SetRelativeRotation` (`self.CanonSocket`) (`KismetMathLibrary.MakeRotator` 0.0 (`KismetMathLibrary.Lerp` (`self.Relative Rotation Y (Pitch)`) (/ (`self.SwingAngle`) 2.0) _newtrack_0)) false false))
    (:`Finished`
      (`KismetSystemLibrary.Delay` (`self.DelayBeforeNextSwing`))
      (if (`self.RL`)
        (set `self.RL` false)
        (goto _label_3 :!via `Reverse`)
        (else
          (goto _label_2))))))

(event `Shoot`
  (bind _asbp_player_rock (`/Game/Blueprint/BFL_Rock.GetPlayerActorRef`))
  (bind _movingcomponent (`/Game/Blueprint/BFL_Rock.GetPhysicPlayerRef`))
  (bind _shootsocket (`self.ShootSocket`))
  (bind _boss (`self.BOSS`))
  (`|ExecutionSequence`
    (:`then_0`
      (`GameplayStatics.PlaySound2D` "/Game/Audio/Sounds/SFX/Canon/SC_CanonShoot.SC_CanonShoot" 1.0 1.0 0.0 null null)
      (`PlayerController.PlayDynamicForceFeedback` (`GameplayStatics.GetPlayerController` 0) (`KismetMathLibrary.Lerp` 0.8 0.0 (stale _newtrack_0)) 0.6 true true true true))
    (:`then_1`
      (`KismetSystemLibrary.Delay` 4.0)
      (`self.OpentClappet`)
      (goto _label_4 :!via `Reset`))
    (:`then_2`
      (bind (_direction _newtrack_0) (`Timeline|shake` :!via `PlayFromStart`)))))

(event `self.TrigerBox.OnComponentBeginOverlap`
  (params (OverlappedComponent :type "PrimitiveComponent Object Reference") (OtherActor :type "Actor Object Reference") (OtherComp :type "PrimitiveComponent Object Reference") (OtherBodyIndex :type Integer) (bFromSweep :type Boolean) (SweepResult :type "HitResult Structure (by ref)"))
  (bind _asbp_player_rock (`/Game/Blueprint/BFL_Rock.GetPlayerActorRef`))
  (bind _movingcomponent (`/Game/Blueprint/BFL_Rock.GetPhysicPlayerRef`))
  (bind _shootsocket (`self.ShootSocket`))
  (bind _boss (`self.BOSS`))
  (bind _asbp_player_rock_2 (cast `/Game/Blueprint/Player/BP_PlayerRock` OtherActor))
  (`/Engine/EditorBlueprintResources/StandardMacros.DoOnce` false :!label _label_4
    (:`Completed`
      (`self.EnableInput` (`/Game/Blueprint/BFL_Rock.GetPlayerActorRef`) (`GameplayStatics.GetPlayerController` 0))
      (`self.CloseClappet`)
      (`GameplayStatics.PlaySound2D` "/Game/Audio/Sounds/SFX/Canon/SC_CanonEnter.SC_CanonEnter" 1.0 1.0 0.0 null null)
      (`/Engine/EditorBlueprintResources/StandardMacros.IsValid` _boss
        (:`Is Valid`
          (`/Game/Blueprint/IA/BP_IARock.Ignoreplayer` _boss true))
        (:`Is Not Valid`
          (`/Game/Blueprint/Player/BP_PlayerRock.Cancel Down Dash` _asbp_player_rock_2)
          (`/Game/Blueprint/Player/BP_PlayerRock.LockPlayer` (`/Game/Blueprint/BFL_Rock.GetPlayerActorRef`))
          (`PlayerController.SetViewTargetWithBlend` (`GameplayStatics.GetPlayerController` 0) self 0.2 "VTBlend_Linear" (`self.BlendSpeed`) true)
          (`/Game/Blueprint/Player/BP_PlayerRock.SetCurrentCameraUsed` (`/Game/Blueprint/BFL_Rock.GetPlayerActorRef`) (`self.Camera`))
          (`self.SetActorHiddenInGame` (`/Game/Blueprint/BFL_Rock.GetPlayerActorRef`) false)
          (if (`self.Custom Rota Shoot`)
            (`SceneComponent.K2_SetWorldLocationAndRotation` _movingcomponent (`SceneComponent.K2_GetComponentLocation` _shootsocket) (`SceneComponent.K2_GetComponentRotation` (`self.CustomRotaSocket`)) false false)
            (`/Game/Blueprint/Player/BP_PlayerRock.ResetCameraRotation_CanonCustom` _asbp_player_rock)
            (else
              (`SceneComponent.K2_SetWorldLocationAndRotation` _movingcomponent (`SceneComponent.K2_GetComponentLocation` _shootsocket) (`SceneComponent.K2_GetComponentRotation` _shootsocket) false false)
              (`/Game/Blueprint/Player/BP_PlayerRock.ResetCameraRotation_Death` _asbp_player_rock)))
          (bind _returnvalue (`KismetSystemLibrary.K2_SetTimerDelegate` (delegate `SnapPlayer`) 0.01 true true))
          (if (`self.AutoShoot?`)
            (`KismetSystemLibrary.Delay` 1.0)
            (`self.Shoot`)))))))

(event `ClearSnapPlayer`
  (`KismetSystemLibrary.K2_ClearAndInvalidateTimerHandle` (stale `self.TrigerBox.OnComponentBeginOverlap` _returnvalue)))

(event `SnapPlayer`
  (bind _rocksocket (`self.RockSocket`))
  (`SceneComponent.K2_SetWorldLocationAndRotation` (`/Game/Blueprint/BFL_Rock.GetPhysicPlayerRef`) (`SceneComponent.K2_GetComponentLocation` _rocksocket) (`SceneComponent.K2_GetComponentRotation` _rocksocket) false false)
  (if (and (`/Game/Blueprint/Player/BP_PlayerRock.GetInteracted?` (`/Game/Blueprint/BFL_Rock.GetPlayerActorRef`)) (not (`self.AutoShoot?`)))
    (`self.Shoot`)))

(event `self.TrigerBox.OnComponentEndOverlap`
  (params (OverlappedComponent :type "PrimitiveComponent Object Reference") (OtherActor :type "Actor Object Reference") (OtherComp :type "PrimitiveComponent Object Reference") (OtherBodyIndex :type Integer))
  (cast `/Game/Blueprint/Player/BP_PlayerRock` OtherActor))

(fn `SwingCanon`
  (bind _returnvalue (`KismetMathLibrary.SelectFloat` (`self.RightTarget`) (`self.LeftTarget`) (`self.SwingRight?`)))
  (bind (_relativerotation_roll _relativerotation_pitch) (`KismetMathLibrary.BreakRotator` (`SceneComponent.RelativeRotation` (`self.CanonSocket`))))
  (`SceneComponent.K2_SetRelativeRotation` (`self.CanonSocket`) (`KismetMathLibrary.MakeRotator` (`self.StartXRot`) (`KismetMathLibrary.FInterpTo_Constant` _relativerotation_pitch _returnvalue (`GameplayStatics.GetWorldDeltaSeconds`) (`self.SwingSpeed`)) (`self.StartZRot`)) false false)
  (`KismetSystemLibrary.PrintString` (`KismetStringLibrary.Conv_DoubleToString` _returnvalue) true false (struct :`G` 0.66 :`B` 1.0 :`A` 1.0) 0.0))

(fn `UserConstructionScript`
  (`|ExecutionSequence`
    (:`then_0`
      (if (`self.Swing?`)
        (`SceneComponent.SetVisibility` (`self.CanonA`) true false)
        (`SceneComponent.SetVisibility` (`self.CanonB`) false false)
        (else
          (`SceneComponent.SetVisibility` (`self.CanonA`) false false)
          (`SceneComponent.SetVisibility` (`self.CanonB`) true false))))
    (:`then_1`
      (if (`self.WithDoor?`)
        (`SceneComponent.SetVisibility` (`self.CanonLid`) true false)
        (else
          (`SceneComponent.SetVisibility` (`self.CanonLid`) false false))))))