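; BP_MiniCineTriggerrerRAIL is a level trigger that plays a one-time mini cinematic with a camera riding a spline rail.
; When BP_PlayerRock enters the Box, it locks the player, blends the view to its own Camera and plays the CamRailing timeline, rate-scaled by SequenceLength.
; The timeline drives spline position, smoothed with VInterpTo, and rotation follows the spline.
; On finish, it blends back to the third-person camera, then unlocks the player.
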(event `self.Box.OnComponentBeginOverlap`
  (params (OverlappedComponent :type "PrimitiveComponent Object Reference") (OtherActor :type "Actor Object Reference") (OtherComp :type "PrimitiveComponent Object Reference") (OtherBodyIndex :type Integer) (bFromSweep :type Boolean) (SweepResult :type "HitResult Structure (by ref)"))
  (bind _asbp_player_rock (`/Game/Blueprint/BFL_Rock.GetPlayerActorRef`))
  (bind _asbp_player_rock_2 (`/Game/Blueprint/BFL_Rock.GetPlayerActorRef`))
  (bind _spline (`self.Spline`))
  (bind _camblendspeed_out (`self.CamBlendSpeed_Out`))
  (cast `/Game/Blueprint/Player/BP_PlayerRock` OtherActor)
  (`/Engine/EditorBlueprintResources/StandardMacros.DoOnce` false
    (:`Completed`
      (`/Game/Blueprint/Player/BP_PlayerRock.LockPlayer` _asbp_player_rock)
      (`PlayerController.SetViewTargetWithBlend` (`GameplayStatics.GetPlayerController` 0) self (`self.CamBlendSpeed_In`) "VTBlend_Linear" 0.0 false)
      (`/Game/Blueprint/Player/BP_PlayerRock.SetCurrentCameraUsed` _asbp_player_rock (`self.Camera`))
      (`TimelineComponent.SetPlayRate` (`self.CamRailing`) (/ 1.0 (`self.SequenceLength`)))
      (bind (_direction _newtrack_0) (`Timeline|CamRailing` :!via `PlayFromStart`)
        (:`Update`
          (bind _returnvalue (`SplineComponent.GetLocationAtTime` (`self.Spline`) _newtrack_0 "World" false))
          (`SceneComponent.K2_SetWorldLocationAndRotation` (`self.Camera`) (`KismetMathLibrary.VInterpTo` (`SceneComponent.K2_GetComponentLocation` (`self.Camera`)) _returnvalue (`GameplayStatics.GetWorldDeltaSeconds`) 5.0) (`SplineComponent.GetRotationAtDistanceAlongSpline` _spline (`SplineComponent.GetDistanceAlongSplineAtLocation` _spline _returnvalue "World") "World") false false))
        (:`Finished`
          (`PlayerController.SetViewTargetWithBlend` (`GameplayStatics.GetPlayerController` 0) (`/Game/Blueprint/BFL_Rock.GetPlayerActorRef`) _camblendspeed_out "VTBlend_Linear" 0.0 false)
          (`/Game/Blueprint/Player/BP_PlayerRock.SetCurrentCameraUsed` _asbp_player_rock_2 (`/Game/Blueprint/Player/BP_PlayerRock.ThirdPersonCamera` _asbp_player_rock_2))
          (`KismetSystemLibrary.Delay` _camblendspeed_out)
          (`/Game/Blueprint/Player/BP_PlayerRock.UnlockPlayer` (`/Game/Blueprint/BFL_Rock.GetPlayerActorRef`)))))))

(event `self.Trigger01`)

(event `EndMini ciné`)

(event `self.Shazam`)

(fn `UserConstructionScript`)