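; Boss-section camera rail that takes over the player's view with a spline-following camera and switches music when Boss is set.
; Start triggers toggle the rail camera and move a spline point to the player; end triggers restore third-person view.
; While active, Tick eases the camera along the spline toward the player camera, optionally aiming at the rock.
; Optional flags cap player speed or autoroll it toward an arrow via timed force.
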(event `MusicTransition`
  (bind _soundmanagerref (`self.SoundManagerRef`))
  (`/Game/Blueprint/BP_SoundManager.ChangeMusic` _soundmanagerref (`/Game/Blueprint/BP_SoundManager.SC_WindLoop_VarB` _soundmanagerref)))

(event `MusicBoss`
  (bind _soundmanagerref (`self.SoundManagerRef`))
  (`/Game/Blueprint/BP_SoundManager.ChangeMusic` _soundmanagerref (`/Game/Blueprint/BP_SoundManager.SC_BossMusic` _soundmanagerref))
  (`KismetSystemLibrary.PrintString` "MUSIC BOSS" true false (struct :`R` 0.756335 :`B` 1.0 :`A` 1.0) 10.0))

(event `self.Box1.OnComponentBeginOverlap`
  (params (OverlappedComponent :type "PrimitiveComponent Object Reference") (OtherActor :type "Actor Object Reference") (OtherComp :type "PrimitiveComponent Object Reference") (OtherBodyIndex :type Integer) (bFromSweep :type Boolean) (SweepResult :type "HitResult Structure (by ref)"))
  (bind _asbp_player_rock (`/Game/Blueprint/BFL_Rock.GetPlayerActorRef`))
  (bind _asbp_player_rock_2 (`/Game/Blueprint/BFL_Rock.GetPlayerActorRef`))
  (bind _asbp_player_rock_3 (cast `/Game/Blueprint/Player/BP_PlayerRock` OtherActor))
  (if (`self.Boss?`) :!label _label
    (`self.MusicTransition`))
  (if (`self.cam`)
    (`PlayerController.SetViewTargetWithBlend` (`GameplayStatics.GetPlayerController` 0) _asbp_player_rock 1.0 "VTBlend_Linear" 0.0 true :!label _label_2)
    (set `self.cam` false)
    (`/Game/Blueprint/Player/BP_PlayerRock.ResetCameraRotation_Canon` _asbp_player_rock)
    (`/Game/Blueprint/Player/BP_PlayerRock.SetCurrentCameraUsed` _asbp_player_rock_2 (`/Game/Blueprint/Player/BP_PlayerRock.ThirdPersonCamera` _asbp_player_rock_2))
    (`|ExecutionSequence`
      (:`then_0`
        (if (`self.SlowChara`)
          (set `/Game/Blueprint/Player/BP_PlayerRock.MaxVelocity` 2500.0 (`/Game/Blueprint/BFL_Rock.GetPlayerActorRef`))))
      (:`then_1`
        (if (`self.Autoroll`)
          (`KismetSystemLibrary.K2_ClearAndInvalidateTimerHandle` (stale _returnvalue_2)))))
    (else
      (bind _returnvalue (`SceneComponent.K2_GetComponentLocation` (`/Game/Blueprint/Player/BP_PlayerRock.GetMovingComponent` _asbp_player_rock_3)))
      (`SceneComponent.K2_SetWorldLocation` (`self.Camera`) _returnvalue false false)
      (`SplineComponent.SetLocationAtSplinePoint` (`self.Spline`) 0 _returnvalue "World" true)
      (`PlayerController.SetViewTargetWithBlend` (`GameplayStatics.GetPlayerController` 0) self 1.0 "VTBlend_Linear" 0.0 true)
      (set `self.cam` true)
      (`/Game/Blueprint/Player/BP_PlayerRock.SetCurrentCameraUsed` (`/Game/Blueprint/BFL_Rock.GetPlayerActorRef`) (`self.Camera`))
      (`|ExecutionSequence`
        (:`then_0`
          (if (`self.SlowChara`)
            (set `/Game/Blueprint/Player/BP_PlayerRock.MaxVelocity` 1400.0 (`/Game/Blueprint/BFL_Rock.GetPlayerActorRef`))))
        (:`then_1`
          (if (`self.Autoroll`)
            (bind _returnvalue_2 (`KismetSystemLibrary.K2_SetTimerDelegate` (delegate `Roll`) 0.02 true true))))))))

(event `self.StartTrigerBox.OnComponentBeginOverlap`
  (params (OverlappedComponent :type "PrimitiveComponent Object Reference") (OtherActor :type "Actor Object Reference") (OtherComp :type "PrimitiveComponent Object Reference") (OtherBodyIndex :type Integer) (bFromSweep :type Boolean) (SweepResult :type "HitResult Structure (by ref)"))
  (cast `/Game/Blueprint/Player/BP_PlayerRock` OtherActor)
  (goto _label))

(event `Roll`
  (bind _movingcomponent (`/Game/Blueprint/Player/BP_PlayerRock.GetMovingComponent` (`/Game/Blueprint/BFL_Rock.GetPlayerActorRef`)))
  (`PrimitiveComponent.AddForce` _movingcomponent (* (`KismetMathLibrary.GetDirectionUnitVector` (`SceneComponent.K2_GetComponentLocation` _movingcomponent) (`SceneComponent.K2_GetComponentLocation` (`self.Arrow`))) 500000.0) "None" false))

(event `self.EndTrigerBox.OnComponentBeginOverlap`
  (params (OverlappedComponent :type "PrimitiveComponent Object Reference") (OtherActor :type "Actor Object Reference") (OtherComp :type "PrimitiveComponent Object Reference") (OtherBodyIndex :type Integer) (bFromSweep :type Boolean) (SweepResult :type "HitResult Structure (by ref)"))
  (cast `/Game/Blueprint/Player/BP_PlayerRock` OtherActor)
  (if (`self.Boss?`) :!label _label_3
    (`self.MusicBoss`))
  (if (`self.cam`)
    (goto _label_2)))

(event `self.Box.OnComponentBeginOverlap`
  (params (OverlappedComponent :type "PrimitiveComponent Object Reference") (OtherActor :type "Actor Object Reference") (OtherComp :type "PrimitiveComponent Object Reference") (OtherBodyIndex :type Integer) (bFromSweep :type Boolean) (SweepResult :type "HitResult Structure (by ref)"))
  (cast `/Game/Blueprint/Player/BP_PlayerRock` OtherActor)
  (goto _label_3))

(event `self.ReceiveBeginPlay`
  (bind _camera (`self.Camera`))
  (set `self.BaseLoc` (`SceneComponent.K2_GetComponentLocation` _camera))
  (set `self.BaseRot` (`SceneComponent.K2_GetComponentRotation` _camera))
  (bind _returnvalue (`GameplayStatics.GetActorOfClass` "/Game/Blueprint/BP_SoundManager.BP_SoundManager_C"))
  (set `self.SoundManagerRef` _returnvalue))

(event `self.ReceiveTick`
  (params (DeltaSeconds :type "Float (single-precision)"))
  (bind _camera (`self.Camera`))
  (bind _returnvalue (`KismetMathLibrary.VInterpTo` (`SceneComponent.K2_GetComponentLocation` (`self.Camera`)) (`SplineComponent.FindLocationClosestToWorldLocation` (`self.Spline`) (`SceneComponent.K2_GetComponentLocation` (`/Game/Blueprint/Player/BP_PlayerRock.ThirdPersonCamera` (`/Game/Blueprint/BFL_Rock.GetPlayerActorRef`))) "World") (`GameplayStatics.GetWorldDeltaSeconds`) 5.0))
  (if (`self.cam`)
    (`|ExecutionSequence`
      (:`then_0`
        (if (`self.LookAtPlayer?`)
          (`SceneComponent.K2_SetWorldLocationAndRotation` _camera _returnvalue (`KismetMathLibrary.FindLookAtRotation` (`SceneComponent.K2_GetComponentLocation` (`self.Camera`)) (`SceneComponent.K2_GetComponentLocation` (`/Game/Blueprint/BFL_Rock.GetPhysicPlayerRef`))) false false)
          (else
            (`SceneComponent.K2_SetWorldLocation` _camera _returnvalue false false)))
        (`/Game/Blueprint/Player/BP_PlayerRock.ResetCameraRotation_Canon` (`/Game/Blueprint/BFL_Rock.GetPlayerActorRef`))))))

(event `ResetCameraSnap`
  (bind _asbp_player_rock (`/Game/Blueprint/BFL_Rock.GetPlayerActorRef`))
  (bind _asbp_player_rock_2 (`/Game/Blueprint/BFL_Rock.GetPlayerActorRef`))
  (`PlayerController.SetViewTargetWithBlend` (`GameplayStatics.GetPlayerController` 0) _asbp_player_rock_2 1.0 "VTBlend_Linear" 0.0 true)
  (set `self.cam` false)
  (`/Game/Blueprint/Player/BP_PlayerRock.ResetCameraRotation_Canon` _asbp_player_rock_2)
  (`SceneComponent.K2_SetWorldLocationAndRotation` (`self.Camera`) (`self.BaseLoc`) (`self.BaseRot`) false false)
  (`/Game/Blueprint/Player/BP_PlayerRock.SetCurrentCameraUsed` _asbp_player_rock (`/Game/Blueprint/Player/BP_PlayerRock.ThirdPersonCamera` _asbp_player_rock)))

(fn `UserConstructionScript`)