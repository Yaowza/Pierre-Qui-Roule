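; BP_ChampiLoup is an interactable mushroom prop that squishes when a player or AI rock overlaps its sphere.
; Overlap plays the Squish sequence, with a once-gated Niagara burst and attenuated sound; only the player rock triggers controller rumble.
; When a rock leaves, a 15-second delay precedes the UnSquish sequence and re-arms the gate.
; The construction script applies the configurable mesh and effect asset.
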(event `self.Sphere.OnComponentBeginOverlap`
  (params (OverlappedComponent :type "PrimitiveComponent Object Reference") (OtherActor :type "Actor Object Reference") (OtherComp :type "PrimitiveComponent Object Reference") (OtherBodyIndex :type Integer) (bFromSweep :type Boolean) (SweepResult :type "HitResult Structure (by ref)"))
  (cast `/Game/Blueprint/Player/BP_PlayerRock` OtherActor
    (:`then`
      (`|ExecutionSequence`
        (:`then_0`
          (`PlayerController.PlayDynamicForceFeedback` (`GameplayStatics.GetPlayerController` 0) 0.2 0.6 true true true true))
        (:`then_1`
          (`MovieSceneSequencePlayer.Play` (`ActorSequenceComponent.SequencePlayer` (`self.Squish`)) :!label _label)
          (`|ExecutionSequence`
            (:`then_0`
              (`/Engine/EditorBlueprintResources/StandardMacros.DoOnce` false :!label _label_2
                (:`Completed`
                  (`ActorComponent.Activate` (`self.NS_MiniChampiSquish`) true)
                  (`GameplayStatics.PlaySoundAtLocation` (`self.Sound`) (`self.K2_GetActorLocation`) (struct) 0.6 1.0 0.0 "/Game/Audio/Sounds/SA_Moss.SA_Moss" null null null))))))))
    (:`CastFailed`
      (cast `/Game/Blueprint/IA/BP_IARock` OtherActor)
      (goto _label))))

(event `self.Sphere.OnComponentEndOverlap`
  (params (OverlappedComponent :type "PrimitiveComponent Object Reference") (OtherActor :type "Actor Object Reference") (OtherComp :type "PrimitiveComponent Object Reference") (OtherBodyIndex :type Integer))
  (cast `/Game/Blueprint/Player/BP_PlayerRock` OtherActor
    (:`then`
      _)
    (:`CastFailed`
      (cast `/Game/Blueprint/IA/BP_IARock` OtherActor)))
  (`KismetSystemLibrary.Delay` 15.0)
  (`MovieSceneSequencePlayer.Play` (`ActorSequenceComponent.SequencePlayer` (`self.UnSquish`)))
  (goto _label_2 :!via `Reset`))

(fn `UserConstructionScript`
  (`StaticMeshComponent.SetStaticMesh` (`self.Champi`) (`self.ChampiVAR`))
  (`NiagaraComponent.SetAsset` (`self.NS_MiniChampiSquish`) (`self.FX_Champi`) true))