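; Bouncy mushroom interactable that knocks player and AI rocks away when they overlap its sphere.
; The radial impulse, with an added upward kick, scales with player rock speed or uses a set velocity for AI rocks.
; Each bounce plays bump sequences chosen by speed, squish FX, sound and rumble, plus an optional timeline-driven emissive flash that slowly fades.
; The construction script applies the configurable mesh and FX and creates the dynamic material.
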(event `self.Sphere.OnComponentBeginOverlap`
  (params (OverlappedComponent :type "PrimitiveComponent Object Reference") (OtherActor :type "Actor Object Reference") (OtherComp :type "PrimitiveComponent Object Reference") (OtherBodyIndex :type Integer) (bFromSweep :type Boolean) (SweepResult :type "HitResult Structure (by ref)"))
  (bind _sequenceplayer (`ActorSequenceComponent.SequencePlayer` (`self.MidChampiBump_MID`)))
  (bind _sequenceplayer_2 (`ActorSequenceComponent.SequencePlayer` (`self.MidChampiBump_Strong`)))
  (bind _sequenceplayer_3 (`ActorSequenceComponent.SequencePlayer` (`self.MidChampiBump_Weak2`)))
  (bind _sequenceplayer_4 (`ActorSequenceComponent.SequencePlayer` (`self.MidChampiBump_MID`)))
  (bind _asbp_player_rock (cast `/Game/Blueprint/Player/BP_PlayerRock` OtherActor)
    (:`then`
      (`|ExecutionSequence`
        (:`then_0`
          (bind _speedrock (`/Game/Blueprint/Player/BP_PlayerRock.SpeedRock` _asbp_player_rock))
          (if (<= _speedrock 1000.0)
            (`MovieSceneSequencePlayer.Stop` _sequenceplayer_3)
            (`MovieSceneSequencePlayer.Play` _sequenceplayer_3)))
        (:`then_1`
          (if (<= _speedrock 1900.0)
            (`MovieSceneSequencePlayer.Stop` _sequenceplayer)
            (`MovieSceneSequencePlayer.Play` _sequenceplayer)
            (else
              (`MovieSceneSequencePlayer.Stop` _sequenceplayer_2)
              (`MovieSceneSequencePlayer.Play` _sequenceplayer_2))))
        (:`then_2`
          (bind _spherecollision (`/Game/Blueprint/Player/BP_PlayerRock.SphereCollision` _asbp_player_rock))
          (`PrimitiveComponent.AddImpulse` _spherecollision (+ (* (`KismetMathLibrary.Normal` (`KismetMathLibrary.GetDirectionUnitVector` (`self.K2_GetActorLocation`) (`SceneComponent.K2_GetComponentLocation` _spherecollision))) (`KismetMathLibrary.MapRangeClamped` (`/Game/Blueprint/Player/BP_PlayerRock.SpeedRock` _asbp_player_rock) 1.0 2400.0 450.0 2100.0)) (0.0 0.0 300.0)) "None" true)
          (`ActorComponent.Activate` (`self.NS_MiniChampiSquish`) true :!label _label)
          (`PlayerController.PlayDynamicForceFeedback` (`GameplayStatics.GetPlayerController` 0) 0.3 0.2 true true true true)
          (`GameplayStatics.PlaySoundAtLocation` (`self.Sound`) (`self.K2_GetActorLocation`) (struct) 0.6 1.0 0.0 "/Game/Audio/Sounds/SA_Moss.SA_Moss" null null null)
          (if (`self.Lumi?`)
            (if (`self.Glowing`)
              (`TimelineComponent.SetPlayRate` (`self.Glowin`) (/ 1.0 5.0) :!label _label_2)
              (bind (_direction _newtrack_0) (`Timeline|Glowin` :!via `PlayFromStart`)
                (:`Update`
                  (`MaterialInstanceDynamic.SetScalarParameterValue` (`self.MAterial`) "EmissMult" (`KismetMathLibrary.Lerp` 10.0 1.0 _newtrack_0))
                  (set `self.Glowing` true))
                (:`Finished`
                  (set `self.Glowing` false)))
              (else
                (`TimelineComponent.SetPlayRate` (`self.glowi`) (/ 1.0 0.1))
                (bind (_direction_2 _newtrack_0_2) (`Timeline|glowi` :!via `PlayFromStart`)
                  (:`Update`
                    (`MaterialInstanceDynamic.SetScalarParameterValue` (`self.MAterial`) "EmissMult" (`KismetMathLibrary.Lerp` 1.0 10.0 _newtrack_0_2)))
                  (:`Finished`
                    (goto _label_2)))))))))
    (:`CastFailed`
      (bind _asbp_iarock (cast `/Game/Blueprint/IA/BP_IARock` OtherActor))
      (`MovieSceneSequencePlayer.Stop` _sequenceplayer_4)
      (`MovieSceneSequencePlayer.Play` _sequenceplayer_4)
      (bind _collisionshape (`/Game/Blueprint/IA/BP_IARock.CollisionShape` _asbp_iarock))
      (`PrimitiveComponent.AddImpulse` _collisionshape (+ (* (`KismetMathLibrary.Normal` (`KismetMathLibrary.GetDirectionUnitVector` (`self.K2_GetActorLocation`) (`SceneComponent.K2_GetComponentLocation` _collisionshape))) (`self.InVEL`)) (0.0 0.0 300.0)) "None" true)
      (goto _label))))

(fn `UserConstructionScript`
  (bind _champignon (`self.champignon`))
  (`StaticMeshComponent.SetStaticMesh` (`self.champignon`) (`self.ChampiVAR`))
  (`NiagaraComponent.SetAsset` (`self.NS_MiniChampiSquish`) (`self.FX_Champi`) true)
  (bind _returnvalue (`PrimitiveComponent.CreateDynamicMaterialInstance` _champignon 0 (`PrimitiveComponent.GetMaterial` _champignon 0) "None"))
  (set `self.MAterial` _returnvalue)
  (`PrimitiveComponent.SetMaterial` _champignon 0 _returnvalue))