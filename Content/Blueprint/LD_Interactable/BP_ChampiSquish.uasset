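; Interactable mushroom that squishes when a player or AI rock overlaps its sphere, with sound, Niagara FX, and controller rumble for the player.
; If Lumi is set, a timeline animates the material's emissive on squish.
; Separate DoOnce/Gate pairs per rock type delay the un-squish until a few seconds after overlap ends, with re-entry closing the gate.
; The construction script applies the configurable mesh and FX and creates the dynamic material.
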(event `self.Sphere.OnComponentBeginOverlap`
  (params (OverlappedComponent :type "PrimitiveComponent Object Reference") (OtherActor :type "Actor Object Reference") (OtherComp :type "PrimitiveComponent Object Reference") (OtherBodyIndex :type Integer) (bFromSweep :type Boolean) (SweepResult :type "HitResult Structure (by ref)"))
  (cast `/Game/Blueprint/Player/BP_PlayerRock` OtherActor
    (:`then`
      (`/Engine/EditorBlueprintResources/StandardMacros.DoOnce` false :!label _label
        (:`Completed`
          (`|ExecutionSequence`
            (:`then_0`
              (`MovieSceneSequencePlayer.Play` (`ActorSequenceComponent.SequencePlayer` (`self.Squish`)) :!label _label_2)
              (`ActorComponent.Activate` (`self.NS_MiniChampiSquish`) true)
              (`GameplayStatics.PlaySoundAtLocation` (`self.Sound`) (`self.K2_GetActorLocation`) (struct) 0.6 1.0 0.0 "/Game/Audio/Sounds/SA_Moss.SA_Moss" null null null)
              (if (`self.Lumi?`)
                (`TimelineComponent.SetPlayRate` (`self.Glow`) (/ 1.0 5.0))
                (bind (_direction _newtrack_0) (`Timeline|Glow` :!via `PlayFromStart`)
                  (:`Update`
                    (`MaterialInstanceDynamic.SetScalarParameterValue` (`self.MAterial`) "EmissMult" (`KismetMathLibrary.Lerp` 10.0 1.0 _newtrack_0))))))
            (:`then_1`
              (`PlayerController.PlayDynamicForceFeedback` (`GameplayStatics.GetPlayerController` 0) 0.3 0.1 true true true true))
            (:`then_2`
              (goto _label_4 :!via `Close`))))))
    (:`CastFailed`
      (cast `/Game/Blueprint/IA/BP_IARock` OtherActor)
      (`/Engine/EditorBlueprintResources/StandardMacros.DoOnce` false :!label _label_3
        (:`Completed`
          (`|ExecutionSequence`
            (:`then_0`
              (goto _label_2))
            (:`then_1`
              (goto _label_5 :!via `Close`))))))))

(event `self.Sphere.OnComponentEndOverlap`
  (params (OverlappedComponent :type "PrimitiveComponent Object Reference") (OtherActor :type "Actor Object Reference") (OtherComp :type "PrimitiveComponent Object Reference") (OtherBodyIndex :type Integer))
  (cast `/Game/Blueprint/Player/BP_PlayerRock` OtherActor
    (:`then`
      (`|ExecutionSequence`
        (:`then_0`
          (goto _label_4 :!via `Open`))
        (:`then_1`
          (`KismetSystemLibrary.RetriggerableDelay` 4.0)
          (`/Engine/EditorBlueprintResources/StandardMacros.Gate` false :!label _label_4
            (:`Exit`
              (`GameplayStatics.PlaySoundAtLocation` "/Game/Audio/Sounds/SFX/MiniCHampi/SC_MiniChampiUp.SC_MiniChampiUp" (`self.K2_GetActorLocation`) (struct) 0.5 1.0 0.0 "/Game/Audio/Sounds/SA_Moss.SA_Moss" null null null)
              (`MovieSceneSequencePlayer.Play` (`ActorSequenceComponent.SequencePlayer` (`self.UnSquish`)))
              (goto _label :!via `Reset`))))))
    (:`CastFailed`
      (cast `/Game/Blueprint/IA/BP_IARock` OtherActor)
      (`|ExecutionSequence`
        (:`then_0`
          (goto _label_5 :!via `Open`))
        (:`then_1`
          (`KismetSystemLibrary.RetriggerableDelay` 4.0)
          (`/Engine/EditorBlueprintResources/StandardMacros.Gate` false :!label _label_5
            (:`Exit`
              (`GameplayStatics.PlaySoundAtLocation` "/Game/Audio/Sounds/SFX/MiniCHampi/SC_MiniChampiUp.SC_MiniChampiUp" (`self.K2_GetActorLocation`) (struct) 0.5 1.0 0.0 "/Game/Audio/Sounds/SA_Moss.SA_Moss" null null null)
              (`MovieSceneSequencePlayer.Play` (`ActorSequenceComponent.SequencePlayer` (`self.UnSquish`)))
              (goto _label_3 :!via `Reset`))))))))

(fn `UserConstructionScript`
  (bind _champi (`self.Champi`))
  (`StaticMeshComponent.SetStaticMesh` (`self.Champi`) (`self.ChampiVAR`))
  (`NiagaraComponent.SetAsset` (`self.NS_MiniChampiSquish`) (`self.FX_Champi`) true)
  (bind _returnvalue (`PrimitiveComponent.CreateDynamicMaterialInstance` _champi 0 (`PrimitiveComponent.GetMaterial` _champi 0) "None"))
  (set `self.MAterial` _returnvalue)
  (`PrimitiveComponent.SetMaterial` _champi 0 _returnvalue))