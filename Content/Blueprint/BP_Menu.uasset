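; BP_Menu is the main and pause menu actor, which also serves as the menu camera.
; On initialization it takes the view target, creates WBP_MainMenu, focuses it and adds the IMC_UI Enhanced Input mapping context.
; Play closes the widget and initializes the player only once.
; Separate events open it as a pause screen that hides the HUD, step back, unpause, and close it with a delayed collapse.
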(event `InitializeCamera`
  (bind _returnvalue (`GameplayStatics.GetPlayerController` 0))
  (`PlayerController.SetViewTargetWithBlend` (`GameplayStatics.GetPlayerController` 0) self 0.0 "VTBlend_Linear" 0.0 true)
  (`/Game/Blueprint/Player/BP_PlayerRock.SetCurrentCameraUsed` (`/Game/Blueprint/BFL_Rock.GetPlayerActorRef`) (`self.CineCamera`))
  (bind _returnvalue_2 (`|CreateWidget` "/Game/UI/WBP/WBP_MainMenu.WBP_MainMenu_C"))
  (`UserWidget.AddToViewport` _returnvalue_2 0)
  (bind _output_get (set `self.WBP_MenuRef` _returnvalue_2))
  (`WidgetBlueprintLibrary.SetInputMode_GameAndUIEx` _returnvalue _output_get)
  (set `PlayerController.bShowMouseCursor` false _returnvalue)
  (`EnhancedInputSubsystemInterface.AddMappingContext` (pcsubsystem `EnhancedInputLocalPlayerSubsystem` (cast `/Game/Blueprint/Player/PC_Rock` (`GameplayStatics.GetPlayerController` 0) :!pure true)) "/Game/Blueprint/Player/Input/IMC_UI.IMC_UI" 1 (struct)))

(event `Play`
  (bind _returnvalue (`GameplayStatics.GetPlayerController` 0))
  (`/Game/UI/WBP/WBP_MainMenu.Close` (`self.WBP_MenuRef`))
  (`WidgetBlueprintLibrary.SetInputMode_GameOnly` _returnvalue)
  (set `PlayerController.bShowMouseCursor` false _returnvalue)
  (`KismetSystemLibrary.Delay` 0.5)
  (`Widget.SetVisibility` (`self.WBP_MenuRef`) "Collapsed")
  (`/Engine/EditorBlueprintResources/StandardMacros.DoOnce` false
    (:`Completed`
      (`/Game/Blueprint/Player/BP_PlayerRock.InitializePlayer` (`/Game/Blueprint/BFL_Rock.GetPlayerActorRef`)))))

(event `Unpause`
  (`EnhancedInputSubsystemInterface.RemoveMappingContext` (pcsubsystem `EnhancedInputLocalPlayerSubsystem` (cast `/Game/Blueprint/Player/PC_Rock` (`GameplayStatics.GetPlayerController` 0) :!pure true)) "/Game/Blueprint/Player/Input/IMC_UI.IMC_UI" (struct))
  (`GameplayStatics.SetGamePaused` false))

(event `OpenWidget`
  (bind _returnvalue (`GameplayStatics.GetPlayerController` 0))
  (bind _wbp_menuref (`self.WBP_MenuRef`))
  (`GameplayStatics.SetGamePaused` true)
  (`EnhancedInputSubsystemInterface.AddMappingContext` (pcsubsystem `EnhancedInputLocalPlayerSubsystem` (cast `/Game/Blueprint/Player/PC_Rock` (`GameplayStatics.GetPlayerController` 0) :!pure true)) "/Game/Blueprint/Player/Input/IMC_UI.IMC_UI" 1 (struct))
  (`WidgetBlueprintLibrary.SetInputMode_GameAndUIEx` _returnvalue (`self.WBP_MenuRef`))
  (`/Game/Blueprint/HUD/PQR_HUD.Set Visibility` (cast `/Game/Blueprint/HUD/PQR_HUD` (`PlayerController.GetHUD` _returnvalue) :!pure true) false)
  (set `PlayerController.bShowMouseCursor` (`/Game/Blueprint/Player/BP_PlayerRock.UseKeyboard?` (`/Game/Blueprint/BFL_Rock.GetPlayerActorRef`)) _returnvalue)
  (`Widget.SetVisibility` _wbp_menuref "Visible")
  (`/Game/UI/WBP/WBP_MainMenu.Open` _wbp_menuref))

(event `Back`
  (`/Game/UI/WBP/WBP_MainMenu.Back` (`self.WBP_MenuRef`)))

(event `CloseWidget`
  (bind _returnvalue (`GameplayStatics.GetPlayerController` 0))
  (bind _wbp_menuref (`self.WBP_MenuRef`))
  (if (`/Game/UI/WBP/WBP_MainMenu.CanClose` _wbp_menuref)
    (`KismetSystemLibrary.PrintString` "Hello")
    (`/Game/UI/WBP/WBP_MainMenu.Close` _wbp_menuref)
    (`WidgetBlueprintLibrary.SetInputMode_GameOnly` _returnvalue)
    (set `PlayerController.bShowMouseCursor` false _returnvalue)
    (`KismetSystemLibrary.Delay` 0.5)
    (`Widget.SetVisibility` (`self.WBP_MenuRef`) "Collapsed")))

(fn `UserConstructionScript`)