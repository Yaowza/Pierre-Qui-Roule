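; Cinematic player rock character: a mossy body with an expressive face, sized by a MossQuantity value.
; The construction script runs UpdateScale, which maps MossQuantity to mesh, collision and face scale, then scatters moss and optional flower HISM instances along random directions around the body.
; SetFace swaps eye and mouth textures on the face material, optionally saving the expression.
; A HOLD macro gates repeated input until held long enough, resetting shortly after it stops.
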(fn `SetFace`
  (params (eyes :type "/Game/Art/Material/Face/E_eyes Enum" :default "NewEnumerator0") (mouth :type "/Game/Art/Material/Face/E_mouth Enum" :default "NewEnumerator0") (`ShouldSaveFace?` :type Boolean :default true))
  (locals (eyes_normal_texture :type "Texture Object Reference" :default "/Script/Engine.Texture2D'/Game/Art/Material/Face/e_none.e_none'") (eyes_happy_texture :type "Texture Object Reference" :default "/Script/Engine.Texture2D'/Game/Art/Material/Face/e_happy.e_happy'") (eyes_tired_texture :type "Texture Object Reference" :default "/Script/Engine.Texture2D'/Game/Art/Material/Face/e_tired.e_tired'") (eyes_suspicious_texture :type "Texture Object Reference" :default "/Script/Engine.Texture2D'/Game/Art/Material/Face/e_suspicious.e_suspicious'") (eyes_angry_texture :type "Texture Object Reference" :default "/Script/Engine.Texture2D'/Game/Art/Material/Face/e_angry.e_angry'") (eyes_sad_texture :type "Texture Object Reference" :default "/Script/Engine.Texture2D'/Game/Art/Material/Face/e_sad.e_sad'") (mouth_sad_texture :type "Texture Object Reference" :default "/Script/Engine.Texture2D'/Game/Art/Material/Face/m_sad.m_sad'") (mouth_happy_texture :type "Texture Object Reference" :default "/Script/Engine.Texture2D'/Game/Art/Material/Face/m_happy.m_happy'") (mouth_surprised_texture :type "Texture Object Reference" :default "/Script/Engine.Texture2D'/Game/Art/Material/Face/m_surprised.m_surprised'"))
  (`MaterialInstanceDynamic.SetTextureParameterValue` (`self.FaceMaterial`) "eyes_texture" (select `/Game/Art/Material/Face/E_eyes` eyes :`NewEnumerator0` (`local.eyes_happy_texture`) :`NewEnumerator1` (`local.eyes_sad_texture`) :`NewEnumerator2` (`local.eyes_tired_texture`) :`NewEnumerator3` (`local.eyes_suspicious_texture`) :`NewEnumerator4` (`local.eyes_normal_texture`) :`NewEnumerator5` (`local.eyes_sad_texture`)))
  (`MaterialInstanceDynamic.SetTextureParameterValue` (`self.FaceMaterial`) "mouth_texture" (select `/Game/Art/Material/Face/E_mouth` mouth :`NewEnumerator0` (`local.mouth_happy_texture`) :`NewEnumerator1` (`local.mouth_sad_texture`) :`NewEnumerator2` (`local.mouth_surprised_texture`)))
  (`PrimitiveComponent.SetMaterial` (`self.SM_Face`) 0 (`self.FaceMaterial`))
  (if (`local.ShouldSaveFace?`)
    (set `self.CurrentEyes` eyes)
    (set `self.CurrentMouth` mouth)))

(fn `UpdateScale`
  (params (`ReduceScale?` :type Boolean))
  (bind _hism_moss (`self.HISM_Moss`))
  (bind _hism_flower (`self.HISM_Flower`))
  (bind _ns_mousseparticules (`self.NS_MousseParticules`))
  (bind _returnvalue (* (`KismetMathLibrary.RandomUnitVector`) (`self.r`)))
  (bind _returnvalue_2 (* (`KismetMathLibrary.RandomUnitVector`) (`self.r`)))
  (bind (_returnvalue_min _returnvalue_max) (break `Box` (`StaticMesh.GetBoundingBox` (`StaticMeshComponent.StaticMesh` (`self.SM_Moss`)))))
  (bind (_returnvalue_min_2 _returnvalue_max_2) (break `Box` (`StaticMesh.GetBoundingBox` (`StaticMeshComponent.StaticMesh` (`self.SM_Moss`)))))
  (bind (_returnvalue_roll _returnvalue_pitch _returnvalue_yaw) (`KismetMathLibrary.BreakRotator` (`KismetMathLibrary.MakeRotFromZ` (- _returnvalue_2 (0.0 0.0 0.0)))))
  (bind (_returnvalue_roll_2 _returnvalue_pitch_2 _returnvalue_yaw_2) (`KismetMathLibrary.BreakRotator` (`KismetMathLibrary.MakeRotFromZ` (- _returnvalue (0.0 0.0 0.0)))))
  (bind _returnvalue_x (`KismetMathLibrary.BreakVector` (* (- _returnvalue_max _returnvalue_min) (`self.HISM_Moss_radmult`))))
  (bind _returnvalue_x_2 (`KismetMathLibrary.BreakVector` (* (- _returnvalue_max_2 _returnvalue_min_2) (`self.HISM_Flowers_radmult`))))
  (if (`self.ShowMossFX`)
    (`ActorComponent.Activate` _ns_mousseparticules true)
    (else
      (`ActorComponent.Deactivate` _ns_mousseparticules)))
  (`SceneComponent.SetRelativeScale3D` (`self.SphereCollision`) (`KismetMathLibrary.Conv_DoubleToVector` (`self.ScaleGlobal`)))
  (`SceneComponent.SetRelativeScale3D` (`self.SM_Moss`) (`KismetMathLibrary.Conv_DoubleToVector` (`KismetMathLibrary.MapRangeClamped` (`KismetMathLibrary.Conv_IntToDouble` (`self.MossQuantity`)) 0.0 1000.0 0.7 2.75)))
  (`SphereComponent.SetSphereRadius` (`self.SphereCollision`) (`KismetMathLibrary.Lerp` 50.0 150.0 (`CurveFloat.GetFloatValue` (`self.CollisionScalingCurve`) (`KismetMathLibrary.MapRangeClamped` (`KismetMathLibrary.Conv_IntToDouble` (`self.MossQuantity`)) (`self.Min Moss`) 1000.0 0.0 1.0))) true)
  (`SceneComponent.SetRelativeScale3D` (`self.SM_Face`) (`KismetMathLibrary.Conv_DoubleToVector` (* (`KismetMathLibrary.MapRangeClamped` (`KismetMathLibrary.Conv_IntToDouble` (`self.MossQuantity`)) (`self.Min Moss`) 1000.0 1.2 3.8) (`self.MossVisageMult`))))
  (`MeshComponent.SetScalarParameterValueOnMaterials` (`self.SM_Face`) "Size" (`KismetMathLibrary.MapRangeClamped` (`KismetMathLibrary.Conv_IntToDouble` (`self.MossQuantity`)) (`self.Min Moss`) 1000.0 0.5 0.3))
  (`StaticMeshComponent.SetStaticMesh` (`self.HISM_Flower`) (`self.HISM_Flowers`))
  (`InstancedStaticMeshComponent.ClearInstances` (`self.HISM_Moss`))
  (for _ (range (`KismetMathLibrary.MapRangeClamped` (`KismetMathLibrary.Conv_IntToDouble` (`self.MossQuantity`)) (`self.Min Moss`) 1000.0 500.0 1000.0))
    (set `self.r` _returnvalue_x)
    (`InstancedStaticMeshComponent.AddInstance` _hism_moss (`KismetMathLibrary.MakeTransform` _returnvalue (`KismetMathLibrary.MakeRotator` _returnvalue_roll_2 _returnvalue_pitch_2 _returnvalue_yaw_2) (* (1.0 1.0 1.0) (`self.hismMossScale`))) false)
    (`SceneComponent.K2_AttachToComponent` _hism_moss (`self.SM_Moss`) "None" "SnapToTarget" "SnapToTarget" "SnapToTarget" true))
  (if (`self.ShowFlowers`)
    (`InstancedStaticMeshComponent.ClearInstances` (`self.HISM_Flower`))
    (for _ (range (`KismetMathLibrary.MapRangeClamped` (`KismetMathLibrary.Conv_IntToDouble` (`self.MossQuantity`)) (`self.Min Moss`) 1000.0 0.0 20.0))
      (set `self.r` _returnvalue_x_2)
      (`InstancedStaticMeshComponent.AddInstance` _hism_flower (`KismetMathLibrary.MakeTransform` _returnvalue_2 (`KismetMathLibrary.MakeRotator` _returnvalue_roll _returnvalue_pitch _returnvalue_yaw) (* (1.0 1.0 1.0) (`self.hismFlowersScale`))) false)
      (`SceneComponent.K2_AttachToComponent` _hism_flower (`self.SM_Moss`) "None" "SnapToTarget" "SnapToTarget" "SnapToTarget" true))))

(fn `UserConstructionScript`
  (`self.UpdateScale` false))