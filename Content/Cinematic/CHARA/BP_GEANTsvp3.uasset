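; Cinematic mossy character actor with a textured expression face, scalable body parts and optional flowers and particles.
; Construction scatters moss and flower HISM instances on a seeded sphere around the moss mesh; BeginPlay redoes it from MossQuantity when Animations is on.
; SetFace swaps eye and mouth textures on a dynamic material.
; Tick reapplies face and scales, overriding the idle blink loop; face rotation animation is disconnected.
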(event `self.ReceiveBeginPlay`
  (bind _hism_moss (`self.HISM_Moss`))
  (bind _hism_flower (`self.HISM_Flower`))
  (bind (_returnvalue_min _returnvalue_max) (break `Box` (`StaticMesh.GetBoundingBox` (`StaticMeshComponent.StaticMesh` (`self.SM_Moss`)))))
  (bind (_returnvalue_min_2 _returnvalue_max_2) (break `Box` (`StaticMesh.GetBoundingBox` (`StaticMeshComponent.StaticMesh` (`self.SM_Moss`)))))
  (bind _returnvalue (* (`KismetMathLibrary.RandomUnitVectorFromStream` (`self.s`)) (`self.r`)))
  (bind _returnvalue_2 (* (`KismetMathLibrary.RandomUnitVectorFromStream` (`self.s`)) (`self.r`)))
  (bind (_returnvalue_roll _returnvalue_pitch _returnvalue_yaw) (`KismetMathLibrary.BreakRotator` (`KismetMathLibrary.MakeRotFromZ` (- _returnvalue_2 (0.0 0.0 0.0)))))
  (bind (_returnvalue_roll_2 _returnvalue_pitch_2 _returnvalue_yaw_2) (`KismetMathLibrary.BreakRotator` (`KismetMathLibrary.MakeRotFromZ` (- _returnvalue (0.0 0.0 0.0)))))
  (bind _returnvalue_x (`KismetMathLibrary.BreakVector` (* (- _returnvalue_max _returnvalue_min) (`self.HISM_Moss_radmult`))))
  (bind _returnvalue_x_2 (`KismetMathLibrary.BreakVector` (* (- _returnvalue_max_2 _returnvalue_min_2) (`self.HISM_Flowers_radmult`))))
  (bind _returnvalue_3 (`KismetMaterialLibrary.CreateDynamicMaterialInstance` "/Game/Art/Material/Face/M_Face.M_Face"))
  (bind _output_get (set `self.FaceMaterial` _returnvalue_3))
  (`PrimitiveComponent.SetMaterial` (`self.SM_Face`) 0 _output_get)
  (`self.SetFace` (`self.Eyes`) (`self.Mouth`))
  (`self.UpdateScale` false)
  (if (`self.Animations`)
    (`self.IdleFaceAnim`)
    (set `self.StartRotFaceAnim` (`SceneComponent.RelativeRotation` (`self.SM_Face`)))
    (`self.RotationFaceAnim`)
    (`StaticMeshComponent.SetStaticMesh` (`self.HISM_Flower`) (`self.HISM_Flowers`))
    (`InstancedStaticMeshComponent.ClearInstances` (`self.HISM_Moss`))
    (for _ (range (`KismetMathLibrary.MapRangeClamped` (`self.MossQuantity`) (`self.Min Moss`) 1000.0 500.0 1000.0))
      (set `self.r` _returnvalue_x)
      (`InstancedStaticMeshComponent.AddInstance` _hism_moss (`KismetMathLibrary.MakeTransform` _returnvalue (`KismetMathLibrary.MakeRotator` _returnvalue_roll_2 _returnvalue_pitch_2 _returnvalue_yaw_2) (* (1.0 1.0 1.0) (`self.HISMMossScale`))) false)
      (`SceneComponent.K2_AttachToComponent` _hism_moss (`self.SM_Moss`) "None" "SnapToTarget" "SnapToTarget" "SnapToTarget" true))
    (if (`self.ShowFlowers`)
      (`InstancedStaticMeshComponent.ClearInstances` (`self.HISM_Flower`))
      (for _ (range (`KismetMathLibrary.MapRangeClamped` (`self.MossQuantity`) (`self.Min Moss`) 1000.0 0.0 20.0))
        (set `self.r` _returnvalue_x_2)
        (`InstancedStaticMeshComponent.AddInstance` _hism_flower (`KismetMathLibrary.MakeTransform` _returnvalue_2 (`KismetMathLibrary.MakeRotator` _returnvalue_roll _returnvalue_pitch _returnvalue_yaw) (* (1.0 1.0 1.0) (`self.HISMFlowersScale`))) false)
        (`SceneComponent.K2_AttachToComponent` _hism_flower (`self.SM_Moss`) "None" "SnapToTarget" "SnapToTarget" "SnapToTarget" true)))))

(event `self.ReceiveTick`
  (params (DeltaSeconds :type "Float (single-precision)"))
  (`self.SetFace` (`self.Eyes`) (`self.Mouth`))
  (`self.UpdateScale` false))

(event `IdleFaceAnim`
  (`self.SetFace` "NewEnumerator3" (`self.CurrentMouth`) false)
  (`KismetSystemLibrary.Delay` 0.5)
  (`self.SetFace` (`self.CurrentEyes`) (`self.CurrentMouth`) false)
  (`KismetSystemLibrary.Delay` (`KismetMathLibrary.RandomFloatInRange` 0.5 10.0))
  (`self.IdleFaceAnim`))

(event `RotationFaceAnim`)

(fn `SetFace`
  (params (eyes :type "/Game/Art/Material/Face/E_eyes Enum" :default "NewEnumerator0") (mouth :type "/Game/Art/Material/Face/E_mouth Enum" :default "NewEnumerator0") (`ShouldSaveFace?` :type Boolean :default true))
  (locals (eyes_normal_texture :type "Texture Object Reference" :default "/Script/Engine.Texture2D'/Game/Art/Material/Face/e_none.e_none'") (eyes_happy_texture :type "Texture Object Reference" :default "/Script/Engine.Texture2D'/Game/Art/Material/Face/e_happy.e_happy'") (eyes_tired_texture :type "Texture Object Reference" :default "/Script/Engine.Texture2D'/Game/Art/Material/Face/e_tired.e_tired'") (eyes_suspicious_texture :type "Texture Object Reference" :default "/Script/Engine.Texture2D'/Game/Art/Material/Face/e_suspicious.e_suspicious'") (eyes_angry_texture :type "Texture Object Reference" :default "/Script/Engine.Texture2D'/Game/Art/Material/Face/e_angry.e_angry'") (eyes_sad_texture :type "Texture Object Reference" :default "/Script/Engine.Texture2D'/Game/Art/Material/Face/e_sad.e_sad'") (mouth_sad_texture :type "Texture Object Reference" :default "/Script/Engine.Texture2D'/Game/Art/Material/Face/m_sad.m_sad'") (mouth_happy_texture :type "Texture Object Reference" :default "/Script/Engine.Texture2D'/Game/Art/Material/Face/m_happy.m_happy'") (mouth_surprised_texture :type "Texture Object Reference" :default "/Script/Engine.Texture2D'/Game/Art/Material/Face/m_surprised.m_surprised'") (mouth_smirk_texture :type "Texture Object Reference" :default "/Script/Engine.Texture2D'/Game/Art/Material/Face/ManfaceMouth.ManfaceMouth'") (eyes_smirk_texture :type "Texture Object Reference" :default "/Script/Engine.Texture2D'/Game/Art/Material/Face/Manface.Manface'") (eyes_devastated_testure :type "Texture Object Reference" :default "/Script/Engine.Texture2D'/Game/Art/Material/Face/VisagesSerieuxLarme_copie.VisagesSerieuxLarme_copie'") (eyes_dramatique_testure :type "Texture Object Reference" :default "/Script/Engine.Texture2D'/Game/Art/Material/Face/T_SeriousFace.T_SeriousFace'") (mouth_null_testure :type "Texture Object Reference" :default "/Script/Engine.Texture2D'/Game/Art/Material/Face/m_null.m_null'"))
  (`MaterialInstanceDynamic.SetTextureParameterValue` (`self.FaceMaterial`) "eyes_tex" (select `/Game/Art/Material/Face/E_eyes` eyes :`NewEnumerator0` (`local.eyes_happy_texture`) :`NewEnumerator1` (`local.eyes_sad_texture`) :`NewEnumerator2` (`local.eyes_tired_texture`) :`NewEnumerator3` (`local.eyes_suspicious_texture`) :`NewEnumerator4` (`local.eyes_normal_texture`) :`NewEnumerator5` (`local.eyes_angry_texture`) :`NewEnumerator7` (`local.eyes_smirk_texture`) :`NewEnumerator8` (`local.eyes_dramatique_testure`) :`NewEnumerator9` (`local.eyes_devastated_testure`) :`NewEnumerator10` "/Game/Art/Material/Face/VisagesSerieuxGrinch.VisagesSerieuxGrinch"))
  (`MaterialInstanceDynamic.SetTextureParameterValue` (`self.FaceMaterial`) "mouth_texture" (select `/Game/Art/Material/Face/E_mouth` mouth :`NewEnumerator0` (`local.mouth_happy_texture`) :`NewEnumerator1` (`local.mouth_sad_texture`) :`NewEnumerator2` (`local.mouth_surprised_texture`) :`NewEnumerator3` (`local.mouth_smirk_texture`) :`NewEnumerator4` (`local.mouth_null_testure`)))
  (`PrimitiveComponent.SetMaterial` (`self.SM_Face`) 0 (`self.FaceMaterial`))
  (if (`local.ShouldSaveFace?`)
    (set `self.CurrentEyes` eyes)
    (set `self.CurrentMouth` mouth)))

(fn `UpdateScale`
  (params (`ReduceScale?` :type Boolean))
  (bind _ns_mousseparticules (`self.NS_MousseParticules`))
  (if (`self.ShowMossFX`)
    (`SceneComponent.SetVisibility` _ns_mousseparticules true false)
    (else
      (`SceneComponent.SetVisibility` _ns_mousseparticules false false)))
  (`SceneComponent.SetRelativeScale3D` (`self.SphereCollision`) (`KismetMathLibrary.Conv_DoubleToVector` (`self.ScaleGlobal`)))
  (`SceneComponent.SetRelativeScale3D` (`self.SM_Moss`) (`KismetMathLibrary.Conv_DoubleToVector` (`self.SM_MossScale`)))
  (`SceneComponent.SetRelativeScale3D` (`self.SphereCollision`) (`KismetMathLibrary.Conv_DoubleToVector` (`self.ScaleGlobal`)))
  (`SceneComponent.SetRelativeScale3D` (`self.Armor`) (`KismetMathLibrary.Conv_DoubleToVector` (`self.ArmorScale`)))
  (`SceneComponent.SetRelativeScale3D` (`self.SM_Face`) (`KismetMathLibrary.Conv_DoubleToVector` (`self.VisageScale`)))
  (`MeshComponent.SetScalarParameterValueOnMaterials` (`self.SM_Face`) "Size" (`self.FaceSize`)))

(fn `UserConstructionScript`
  (bind _hism_moss (`self.HISM_Moss`))
  (bind _hism_flower (`self.HISM_Flower`))
  (bind (_returnvalue_min _returnvalue_max) (break `Box` (`StaticMesh.GetBoundingBox` (`StaticMeshComponent.StaticMesh` (`self.SM_Moss`)))))
  (bind (_returnvalue_min_2 _returnvalue_max_2) (break `Box` (`StaticMesh.GetBoundingBox` (`StaticMeshComponent.StaticMesh` (`self.SM_Moss`)))))
  (bind _returnvalue (* (`KismetMathLibrary.RandomUnitVectorFromStream` (`self.s`)) (`self.r`)))
  (bind _returnvalue_2 (* (`KismetMathLibrary.RandomUnitVectorFromStream` (`self.s`)) (`self.r`)))
  (bind (_returnvalue_roll _returnvalue_pitch _returnvalue_yaw) (`KismetMathLibrary.BreakRotator` (`KismetMathLibrary.MakeRotFromZ` (- _returnvalue_2 (0.0 0.0 0.0)))))
  (bind (_returnvalue_roll_2 _returnvalue_pitch_2 _returnvalue_yaw_2) (`KismetMathLibrary.BreakRotator` (`KismetMathLibrary.MakeRotFromZ` (- _returnvalue (0.0 0.0 0.0)))))
  (bind _returnvalue_x (`KismetMathLibrary.BreakVector` (* (- _returnvalue_max _returnvalue_min) (`self.HISM_Moss_radmult`))))
  (bind _returnvalue_x_2 (`KismetMathLibrary.BreakVector` (* (- _returnvalue_max_2 _returnvalue_min_2) (`self.HISM_Flowers_radmult`))))
  (`self.UpdateScale` false)
  (bind _returnvalue_3 (`KismetMaterialLibrary.CreateDynamicMaterialInstance` "/Game/Art/Material/Face/M_Face.M_Face"))
  (bind _output_get (set `self.FaceMaterial` _returnvalue_3))
  (`PrimitiveComponent.SetMaterial` (`self.SM_Face`) 0 _output_get)
  (`self.SetFace` (`self.Eyes`) (`self.Mouth`))
  (`StaticMeshComponent.SetStaticMesh` (`self.HISM_Flower`) (`self.HISM_Flowers`))
  (`InstancedStaticMeshComponent.ClearInstances` (`self.HISM_Moss`))
  (for _ (range (`self.HISMMossQuantity`))
    (set `self.r` _returnvalue_x)
    (`InstancedStaticMeshComponent.AddInstance` _hism_moss (`KismetMathLibrary.MakeTransform` _returnvalue (`KismetMathLibrary.MakeRotator` _returnvalue_roll_2 _returnvalue_pitch_2 _returnvalue_yaw_2) (* (1.0 1.0 1.0) (`self.HISMMossScale`))) false)
    (`SceneComponent.K2_AttachToComponent` _hism_moss (`self.SM_Moss`) "None" "SnapToTarget" "SnapToTarget" "SnapToTarget" true))
  (if (`self.ShowFlowers`)
    (`InstancedStaticMeshComponent.ClearInstances` (`self.HISM_Flower`))
    (for _ (range (`self.HISMFlowerQuantity`))
      (set `self.r` _returnvalue_x_2)
      (`InstancedStaticMeshComponent.AddInstance` _hism_flower (`KismetMathLibrary.MakeTransform` _returnvalue_2 (`KismetMathLibrary.MakeRotator` _returnvalue_roll _returnvalue_pitch _returnvalue_yaw) (* (1.0 1.0 1.0) (`self.HISMFlowersScale`))) false)
      (`SceneComponent.K2_AttachToComponent` _hism_flower (`self.SM_Moss`) "None" "SnapToTarget" "SnapToTarget" "SnapToTarget" true))))